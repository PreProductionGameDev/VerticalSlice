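; BP_Room is a modular room builder that assembles an optional scaled floor and four walls from static mesh components in the construction script.
; BuildWall (X axis) and BuildWallB (Y axis) lay 100-unit pieces in a grid, sized by Length, Width and Height.
; Per-wall settings can omit a wall or cut door openings, spaced by splitting the remaining wall into equal runs and filled in above door height.
; The event graph has no active logic.
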(fn `BuildWall`
  (params (Width :type Integer) (Count :type Integer) (WallSize :type Integer) (Position :type "Transform Structure") (Height :type Integer) (DoorHeight :type Integer) (NoWall :type Boolean))
  (locals (WallCount :type "Float (double-precision)") (IsPlacingWall :type Boolean :default true) (OffsetPiece :type "Float (double-precision)") (WallLength :type "Float (double-precision)") (USEEXTRA :type Boolean) (`Door Counter` :type Integer) (DoorPlaced :type Integer) (WallPlaced :type Integer) (DoorPlace :type Integer))
  (bind _location (.location Position))
  (bind _rotation (.rotation Position))
  (bind _scale (.scale Position))
  (if (not NoWall)
    (set `local.WallCount` (`KismetMathLibrary.Conv_IntToDouble` (`KismetMathLibrary.FFloor` (/ (`KismetMathLibrary.Conv_IntToDouble` (- WallSize (* Width Count))) (`KismetMathLibrary.Conv_IntToDouble` (+ Count 1))))))
    (for _index (range WallSize)
      (for _index_2 (range DoorHeight Height)
        (bind _returnvalue (* _index 100))
        (`AddComponent|NODE_AddStaticMeshComponent-9` :`RelativeTransform` (`KismetMathLibrary.MakeTransform` (+ _location (`KismetMathLibrary.MakeVector` _returnvalue 0.0 (* _index_2 100))) _rotation _scale)))
      (if (`local.IsPlacingWall`)
        (set `local.WallPlaced` (+ (`local.WallPlaced`) 1))
        (for _index_3 (range DoorHeight)
          (`AddComponent|NODE_AddStaticMeshComponent-8` :`RelativeTransform` (`KismetMathLibrary.MakeTransform` (+ _location (`KismetMathLibrary.MakeVector` _returnvalue 0.0 (* _index_3 100))) _rotation _scale)))
        (if (== (`local.WallPlaced`) (`local.WallCount`))
          (if (not (== (`local.DoorPlace`) Count))
            (set `local.IsPlacingWall` false)
            (set `local.WallPlaced` 0)))
        (else
          (set `local.Door Counter` (+ (`local.Door Counter`) 1))
          (if (and (== (`local.Door Counter`) Width) (!= Width 0))
            (set `local.IsPlacingWall` true)
            (set `local.Door Counter` 0)
            (set `local.DoorPlaced` (+ (`local.DoorPlaced`) 1))
            (set `local.DoorPlace` (+ (`local.DoorPlace`) 1))))))))

(fn `BuildWallB`
  (params (Width :type Integer) (Count :type Integer) (WallSize :type Integer) (Position :type "Transform Structure") (Height :type Integer) (DoorHeight :type Integer) (NoWall :type Boolean))
  (locals (WallCount :type "Float (double-precision)") (IsPlacingWall :type Boolean :default true) (OffsetPiece :type "Float (double-precision)") (WallLength :type "Float (double-precision)") (USEEXTRA :type Boolean) (`Door Counter` :type Integer) (DoorPlaced :type Integer) (WallPlaced :type Integer) (DoorPlace :type Integer))
  (bind _location (.location Position))
  (bind _rotation (.rotation Position))
  (bind _scale (.scale Position))
  (if (not NoWall)
    (set `local.WallCount` (`KismetMathLibrary.Conv_IntToDouble` (`KismetMathLibrary.FFloor` (/ (`KismetMathLibrary.Conv_IntToDouble` (- WallSize (* Width Count))) (`KismetMathLibrary.Conv_IntToDouble` (+ Count 1))))))
    (for _index (range WallSize)
      (for _index_2 (range DoorHeight Height)
        (bind _returnvalue (* _index 100))
        (`AddComponent|NODE_AddStaticMeshComponent-11` :`RelativeTransform` (`KismetMathLibrary.MakeTransform` (+ _location (`KismetMathLibrary.MakeVector` 0.0 _returnvalue (* _index_2 100))) _rotation _scale)))
      (if (`local.IsPlacingWall`)
        (set `local.WallPlaced` (+ (`local.WallPlaced`) 1))
        (for _index_3 (range DoorHeight)
          (`AddComponent|NODE_AddStaticMeshComponent-10` :`RelativeTransform` (`KismetMathLibrary.MakeTransform` (+ _location (`KismetMathLibrary.MakeVector` 0.0 _returnvalue (* _index_3 100))) _rotation _scale)))
        (if (== (`local.WallPlaced`) (`local.WallCount`))
          (if (not (== (`local.DoorPlace`) Count))
            (set `local.IsPlacingWall` false)
            (set `local.WallPlaced` 0)))
        (else
          (set `local.Door Counter` (+ (`local.Door Counter`) 1))
          (if (and (== (`local.Door Counter`) Width) (!= Width 0))
            (set `local.IsPlacingWall` true)
            (set `local.Door Counter` 0)
            (set `local.DoorPlaced` (+ (`local.DoorPlaced`) 1))
            (set `local.DoorPlace` (+ (`local.DoorPlace`) 1))))))))

(fn `UserConstructionScript`
  (if (`self.UseFloor`)
    (`AddComponent|NODE_AddStaticMeshComponent-0` :`RelativeTransform` (`KismetMathLibrary.MakeTransform` (0.0 0.0 0.0) (struct) (`KismetMathLibrary.MakeVector` (`KismetMathLibrary.Conv_IntToDouble` (`self.Length`)) (`KismetMathLibrary.Conv_IntToDouble` (`self.Width`)) 1.0))))
  (`self.BuildWall` (`self.DoorWidthA`) (`self.DoorsWallA`) (`self.Length`) (`KismetMathLibrary.MakeTransform` (0.0 0.0 0.0)) (`self.Height`) (`self.DoorHeightA`) (`self.NoWallA`))
  (`self.BuildWallB` (`self.DoorWidthB`) (`self.DoorsWallB`) (`self.Width`) (`KismetMathLibrary.MakeTransform` (0.0 100.0 0.0) (struct :`Yaw` 270.0)) (`self.Height`) (`self.DoorHeightB`) (`self.NoWallB`))
  (`self.BuildWall` (`self.DoorWidthC`) (`self.DoorsWallC`) (`self.Length`) (`KismetMathLibrary.MakeTransform` (`KismetMathLibrary.MakeVector` 100.0 (`KismetMathLibrary.Conv_IntToDouble` (* (`self.Width`) 100))) (struct :`Yaw` 180.0)) (`self.Height`) (`self.DoorHeightC`) (`self.NoWallC`))
  (`self.BuildWallB` (`self.DoorWidthD`) (`self.DoorsWallD`) (`self.Width`) (`KismetMathLibrary.MakeTransform` (`KismetMathLibrary.MakeVector` (`KismetMathLibrary.Conv_IntToDouble` (* (`self.Length`) 100))) (struct :`Yaw` 90.0)) (`self.Height`) (`self.DoorHeightD`) (`self.NoWallD`)))