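; Ambient tree sound actor that plays cricket and bird cues at randomised intervals.
; BeginPlay starts a one-shot timer of roughly 2 to 12 seconds, which triggers a random MultiGate choosing one cue and re-arming the timer.
; The gate is non-looping and never reset, so each cue plays only once.
; Tick also re-arms the timer whenever its handle is invalid.
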(event `self.ReceiveBeginPlay`
  (bind _returnvalue (`KismetSystemLibrary.K2_SetTimerDelegate` (delegate `PlayCue`) (+ (* (`KismetMathLibrary.RandomFloat`) 10.0) 2.0) :!label _label))
  (set `self.sound handle` _returnvalue))

(event `PlayCue`
  (`|MultiGate` true
    (:`Out 0`
      (`AudioComponent.Play` (`self.Cricket_Cue`) 0.0)
      (goto _label))
    (:`Out 1`
      (`AudioComponent.Play` (`self.Bird_Cue`) 0.0)
      (goto _label))))

(event `self.ReceiveTick`
  (params (DeltaSeconds :type "Float (single-precision)"))
  (if (not (`KismetSystemLibrary.K2_IsValidTimerHandle` (`self.sound handle`)))
    (goto _label)))

(fn `UserConstructionScript`)