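; Death camera actor that flies from the instigating character's first-person view toward a final position.
; Tick lerps it over about half a second, with sweep, to 600 units short of that point, facing it.
; On arrival it captures the scene with a SceneCapture2D.
; Once the respawn HUD is valid, it turns that HUD's border white, returns player 0's view to the character and destroys itself.
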(event `self.ReceiveBeginPlay`
  (bind _firstpersoncameracomponent (`FP_Character.FirstPersonCameraComponent` (cast `/Game/ShiitakeSorcerers/Character/BP_FPCharacter` (`self.GetInstigator`) :!pure true)))
  (set `self.InitalPosition` (`SceneComponent.K2_GetComponentLocation` _firstpersoncameracomponent))
  (set `self.InitalRotation` (`SceneComponent.K2_GetComponentRotation` _firstpersoncameracomponent)))

(event `self.ReceiveTick`
  (params (DeltaSeconds :type "Float (single-precision)"))
  (bind _returnvalue (+ DeltaSeconds DeltaSeconds))
  (bind _finalposition (`self.FinalPosition`))
  (bind _alpha (`self.Alpha`))
  (bind _defaultsceneroot (`self.DefaultSceneRoot`))
  (bind _returnvalue_2 (`KismetMathLibrary.Normal` (- (`self.InitalPosition`) _finalposition)))
  (bind _respawn_hud (`/Game/ShiitakeSorcerers/Character/BP_FPCharacter.Respawn Hud` (cast `/Game/ShiitakeSorcerers/Character/BP_FPCharacter` (`self.GetInstigator`) :!pure true)))
  (bind _returnvalue_3 (`KismetMathLibrary.VLerp` (`self.InitalPosition`) (+ _finalposition (* _returnvalue_2 600.0)) _alpha))
  (bind _returnvalue_4 (`KismetMathLibrary.RLerp` (`self.InitalRotation`) (`KismetMathLibrary.FindLookAtRotation` (`KismetMathLibrary.MakeVector` 0.0) (* _returnvalue_2 -1.0)) _alpha))
  (if (< (+ _returnvalue (`self.Alpha`)) 1.0)
    (set `self.Alpha` (+ _returnvalue (`self.Alpha`)))
    (`SceneComponent.K2_SetWorldLocationAndRotation` _defaultsceneroot _returnvalue_3 _returnvalue_4 true false)
    (else
      (set `self.Alpha` 1.0)
      (`SceneComponent.K2_SetWorldLocationAndRotation` _defaultsceneroot _returnvalue_3 _returnvalue_4 true false)
      (`SceneCaptureComponent2D.CaptureScene` (`self.SceneCaptureComponent2D`))
      (`/Engine/EditorBlueprintResources/StandardMacros.IsValid` _respawn_hud
        (:`Is Valid`
          (`Border.SetBrushColor` (`/Game/ShiitakeSorcerers/UI/ElementSelect/UW_ElementSelect.Border_0` _respawn_hud) (struct :`R` 1.0 :`G` 1.0 :`B` 1.0 :`A` 1.0))
          (`PlayerController.SetViewTargetWithBlend` (`GameplayStatics.GetPlayerController` 0) (cast `/Game/ShiitakeSorcerers/Character/BP_FPCharacter` (`self.GetInstigator`) :!pure true) 0.0 "VTBlend_Linear" 0.0 false)
          (`self.K2_DestroyActor`))))))

(fn `UserConstructionScript`)