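; First-person multiplayer player character for Shiitake Sorcerers, combining GAS health and abilities with swappable guns.
; Damage and health events drive the HUD, hit indicators and camera-facing health bars; death reports the kill, ragdolls via multicast and starts a respawn timer.
; Number keys spawn weapons, Q swaps elemental abilities by rewriting input mappings, and Tab shows the scoreboard.
; Also handles heat-based decaying recoil and replicated material hues.
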(event `Key|Escape`
  (params (Key :type "Key Structure"))
  (:`Pressed`
    (bind _asbp_gi_multiplayer (cast `/Game/ShiitakeSorcerers/UI/Networking/BP_GI_Multiplayer` (`GameplayStatics.GetGameInstance`)))
    (`/Game/ShiitakeSorcerers/UI/Networking/BP_GI_Multiplayer.Leave Session` _asbp_gi_multiplayer)))

(event `ClientGameOver`
  (`self.DisableInput` (`GameplayStatics.GetPlayerController` 0))
  (`KismetSystemLibrary.K2_ClearAndInvalidateTimerHandle` (`self.RespawnTimer`))
  (`self.ServerGetScore`))

(event `Respawn`
  ;[1 1 1] Respawns the player
  (message `/Game/ShiitakeSorcerers/Core/GamemodeInterface.Respawn` (`GameplayStatics.GetGameMode`) self)
  (`self.MulticastEnableInput`)
  (`AbilitySystemComponent.PressInputID` (`self.AbilitySystemComponent`) (`KismetMathLibrary.Conv_ByteToInt` (enumliteral `EPlayerAbilityInputID` "Respawn")))
  (bind _returnvalue (`self.GetEquippedGun`))
  (`SceneComponent.SetVisibility` (`BaseWeapon.FP_Mesh` _returnvalue) true false))

(event `ClientSpawnHud`
  ;[1 1 1] Spawns the hud on the client
  (bind _returnvalue (`|CreateWidget` "/Game/ShiitakeSorcerers/UI/HUD/WB_HUD.WB_HUD_C"))
  (set `self.Hud` _returnvalue)
  (`UserWidget.AddToViewport` _returnvalue 0))

(event `ClientHealthHud`
  (params (OldHealth :type "Float (double-precision)") (NewHealth :type "Float (double-precision)"))
  (bind _hud (`self.Hud`))
  ;[1 1 1] Updates the hud on the owning client
  (`/Engine/EditorBlueprintResources/StandardMacros.IsValid` _hud
    (:`Is Valid`
      (`/Game/ShiitakeSorcerers/UI/HUD/WB_PlayerHealthBar.Health Changed` (`/Game/ShiitakeSorcerers/UI/HUD/WB_HUD.WB_PlayerHealthBar` _hud) OldHealth NewHealth))))

(event `MulticastUpdateHealthBar`
  (params (Health :type "Float (double-precision)"))
  ;[1 1 1] Waits for server to replicate health to update client
  (`KismetSystemLibrary.DelayUntilNextTick`)
  (`self.UpdateHealthBar` Health))

(event `ClientHitDirection`
  (params (FiringTarget :type "Actor Object Reference"))
  ;[1 1 1] Spawns a hit dir marker on owning client
  (if (`self.IsLocallyControlled`)
    (bind _returnvalue (`|CreateWidget` "/Game/ShiitakeSorcerers/UI/HitIndicator/WB_HitIndicator.WB_HitIndicator_C" null FiringTarget))
    (`UserWidget.AddToViewport` _returnvalue 0)))

(event `MulticastEnableInput`
  ;[1 1 1] Remove ragdoll, reset player, enable input
  (`self.EnableInput` (`GameplayStatics.GetPlayerController` 0))
  (`PrimitiveComponent.SetSimulatePhysics` (`self.Mesh`) false)
  (`PrimitiveComponent.SetCollisionProfileName` (`self.Mesh`) "CharacterMesh" true)
  (`SceneComponent.K2_AttachToComponent` (`self.Mesh`) (`self.CapsuleComponent`) "None" "KeepRelative" "KeepRelative" "KeepRelative" true)
  (`PrimitiveComponent.SetCollisionProfileName` (`self.CapsuleComponent`) "Pawn" true)
  (set `self.Ammo` 80))

(event `MulticastDisableInput`
  ;[1 1 1] Disable user input and ragdoll
  (`self.DisableInput` (`GameplayStatics.GetPlayerController` 0))
  (`PrimitiveComponent.SetCollisionProfileName` (`self.Mesh`) "Ragdoll" true)
  (`PrimitiveComponent.SetCollisionResponseToChannel` (`self.Mesh`) "ECC_Camera" "ECR_Ignore")
  (`PrimitiveComponent.SetSimulatePhysics` (`self.Mesh`) true)
  (`PrimitiveComponent.SetCollisionProfileName` (`self.CapsuleComponent`) "NoCollision" true)
  (bind _returnvalue (`self.GetEquippedGun`))
  (`BaseWeapon.OnUnequip` _returnvalue))

(event `self.OnDamaged`
  (params (DamageAmount :type "Float (single-precision)") (HitInfo :type "HitResult Structure (by ref)") (DamageTags :type "GameplayTagContainer Structure (by ref)") (InstigatorCharacter :type "FP_Character Object Reference") (DamageCauser :type "Actor Object Reference"))
  ;[1 1 1] Server event when damage is delt
  (set `self.LastDamagingPlayer` (`PlayerState.GetPlayerName` (`Pawn.PlayerState` InstigatorCharacter)))
  (`self.ClientHitDirection` DamageCauser))

(event `self.OnHealthChanged`
  (params (DeltaValue :type "Float (single-precision)") (EventTags :type "GameplayTagContainer Structure (by ref)"))
  ;[1 1 1] Server Event when health is changed
  (bind _returnvalue (`self.GetHealth`))
  (`self.MulticastUpdateHealthBar` _returnvalue)
  (bind _returnvalue_2 (`self.GetHealth`))
  (`self.ClientHealthHud` (- _returnvalue_2 DeltaValue) _returnvalue_2))

(event `self.OnDeath`
  ;[1 1 1] Server event when player health is <=0.01
  (message `/Game/ShiitakeSorcerers/Core/GamemodeInterface.PlayerScored` (`GameplayStatics.GetGameMode`) (`self.LastDamagingPlayer`) (`PlayerState.GetPlayerName` (`self.PlayerState`)))
  (`self.MulticastDisableInput`)
  (bind _returnvalue (`KismetSystemLibrary.K2_SetTimerDelegate` (`|CreateDelegate` :!event `Respawn`) 5.0))
  (set `self.RespawnTimer` _returnvalue))

(event `self.ReceiveBeginPlay`
  (`self.ClientClearHud`)
  (`/Engine/EditorBlueprintResources/ActorMacros.Switch Has Authority`
    (:`Authority`
      _)
    (:`Remote`
      _))
  (`KismetSystemLibrary.DelayUntilNextTick`)
  (if (`self.IsLocallyControlled`)
    (`self.ClientSpawnHud`))
  (`KismetSystemLibrary.DelayUntilNextTick`)
  ;[1 1 1] Fills the health bar and hides it if owning player
  (bind _returnvalue (`self.GetHealth`))
  (`self.UpdateHealthBar` _returnvalue)
  (bind _asbp_fpcharacter (cast `/Game/ShiitakeSorcerers/Character/BP_FPCharacter` (`GameplayStatics.GetPlayerCharacter` 0)))
  (if (== _asbp_fpcharacter self)
    (`SceneComponent.SetVisibility` (`self.Widget`) false false)
    (`self.SwapAbility`)))

(event `ClientClearHud`
  (`WidgetLayoutLibrary.RemoveAllWidgets`))

(event `self.ReceiveTick`
  (params (DeltaSeconds :type "Float (single-precision)"))
  (bind _widget (`self.Widget`))
  (bind _wb_guns (`/Game/ShiitakeSorcerers/UI/HUD/WB_HUD.WB_Guns` (`self.Hud`)))
  (`self.RecoilUpdate`)
  ;[1 1 1] Points the healthbar towards the local player
  (`self.RecoilDecay`)
  (bind _asbp_fpcharacter (cast `/Game/ShiitakeSorcerers/Character/BP_FPCharacter` (`GameplayStatics.GetPlayerCharacter` 0)))
  (`SceneComponent.K2_SetWorldRotation` _widget (`KismetMathLibrary.FindLookAtRotation` (`SceneComponent.K2_GetComponentLocation` _widget) (`SceneComponent.K2_GetComponentLocation` (`FP_Character.FirstPersonCameraComponent` _asbp_fpcharacter))) false false)
  (if (`self.IsLocallyControlled`)
    (bind _returnvalue (`self.GetEquippedGun`))
    (`/Engine/EditorBlueprintResources/StandardMacros.IsValid` _returnvalue
      (:`Is Valid`
        (bind _data (`BaseWeapon.Data` _returnvalue))
        (`Image.SetBrushFromTexture` (`/Game/ShiitakeSorcerers/UI/HUD/WB_Guns.Image_34` _wb_guns) (`BaseWeaponDataAsset.WeaponIcon` _data) false)
        (`TextBlock.SetText` (`/Game/ShiitakeSorcerers/UI/HUD/WB_Guns.TextBlock_160` _wb_guns) (`KismetTextLibrary.Conv_IntToText` (/ (`self.Ammo`) (`BaseWeaponDataAsset.StartingAmmo` _data))))))))

(event `ClientHudSwap`
  (bind _wb_iconbutton (`/Game/ShiitakeSorcerers/UI/HUD/WB_HUD.WB_IconButton` (`self.Hud`)))
  (bind _wb_secondaryiconbutton (`/Game/ShiitakeSorcerers/UI/HUD/WB_HUD.WB_SecondaryIconButton` (`self.Hud`)))
  (bind _wb_iconbutton_2 (`/Game/ShiitakeSorcerers/UI/HUD/WB_HUD.WB_IconButton` (`self.Hud`)))
  (bind _wb_secondaryiconbutton_2 (`/Game/ShiitakeSorcerers/UI/HUD/WB_HUD.WB_SecondaryIconButton` (`self.Hud`)))
  ;[1 1 1] Swaps the Hud Timer Handles across
  (set `self.TempAbility CD` (`/Game/ShiitakeSorcerers/UI/HUD/WB_IconButton.AbilityCD` (`/Game/ShiitakeSorcerers/UI/HUD/WB_HUD.WB_IconButton` (`self.Hud`))))
  (set `/Game/ShiitakeSorcerers/UI/HUD/WB_IconButton.AbilityCD` (`/Game/ShiitakeSorcerers/UI/HUD/WB_IconButton.AbilityCD` (`/Game/ShiitakeSorcerers/UI/HUD/WB_HUD.WB_SecondaryIconButton` (`self.Hud`))) (`/Game/ShiitakeSorcerers/UI/HUD/WB_HUD.WB_IconButton` (`self.Hud`)))
  (set `/Game/ShiitakeSorcerers/UI/HUD/WB_IconButton.AbilityCD` (`self.TempAbility CD`) (`/Game/ShiitakeSorcerers/UI/HUD/WB_HUD.WB_SecondaryIconButton` (`self.Hud`)))
  (if (`self.PrimaryElement`)
    (`Widget.SetVisibility` (`/Game/ShiitakeSorcerers/UI/HUD/WB_IconButton.Element` _wb_iconbutton) "Visible")
    (`Widget.SetVisibility` (`/Game/ShiitakeSorcerers/UI/HUD/WB_IconButton.ElementBorder` _wb_iconbutton) "Visible")
    (`Widget.SetVisibility` (`/Game/ShiitakeSorcerers/UI/HUD/WB_IconButton.Element_2` _wb_iconbutton) "Hidden")
    (`Widget.SetVisibility` (`/Game/ShiitakeSorcerers/UI/HUD/WB_IconButton.Element` _wb_secondaryiconbutton) "Hidden")
    (`Widget.SetVisibility` (`/Game/ShiitakeSorcerers/UI/HUD/WB_IconButton.ElementBorder` _wb_secondaryiconbutton) "Hidden")
    (`Widget.SetVisibility` (`/Game/ShiitakeSorcerers/UI/HUD/WB_IconButton.Element_2` _wb_secondaryiconbutton) "Visible")
    (else
      (`Widget.SetVisibility` (`/Game/ShiitakeSorcerers/UI/HUD/WB_IconButton.Element` _wb_iconbutton_2) "Hidden")
      (`Widget.SetVisibility` (`/Game/ShiitakeSorcerers/UI/HUD/WB_IconButton.ElementBorder` _wb_iconbutton_2) "Hidden")
      (`Widget.SetVisibility` (`/Game/ShiitakeSorcerers/UI/HUD/WB_IconButton.Element_2` _wb_iconbutton_2) "Visible")
      (`Widget.SetVisibility` (`/Game/ShiitakeSorcerers/UI/HUD/WB_IconButton.Element` _wb_secondaryiconbutton_2) "Visible")
      (`Widget.SetVisibility` (`/Game/ShiitakeSorcerers/UI/HUD/WB_IconButton.ElementBorder` _wb_secondaryiconbutton_2) "Visible")
      (`Widget.SetVisibility` (`/Game/ShiitakeSorcerers/UI/HUD/WB_IconButton.Element_2` _wb_secondaryiconbutton_2) "Hidden"))))

(event `ServerGetScore`
  ;[1 1 1] Gets the score from the gamemode
  (bind _scores (message `/Game/ShiitakeSorcerers/Core/GamemodeInterface.GetScores` (`GameplayStatics.GetGameMode`)))
  (bind _keys (`BlueprintMapLibrary.Map_Keys` _scores))
  (bind _values (`BlueprintMapLibrary.Map_Values` _scores))
  (`self.ClientOpenLeaderBoard` _keys _values))

(event `ClientOpenLeaderBoard`
  (params (`Players ` :type "Array of String") (Scores :type "Array of Integer"))
  ;[1 1 1] Displays the leaderboard on the client
  (bind _returnvalue (`|CreateWidget` "/Game/ShiitakeSorcerers/UI/ScoreBoard/UW_ScoreBoard.UW_ScoreBoard_C" null `Players ` Scores))
  (bind _output_get (set `self.LeaderBoard` _returnvalue))
  (`UserWidget.AddToViewport` _output_get 0))

(event `RecoilUpdate`
  (bind (_returnvalue_x _returnvalue_y) (`KismetMathLibrary.BreakVector` (- (`self.DesiredRecoil`) (`self.CurrentRecoil`))))
  (`self.AddControllerYawInput` _returnvalue_x)
  (`self.AddControllerPitchInput` _returnvalue_y)
  (set `self.CurrentRecoil` (`self.DesiredRecoil`)))

(event `RecoilDecay`
  (set `self.DesiredRecoil` (* (`self.DesiredRecoil`) 0.95)))

(event `Cooldown`
  (if (> (`self.Heat`) 0)
    (`/Engine/EditorBlueprintResources/StandardMacros.DecrementInt` (`self.Heat`)
      (:`  `
        (`KismetSystemLibrary.K2_ClearAndInvalidateTimerHandle` (`self.CooldownTimer`))
        (bind _returnvalue (`KismetSystemLibrary.K2_SetTimerDelegate` (`|CreateDelegate` :!event `Cooldown`) 0.1))
        (set `self.CooldownTimer` _returnvalue)))))

(event `ServerSpawnFire`
  (params (Location :type "Vector Structure"))
  (`|SpawnActorFromClass` "/Game/ShiitakeSorcerers/Core/Abilities/FireBall/BP_FireBallHitbox.BP_FireBallHitbox_C" (`KismetMathLibrary.MakeTransform` Location) "Undefined" "OverrideRootScale" null self))

(event `Key|Tab`
  (params (Key :type "Key Structure"))
  ;[1 1 1] Opens and closes the scoreboard
  (:`Pressed`
    (`self.ServerGetScore`))
  (:`Released`
    (`Widget.RemoveFromParent` (`self.LeaderBoard`))))

(event `SwapAbility`
  (bind _outmappings (`InputSettings.GetActionMappingByName` (`InputSettings.GetInputSettings`) (`self.ElementTwo`)))
  (set `self.PrimaryElement` (not (`self.PrimaryElement`)) :!label _label)
  (`self.ClientHudSwap`)
  ;[1 1 1] Switches the axis mapping to the currently active skill
  (if (`self.PrimaryElement`)
    (if (not (== (`KismetArrayLibrary.Array_Length` _outmappings) 0))
      (`InputSettings.RemoveActionMapping` (`InputSettings.GetInputSettings`) (`|GetArrayItem` _outmappings) true))
    (`InputSettings.AddActionMapping` (`InputSettings.GetInputSettings`) (make `InputActionKeyMapping` (`self.ElementOne`) false false false false "E") true)
    (else
      (`InputSettings.RemoveActionMapping` (`InputSettings.GetInputSettings`) (`|GetArrayItem` (`InputSettings.GetActionMappingByName` (`InputSettings.GetInputSettings`) (`self.ElementOne`))) true)
      (`InputSettings.AddActionMapping` (`InputSettings.GetInputSettings`) (make `InputActionKeyMapping` (`self.ElementTwo`) false false false false "E") true))))

(event `Key|Q`
  (params (Key :type "Key Structure"))
  (:`Pressed`
    (goto _label)))

(event `Key|One`
  (params (Key :type "Key Structure"))
  (:`Pressed`
    (bind _returnvalue (`self.GetEquippedGun`))
    (`/Engine/EditorBlueprintResources/StandardMacros.IsValid` _returnvalue
      (:`Is Valid`
        (`BaseWeapon.OnUnequip` _returnvalue))
      (:`Is Not Valid`
        _))
    (`self.Server_SpawnWeapon` "/Game/ShiitakeSorcerers/Weapons/Sniper/BW_Sniper.BW_Sniper_C" (`SceneComponent.GetRelativeTransform` (`self.FP_GunPos`)) self)))

(event `Key|Three`
  (params (Key :type "Key Structure"))
  (:`Pressed`
    (bind _returnvalue (`self.GetEquippedGun`))
    (`/Engine/EditorBlueprintResources/StandardMacros.IsValid` _returnvalue
      (:`Is Valid`
        (`BaseWeapon.OnUnequip` _returnvalue))
      (:`Is Not Valid`
        _))
    (`self.Server_SpawnWeapon` "/Game/ShiitakeSorcerers/Weapons/Shotgun/BW_Shotgun.BW_Shotgun_C" (`SceneComponent.GetRelativeTransform` (`self.FP_GunPos`)) self)))

(event `Key|Two`
  (params (Key :type "Key Structure"))
  (:`Pressed`
    (bind _returnvalue (`self.GetEquippedGun`))
    (`/Engine/EditorBlueprintResources/StandardMacros.IsValid` _returnvalue
      (:`Is Valid`
        (`BaseWeapon.OnUnequip` _returnvalue))
      (:`Is Not Valid`
        _))
    (`self.Server_SpawnWeapon` "/Game/ShiitakeSorcerers/Weapons/SMG/BW_SMG.BW_SMG_C" (`SceneComponent.GetRelativeTransform` (`self.FP_GunPos`)) self)))

(event `Key|L`
  (params (Key :type "Key Structure"))
  (:`Pressed`
    (`self.RecoilKick`)))

(event `RecoilKick`
  (bind _heat (`self.Heat`))
  (if (< _heat 10)
    (bind _result (`/Engine/EditorBlueprintResources/StandardMacros.IncrementInt` _heat)
      (:`  `
        _)))
  (`KismetSystemLibrary.K2_ClearAndInvalidateTimerHandle` (`self.CooldownTimer`))
  (bind _returnvalue (`KismetSystemLibrary.K2_SetTimerDelegate` (`|CreateDelegate` :!event `Cooldown`) 0.2))
  (set `self.CooldownTimer` _returnvalue)
  (bind _value (`BlueprintMapLibrary.Map_Find` (`self.HeatMap`) _result))
  (set `self.DesiredRecoil` (`KismetMathLibrary.MakeVector` (`KismetMathLibrary.RandomFloatInRange` (* (.x _value) -1.0) (.x _value)) (.y _value))))

(event `Server_SpawnWeapon`
  (params (Class :type "Actor Class Reference") (SpawnTransform :type "Transform Structure") (Owner :type "/Game/ShiitakeSorcerers/Character/BP_FPCharacter Object Reference"))
  (bind _returnvalue (`|SpawnActorFromClass` Class SpawnTransform "Undefined" "OverrideRootScale" Owner null))
  (`self.K2_AttachToComponent` _returnvalue (`/Game/ShiitakeSorcerers/Character/BP_FPCharacter.FP_GunPos` Owner) "None" "SnapToTarget" "SnapToTarget" "SnapToTarget" true)
  (bind _asbase_weapon (cast `BaseWeapon` _returnvalue :!pure true))
  (`SceneComponent.K2_SetRelativeTransform` (`BaseWeapon.FP_Mesh` _asbase_weapon) (`SceneComponent.GetRelativeTransform` (`BaseWeapon.FPHelper` _asbase_weapon)) false false)
  (bind _tp_mesh (`BaseWeapon.TP_Mesh` _asbase_weapon))
  (`SceneComponent.K2_AttachToComponent` _tp_mesh (`self.Mesh`) "TP_GunPos" "KeepRelative" "KeepRelative" "KeepRelative" true)
  (`SceneComponent.K2_SetRelativeTransform` _tp_mesh (`SceneComponent.GetRelativeTransform` (`BaseWeapon.TPHelper` _asbase_weapon)) false false)
  (`self.EquipGun` _asbase_weapon))

(fn `OnRep_Color`
  (bind _returnvalue (`PrimitiveComponent.CreateDynamicMaterialInstance` (`self.Mesh`) 0 null "None"))
  (`MaterialInstanceDynamic.SetScalarParameterValue` _returnvalue "Hue" (.x (`self.Color`)))
  (bind _returnvalue_2 (`PrimitiveComponent.CreateDynamicMaterialInstance` (`self.Mesh`) 3 null "None"))
  (`MaterialInstanceDynamic.SetScalarParameterValue` _returnvalue_2 "Hue" (.y (`self.Color`)))
  (bind _returnvalue_3 (`PrimitiveComponent.CreateDynamicMaterialInstance` (`self.Mesh`) 2 null "None"))
  (`MaterialInstanceDynamic.SetScalarParameterValue` _returnvalue_3 "Hue" (.z (`self.Color`))))

(fn `UpdateHealthBar`
  (params (Health :type "Float (double-precision)"))
  ;[1 1 1] Updates the health bar to the health atrib / max health atrib
  (bind _returnvalue (`self.GetMaxHealth`))
  (bind _aswb_enemy_health_bar (cast `/Game/ShiitakeSorcerers/UI/HUD/WB_EnemyHealthBar` (`WidgetComponent.GetWidget` (`self.Widget`))))
  (`/Game/ShiitakeSorcerers/UI/HUD/WB_EnemyHealthBar.Adjust Health` _aswb_enemy_health_bar (/ Health _returnvalue)))

(fn `UserConstructionScript`)