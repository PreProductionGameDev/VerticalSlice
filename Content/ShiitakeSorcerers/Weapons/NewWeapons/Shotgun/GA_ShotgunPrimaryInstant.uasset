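; Gameplay ability that fires one instant shotgun shot, rate-limited by the timing of GA_ShotgunPrimary.
; The local player runs an eight-trace reusable line-trace target actor with spread, while the server waits for replicated target data.
; Target data commits clip-ammo cost, plays first- and third-person montages, applies SetByCaller damage and executes the fire cue.
; Hit markers check only the first hit, flagging kills when that character's health is near zero.
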(event `self.K2_ActivateAbility`
  (`self.CheckAndSetupCacheables`)
  (`ATA_Trace.ResetSpread` (`self.LineTraceTargetActor`))
  ;[1 1 1] Tell the Server to wait for Replicated TargetData.
  ; Clien Returns from Task's Activate().
  ; If the Player is the Server (HOST), This wont do anything since the Data is never RPC'd and bullet is handled locally on the server
  (bind (_asynctaskproxy _data) (`AT_ServerWaitForClientTargetData.ServerWaitForClientTargetData` "None")
    (:`then`
      (set `self.Server Wait Target Data Task` _asynctaskproxy)
      (`self.FireBullet`))
    (:`ValidData`
      (`self.Handle Target Data` _data)
      (`self.CheckHitMarker` _data))))

(event `FireBullet`
  (bind _linetracetargetactor (`self.LineTraceTargetActor`))
  (`KismetSystemLibrary.PrintString` "Bang")
  (if (`Controller.IsLocalPlayerController` (`.PlayerController` (break `GameplayAbilityActorInfo` (`self.GetActorInfo`))))
    (if (>= (- (`GameplayStatics.GetTimeSeconds`) (`self.Time Of Last Shot`)) (- (`/Game/ShiitakeSorcerers/Weapons/NewWeapons/Shotgun/GA_ShotgunPrimary.TimeBetweenShots` (`self.GA_Primary`)) 0.01))
      (bind _returnvalue (`self.K2_CheckAbilityCost`))
      (if _returnvalue
        (`self.SourceWeapon`
          (:`then`
            (set `self.TraceStartLocation` (make `GameplayAbilityTargetingLocationInfo` "SocketTransform" "0.000000,0.000000,0.000000|0.000000,0.000000,-0.000000|1.000000,1.000000,1.000000" null (`self.Weapon1PMesh`) null "MuzzlePos"))
            (`ATA_LineTrace.Configure` :`self` _linetracetargetactor :`InStartLocation` (`self.TraceStartLocation`) :`InAimingTag` (`self.Aiming Tag`) :`InAimingRemovalTag` (`self.Aiming Removal Tag`) :`InTraceProfile` (struct :`Name` "NoCollision") :`bInDebug` true :`bInTraceFromPlayerViewPoint` true :`bInUseAimingSpreadMod` true :`InBaseSpread` (`self.Weapon Spread`) :`InAimingSpreadMod` (`self.Aiming Spread Mod`) :`InTargetingSpreadIncrement` (`self.Firing Spread Increment`) :`InTargetingSpreadMax` (`self.Firing Spread Max`) :`InNumberOfTraces` 8)
            (bind (_asynctaskproxy _data) (`AT_WaitTargetDataUsingActor.WaitTargetDataWithReusableActor` "None" "Instant" _linetracetargetactor true)
              (:`then`
                (set `self.Time Of Last Shot` (`GameplayStatics.GetTimeSeconds`)))
              (:`ValidData`
                (`self.Handle Target Data` _data))))
          (:`else`))
        (else
          (`self.K2_CancelAbility`))))))

(event `Handle Target Data`
  (params (`Target Data` :type "GameplayAbilityTargetDataHandle Structure"))
  (bind _returnvalue (`self.K2_CommitAbilityCost` false))
  (if _returnvalue
    (`self.PlayAnimations`)
    (bind _returnvalue_2 (`AbilitySystemBlueprintLibrary.AssignTagSetByCallerMagnitude` (`self.MakeOutgoingGameplayEffectSpec` "/Game/ShiitakeSorcerers/Core/Abilities/Shooting/GE_DamageGun.GE_DamageGun_C") (struct :`TagName` "Data.Damage") 8.0))
    (`self.K2_ApplyGameplayEffectSpecToTarget` _returnvalue_2 `Target Data`)
    (bind _returnvalue_3 (`AbilitySystemBlueprintLibrary.GetEffectContext` _returnvalue_2))
    (`AbilitySystemBlueprintLibrary.EffectContextAddHitResult` _returnvalue_3 (`AbilitySystemBlueprintLibrary.GetHitResultFromTargetData` `Target Data`))
    (`self.K2_ExecuteGameplayCueWithParams` (struct :`TagName` "GameplayCue.Weapon.Shotgun.Fire") (`AbilitySystemBlueprintLibrary.MakeGameplayCueParameters` 0.0 0.0 _returnvalue_3))
    (if (`KismetSystemLibrary.IsServer`)
      (`self.CheckHitMarker` `Target Data`))
    (else
      (`self.K2_CancelAbility`))))

(event `CheckHitMarker`
  (params (TargetData :type "GameplayAbilityTargetDataHandle Structure"))
  (bind (_returnvalue_bblockinghit _returnvalue_binitialoverlap _returnvalue_time _returnvalue_distance _returnvalue_location _returnvalue_impactpoint _returnvalue_normal _returnvalue_impactnormal _returnvalue_physmat _returnvalue_hitactor) (`GameplayStatics.BreakHitResult` (`AbilitySystemBlueprintLibrary.GetHitResultFromTargetData` TargetData)))
  ;[1 1 1] HitMarker
  (bind _asfp_character (cast `FP_Character` _returnvalue_hitactor))
  (bind _returnvalue (`FP_Character.GetHealth` _asfp_character))
  (`FP_Character.CreateHitMarker` (`self.OwningPlayer`) (< _returnvalue 0.01)))

(fn `GSApplyCost`
  (params (Handle :type "GameplayAbilitySpecHandle Structure") (ActorInfo :type "GameplayAbilityActorInfo Structure (by ref)") (ActivationInfo :type "GameplayAbilityActivationInfo Structure"))
  (bind _asbweapon (cast `BWeapon` (`self.K2_GetSourceObject` Handle ActorInfo)))
  (if (not (`BWeapon.HasInfiniteAmmo` _asbweapon))
    (`BWeapon.SetPrimaryClipAmmo` _asbweapon (- (`BWeapon.GetPrimaryClipAmmo` _asbweapon) (`self.AmmoCost`))))
  (return))

(fn `GSCheckCost`
  (params (Handle :type "GameplayAbilitySpecHandle Structure") (ActorInfo :type "GameplayAbilityActorInfo Structure (by ref)"))
  (returns (ReturnValue :type Boolean))
  (bind _asbweapon (cast `BWeapon` (`self.K2_GetSourceObject` Handle ActorInfo)))
  (if (and (or (>= (`BWeapon.GetPrimaryClipAmmo` _asbweapon) (`self.AmmoCost`)) (`BWeapon.HasInfiniteAmmo` _asbweapon)) (`parent.GSCheckCost` Handle ActorInfo))
    (return true)
    (else
      (`KismetSystemLibrary.PrintText` "no shoot")
      (return false))))

(fn `K2_CanActivateAbility`
  (params (ActorInfo :type "GameplayAbilityActorInfo Structure") (Handle :type "GameplayAbilitySpecHandle Structure"))
  (returns (RelevantTags :type "GameplayTagContainer Structure") (ReturnValue :type Boolean))
  (bind _ga_primary (`self.GA_Primary`)
    (:`then`
      (if (>= (`KismetMathLibrary.Abs` (- (`GameplayStatics.GetTimeSeconds`) (`self.Time Of Last Shot`))) (`/Game/ShiitakeSorcerers/Weapons/NewWeapons/Shotgun/GA_ShotgunPrimary.TimeBetweenShots` _ga_primary))
        _
        (else
          (return (struct) false))))
    (:`else`
      _))
  (return (struct) true))