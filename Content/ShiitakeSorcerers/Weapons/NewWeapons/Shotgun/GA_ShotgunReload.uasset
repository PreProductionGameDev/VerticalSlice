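; Gameplay ability that reloads the shotgun, allowed only when the clip is not full and reserve ammo remains.
; It caches the source weapon and owning character, plays the Reload montage section on the first-person weapon mesh, then waits a fixed delay rather than montage completion.
; It moves the missing rounds, capped by reserve, deducting reserve through a SetByCaller gameplay effect and setting the clip directly on the weapon.
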(event `self.K2_ActivateAbility`
  (bind _sourceweapon (`self.SourceWeapon`))
  (bind _returnvalue (`FP_Character.GetPrimaryReserveAmmo` (`self.OwningPlayer`)))
  (`self.CheckAndCacheDefaults`)
  (bind _sourceweapon_2 (`self.SourceWeapon`)
    (:`then`
      (`|PlayMontage` (`BWeapon.GetWeaponMesh1P` (`self.SourceWeapon`)) "/Game/ShiitakeSorcerers/Weapons/Shotgun/Animations/AM_Weapon_Shotgun.AM_Weapon_Shotgun" 1.0 0.0 "Reload"
        (:`then`
          (`KismetSystemLibrary.Delay` 0.72)
          (bind _output_get (set `self.AmountWantedToReload` (- (`BWeapon.GetMaxPrimaryClipAmmo` _sourceweapon_2) (`BWeapon.GetPrimaryClipAmmo` _sourceweapon_2))))
          (if (<= _output_get _returnvalue)
            (set `self.AmountCanReload` (`self.AmountWantedToReload`))
            (else
              (set `self.AmountCanReload` _returnvalue)))
          (bind _returnvalue_2 (`AbilitySystemBlueprintLibrary.AssignTagSetByCallerMagnitude` (`self.MakeOutgoingGameplayEffectSpec` "/Game/ShiitakeSorcerers/Weapons/NewWeapons/Shotgun/GE_ShotgunChangeAmmo.GE_ShotgunChangeAmmo_C") (struct :`TagName` "Data.ReloadAmount.Reserve") (`KismetMathLibrary.Conv_IntToDouble` (* (`self.AmountCanReload`) -1))))
          (`self.K2_ApplyGameplayEffectSpecToTarget` _returnvalue_2 (`AbilitySystemBlueprintLibrary.AbilityTargetDataFromActor` (`self.OwningPlayer`)))
          (`BWeapon.SetPrimaryClipAmmo` _sourceweapon (+ (`BWeapon.GetPrimaryClipAmmo` _sourceweapon) (`self.AmountCanReload`)))
          (`self.K2_EndAbility`))))
    (:`else`
      (`KismetSystemLibrary.PrintString` "ShotgunReload Weapon Invalid")
      (`self.K2_EndAbility`))))

(fn `K2_CanActivateAbility`
  (params (ActorInfo :type "GameplayAbilityActorInfo Structure") (Handle :type "GameplayAbilitySpecHandle Structure"))
  (returns (RelevantTags :type "GameplayTagContainer Structure") (ReturnValue :type Boolean))
  (bind _asfp_character (cast `FP_Character` (`.AvatarActor` (break `GameplayAbilityActorInfo` ActorInfo))))
  (return (struct) (and (< (`FP_Character.GetPrimaryClipAmmo` _asfp_character) (`FP_Character.GetMaxPrimaryClipAmmo` _asfp_character)) (> (`FP_Character.GetPrimaryReserveAmmo` _asfp_character) 0))))