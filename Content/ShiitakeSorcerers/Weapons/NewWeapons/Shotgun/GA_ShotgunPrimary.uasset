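; Primary fire ability for the shotgun that keeps firing while input is held.
; It caches the source weapon, its ammo cost and shot interval, and the GA_ShotgunPrimaryInstant instance, which it activates through a batched RPC.
; A delay loop calls FireBullet on that instance until release or a failed cost check ends both abilities.
; The cost check requires enough clip or infinite ammo, otherwise it triggers automatic reload.
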(event `self.K2_ActivateAbility`
  (`self.CheckAndSetupCacheables`)
  (bind _returnvalue (`self.BatchRPCTryActivateAbility` (`self.InstantAbilityHandle`)))
  (if _returnvalue
    (`AbilityTask_WaitInputRelease.WaitInputRelease` true
      (:`then`
        (`AbilityTask_WaitDelay.WaitDelay` (`self.TimeBetweenShots`) :!label _label
          (:`OnFinish`
            (bind _returnvalue_2 (`self.K2_CheckAbilityCost`))
            (if _returnvalue_2
              (`/Game/ShiitakeSorcerers/Weapons/NewWeapons/Shotgun/GA_ShotgunPrimaryInstant.FireBullet` (`self.InstantAbility`))
              (goto _label)
              (else
                _)))))
      (:`OnRelease`
        _))
    (`self.K2_EndAbility` (`self.InstantAbility`))
    (`self.K2_EndAbility`)
    (else
      (`self.K2_EndAbility`))))

(fn `GSCheckCost`
  (params (Handle :type "GameplayAbilitySpecHandle Structure") (ActorInfo :type "GameplayAbilityActorInfo Structure (by ref)"))
  (returns (ReturnValue :type Boolean))
  (bind _asbweapon (cast `BWeapon` (`self.K2_GetSourceObject` Handle ActorInfo)))
  (if (and (or (>= (`BWeapon.GetPrimaryClipAmmo` _asbweapon) (`self.AmmoCost`)) (`BWeapon.HasInfiniteAmmo` _asbweapon)) (`parent.GSCheckCost` Handle ActorInfo))
    (return true)
    (else
      ;[1 1 1] Automated Reload Ability
      (`AbilitySystemComponent.TryActivateAbilitiesByTag` (`.AbilitySystemComponent` (break `GameplayAbilityActorInfo` ActorInfo)) (`BlueprintGameplayTagLibrary.MakeGameplayTagContainerFromArray` (`|MakeArray` (struct :`TagName` "Ability.Weapon.Reload") :!type "GameplayTag Structure")) true)
      (return false))))