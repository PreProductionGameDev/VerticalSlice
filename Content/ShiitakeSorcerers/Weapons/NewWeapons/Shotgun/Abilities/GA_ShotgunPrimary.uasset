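; Shotgun primary fire gameplay ability that handles held-trigger firing for the weapon that granted it.
; It caches the weapon and GA_ShotgunPrimaryInstant, activates that predicted ability via batched RPC, then loops FireBullet on the weapon's shot interval until release or failed cost.
; If activation fails within the shot interval, it waits out the remainder and retries, handling early release.
; The cost check requires clip or infinite ammo and triggers the reload ability on failure.
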(event `self.K2_ActivateAbility`
  (bind _timebetweenshots (`self.TimeBetweenShots`))
  (bind _returnvalue (- (`GameplayStatics.GetTimeSeconds`) (`/Game/ShiitakeSorcerers/Weapons/NewWeapons/Shotgun/Abilities/GA_ShotgunPrimaryInstant.Time Of Last Shot` (`self.InstantAbility`))))
  ;[0.2188 0.1672 0.4927] Try and Activate the Ability. Will fail if cannot shoot. We have catches to handle this now
  (`self.CheckAndSetupCacheables`)
  (bind _returnvalue_2 (`self.BatchRPCTryActivateAbility` (`self.InstantAbilityHandle`)))
  (if _returnvalue_2
    (`AbilityTask_WaitInputRelease.WaitInputRelease` true :!label _label
      (:`then`
        ;[0.1329 1 0.2254] The Shooting loop. Calls the Instant Ability which is locally predicted
        (`AbilityTask_WaitDelay.WaitDelay` (`self.TimeBetweenShots`) :!label _label_2
          (:`OnFinish`
            (bind _returnvalue_3 (`self.K2_CheckAbilityCost`))
            (if _returnvalue_3
              (`/Game/ShiitakeSorcerers/Weapons/NewWeapons/Shotgun/Abilities/GA_ShotgunPrimaryInstant.FireBullet` (`self.InstantAbility`))
              (goto _label_2)
              (else
                _)))))
      (:`OnRelease`
        _))
    (`self.K2_EndAbility` (`self.InstantAbility`) :!label _label_3)
    (`self.K2_EndAbility`)
    (else
      ;[1 0.2617 0.2478] Calculating the Time for the next shot if under the time between shots
      (if (> _returnvalue _timebetweenshots)
        (`KismetSystemLibrary.PrintString` "FATAL ERROR: I DONT THINK THIS SHOULD OCCUR. IF SEEN MESSAGE STEF :)")
        (else
          ;[0.5663 0.469 1] Waits for the next valid shot, and will try to shoot
          (`AbilityTask_WaitDelay.WaitDelay` (- _timebetweenshots _returnvalue)
            (:`then`
              (`AbilityTask_WaitInputRelease.WaitInputRelease` true ; Will handle releasing Fire before it can shoot again\nEnds the Ability to remove issues
                (:`OnRelease`
                  (goto _label_3))))
            (:`OnFinish`
              (bind _returnvalue_4 (`self.BatchRPCTryActivateAbility` (`self.InstantAbilityHandle`)))
              (if _returnvalue_4
                (goto _label)))))))))

(event `self.K2_OnEndAbility`
  (params (bWasCancelled :type Boolean)))

(fn `GSCheckCost`
  (params (Handle :type "GameplayAbilitySpecHandle Structure") (ActorInfo :type "GameplayAbilityActorInfo Structure (by ref)"))
  (returns (ReturnValue :type Boolean))
  (bind _asbweapon (cast `BWeapon` (`self.K2_GetSourceObject` Handle ActorInfo)))
  (if (and (or (>= (`BWeapon.GetPrimaryClipAmmo` _asbweapon) (`self.AmmoCost`)) (`BWeapon.HasInfiniteAmmo` _asbweapon)) (`parent.GSCheckCost` Handle ActorInfo))
    (return true)
    (else
      ;[1 1 1] Automated Reload Ability
      (`AbilitySystemComponent.TryActivateAbilitiesByTag` (`.AbilitySystemComponent` (break `GameplayAbilityActorInfo` ActorInfo)) (`BlueprintGameplayTagLibrary.MakeGameplayTagContainerFromArray` (`|MakeArray` (struct :`TagName` "Ability.Weapon.Reload") :!type "GameplayTag Structure")) true)
      (return false))))