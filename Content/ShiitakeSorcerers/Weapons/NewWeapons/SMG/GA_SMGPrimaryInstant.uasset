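; Gameplay ability that fires a single SMG shot, rate-limited and recoil-timed through the cached GA_SMGPrimary instance.
; The local client line-traces with the weapon's reusable target actor, applies curve-driven recoil and sends target data to the waiting server.
; Both sides handle that data for prediction, committing cost, applying GE_DamageGun, playing montages and executing the fire cue.
; Cost overrides check and deduct the weapon's clip ammo unless infinite.
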(event `self.K2_ActivateAbility`
  (`self.CheckAndSetUpCachables`)
  (`ATA_Trace.ResetSpread` (`self.LineTraceTargetActor`))
  ;[1 1 1] Tell the Server to wait for Replicated TargetData.
  ; Clien Returns from Task's Activate().
  ; If the Player is the Server (HOST), This wont do anything since the Data is never RPC'd and bullet is handled locally on the server
  (bind (_asynctaskproxy _data) (`AT_ServerWaitForClientTargetData.ServerWaitForClientTargetData` "None")
    (:`then`
      (set `self.Server Wait Target Data Task` _asynctaskproxy)
      ;[1 1 1] Client Fires bullet Immediately
      (`self.Fire Bullet`))
    (:`ValidData`
      (`self.Handle Target Data` _data))))

(event `Fire Bullet`
  (bind _linetracetargetactor (`self.LineTraceTargetActor`))
  (`KismetSystemLibrary.PrintString` "bang")
  (if (`Controller.IsLocalPlayerController` (`.PlayerController` (break `GameplayAbilityActorInfo` (`self.GetActorInfo`))))
    ;[1 1 1] Ensure Bullet only fires when not on cooldown
    (if (>= (- (`GameplayStatics.GetTimeSeconds`) (`self.TimeOfLastShot`)) (- (`/Game/ShiitakeSorcerers/Weapons/NewWeapons/SMG/GA_SMGPrimary.TimeBetweenShots` (`self.GA_Primary`)) 0.01))
      (bind _returnvalue (`self.K2_CheckAbilityCost`))
      (if _returnvalue
        (`self.SourceWeapon`
          (:`then`
            ;[1 1 1] Configure AbilityTargetActor Linetrace
            (set `self.TraceStartLocation` (make `GameplayAbilityTargetingLocationInfo` "SocketTransform" "0.000000,0.000000,0.000000|0.000000,0.000000,-0.000000|1.000000,1.000000,1.000000" null (`self.Weapon1PMesh`) null "MuzzlePos"))
            (`ATA_LineTrace.Configure` :`self` _linetracetargetactor :`InStartLocation` (`self.TraceStartLocation`) :`InAimingTag` (`self.Aiming Tag`) :`InAimingRemovalTag` (`self.Aiming Removal Tag`) :`InTraceProfile` (struct :`Name` "NoCollision") :`bInDebug` true :`bInTraceFromPlayerViewPoint` true :`bInUseAimingSpreadMod` true :`InBaseSpread` (`self.Weapon Spread`) :`InAimingSpreadMod` (`self.Aiming Spread Mod`) :`InTargetingSpreadIncrement` (`self.Firing Spread Increment`) :`InTargetingSpreadMax` (`self.Firing Spread Max`))
            ;[1 1 1] RPC TargetData to Server
            (bind (_asynctaskproxy _data) (`AT_WaitTargetDataUsingActor.WaitTargetDataWithReusableActor` "None" "Instant" _linetracetargetactor true)
              (:`then`
                (set `self.TimeOfLastShot` (`GameplayStatics.GetTimeSeconds`))
                (`self.Recoil`))
              (:`ValidData`
                ;[1 1 1] Handle Local Shot Prediction
                (`self.Handle Target Data` _data))))
          (:`else`
            (`KismetSystemLibrary.PrintString` "Error: GA_SMGPrimaryInstant FireBullet SMG is NULL")))
        (else
          (`self.K2_CancelAbility`))))))

(event `Handle Target Data`
  (params (`Target Data` :type "GameplayAbilityTargetDataHandle Structure"))
  ;[1 1 1] Handles a Fired Bullet (Called when Server Recieves TargetData or Client fires a bullet). Server will apply damage. ExecutionCalcs run ServerSide only
  (bind _returnvalue (`self.K2_CommitAbilityCost` false))
  (if _returnvalue
    ;;[1 0 0.02448] Add Firing Animations here
    (`self.PlayAnimations`)
    (bind _returnvalue_2 (`AbilitySystemBlueprintLibrary.AssignTagSetByCallerMagnitude` (`self.MakeOutgoingGameplayEffectSpec` "/Game/ShiitakeSorcerers/Core/Abilities/Shooting/GE_DamageGun.GE_DamageGun_C") (struct :`TagName` "Data.Damage") 10.0))
    (`self.K2_ApplyGameplayEffectSpecToTarget` _returnvalue_2 `Target Data`)
    (bind _returnvalue_3 (`AbilitySystemBlueprintLibrary.GetEffectContext` _returnvalue_2))
    (`AbilitySystemBlueprintLibrary.EffectContextAddHitResult` _returnvalue_3 (`AbilitySystemBlueprintLibrary.GetHitResultFromTargetData` `Target Data`))
    (`self.K2_ExecuteGameplayCueWithParams` (struct :`TagName` "GameplayCue.Weapon.SMG.Fire") (`AbilitySystemBlueprintLibrary.MakeGameplayCueParameters` 0.0 0.0 _returnvalue_3))
    (else
      (`self.K2_CancelAbility`))))

(fn `GSApplyCost`
  (params (Handle :type "GameplayAbilitySpecHandle Structure") (ActorInfo :type "GameplayAbilityActorInfo Structure (by ref)") (ActivationInfo :type "GameplayAbilityActivationInfo Structure"))
  (bind _asbweapon (cast `BWeapon` (`self.K2_GetSourceObject` Handle ActorInfo)))
  (if (not (`BWeapon.HasInfiniteAmmo` _asbweapon))
    (`BWeapon.SetPrimaryClipAmmo` _asbweapon (- (`BWeapon.GetPrimaryClipAmmo` _asbweapon) (`self.AmmoCost`))))
  (return))

(fn `GSCheckCost`
  (params (Handle :type "GameplayAbilitySpecHandle Structure") (ActorInfo :type "GameplayAbilityActorInfo Structure (by ref)"))
  (returns (ReturnValue :type Boolean))
  (bind _asbweapon (cast `BWeapon` (`self.K2_GetSourceObject` Handle ActorInfo)))
  (if (and (or (>= (`BWeapon.GetPrimaryClipAmmo` _asbweapon) (`self.AmmoCost`)) (`BWeapon.HasInfiniteAmmo` _asbweapon)) (`parent.GSCheckCost` Handle ActorInfo))
    (return true)
    (else
      (`KismetSystemLibrary.PrintText` "no shoot")
      (return false))))

(fn `K2_CanActivateAbility`
  (params (ActorInfo :type "GameplayAbilityActorInfo Structure") (Handle :type "GameplayAbilitySpecHandle Structure"))
  (returns (RelevantTags :type "GameplayTagContainer Structure") (ReturnValue :type Boolean))
  (bind _ga_primary (`self.GA_Primary`)
    (:`then`
      (if (>= (`KismetMathLibrary.Abs` (- (`GameplayStatics.GetTimeSeconds`) (`self.TimeOfLastShot`))) (`/Game/ShiitakeSorcerers/Weapons/NewWeapons/SMG/GA_SMGPrimary.TimeBetweenShots` _ga_primary))
        _
        (else
          (return (struct) false))))
    (:`else`
      _))
  (return (struct) true))

(fn `Recoil`
  (bind _owningplayer (`self.OwningPlayer`))
  (bind _ga_primary (`self.GA_Primary`))
  (bind (_returnvalue_x _returnvalue_y) (`KismetMathLibrary.BreakVector` (`CurveVector.GetVectorValue` (`BWeapon.GetRecoilPattern` (`self.SourceWeapon`)) (`/Game/ShiitakeSorcerers/Weapons/NewWeapons/SMG/GA_SMGPrimary.StepBeforeRecoilTime` (`self.GA_Primary`)))))
  (bind (_returnvalue_x_2 _returnvalue_y_2) (`KismetMathLibrary.BreakVector` (`CurveVector.GetVectorValue` (`BWeapon.GetRecoilPattern` (`self.SourceWeapon`)) (`/Game/ShiitakeSorcerers/Weapons/NewWeapons/SMG/GA_SMGPrimary.RecoilTime` (`self.GA_Primary`)))))
  (set `/Game/ShiitakeSorcerers/Weapons/NewWeapons/SMG/GA_SMGPrimary.StepBeforeRecoilTime` (- (`/Game/ShiitakeSorcerers/Weapons/NewWeapons/SMG/GA_SMGPrimary.RecoilTime` (`self.GA_Primary`)) (`BWeapon.GetTimeBetweenShots` (`self.SourceWeapon`))) (`self.GA_Primary`))
  (`Pawn.AddControllerPitchInput` _owningplayer (- _returnvalue_y _returnvalue_y_2))
  (`Pawn.AddControllerYawInput` _owningplayer (- _returnvalue_x _returnvalue_x_2))
  (set `/Game/ShiitakeSorcerers/Weapons/NewWeapons/SMG/GA_SMGPrimary.RecoilTime` (+ (`/Game/ShiitakeSorcerers/Weapons/NewWeapons/SMG/GA_SMGPrimary.RecoilTime` _ga_primary) (`/Game/ShiitakeSorcerers/Weapons/NewWeapons/SMG/GA_SMGPrimary.TimeBetweenShots` _ga_primary)) _ga_primary))