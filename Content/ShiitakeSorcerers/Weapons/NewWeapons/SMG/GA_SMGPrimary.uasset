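; SMG primary fire gameplay ability that handles full-auto shooting while the trigger is held, ending immediately in other fire modes.
; It caches the source weapon plus the GA_SMGPrimaryInstant handle and instance, then activates that ability through a batched RPC without ending it.
; A WaitDelay loop calls FireBullet on the instant ability after each shot interval while cost checks pass.
; Trigger release or a failed cost check ends both abilities.
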(event `self.K2_ActivateAbility`
  (`KismetSystemLibrary.PrintString` "pog")
  (`self.CheckAndSetUpCacheables`)
  (if (== (`BWeapon.FireMode` (`self.SourceWeapon`)) (struct :`TagName` "Weapon.SMG.FireMode.FullAuto"))
    (bind _returnvalue (`self.BatchRPCTryActivateAbility` (`self.InstantAbilityHandle`)))
    (if _returnvalue
      ;[1 1 1] End Both Abilities when Releasing the Trigger
      (`AbilityTask_WaitInputRelease.WaitInputRelease` true
        (:`then`
          ;[1 1 1] Continously Fire a Bullet
          (`AbilityTask_WaitDelay.WaitDelay` (`self.TimeBetweenShots`) :!label _label
            (:`OnFinish`
              (bind _returnvalue_2 (`self.K2_CheckAbilityCost`))
              (if _returnvalue_2
                (`/Game/ShiitakeSorcerers/Weapons/NewWeapons/SMG/GA_SMGPrimaryInstant.Fire Bullet` (`self.InstantAbility`))
                (goto _label)
                (else
                  _)))))
        (:`OnRelease`
          _))
      (`self.K2_EndAbility` (`self.InstantAbility`))
      (`self.K2_EndAbility`)
      (else
        (`self.K2_EndAbility`)))
    (else
      (`self.K2_EndAbility`))))