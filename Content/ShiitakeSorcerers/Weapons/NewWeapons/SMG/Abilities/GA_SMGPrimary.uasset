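; Gameplay Ability for the SMG's primary fire, which only runs when the weapon is in full-auto mode.
; It batch-RPC activates the cached GA_SMGPrimaryInstant ability, then loops on a delay calling its FireBullet until trigger release or a failed cost check ends both.
; The cost check tries to activate Reload when ammo is short.
; A cooldown timer follows firing for recoil reset, and resumed fire clears it and recalculates RecoilTime.
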(event `self.K2_ActivateAbility`
  (`self.CheckAndSetUpCacheables`)
  (if (== (`BWeapon.FireMode` (`self.SourceWeapon`)) (struct :`TagName` "Weapon.SMG.FireMode.FullAuto"))
    (bind _returnvalue (`self.BatchRPCTryActivateAbility` (`self.InstantAbilityHandle`)))
    (if _returnvalue
      ;[1 1 1] End Both Abilities when Releasing the Trigger
      (`AbilityTask_WaitInputRelease.WaitInputRelease` true
        (:`then`
          ;[1 1 1] Continously Fire a Bullet
          (`AbilityTask_WaitDelay.WaitDelay` (`self.TimeBetweenShots`) :!label _label
            (:`OnFinish`
              (bind _returnvalue_2 (`self.K2_CheckAbilityCost`))
              (if _returnvalue_2
                (`self.CheckRecoilStopped`)
                (`/Game/ShiitakeSorcerers/Weapons/NewWeapons/SMG/Abilities/GA_SMGPrimaryInstant.Fire Bullet` (`self.InstantAbility`))
                (goto _label)
                (else
                  _)))))
        (:`OnRelease`
          _))
      (`self.K2_EndAbility` (`self.InstantAbility`))
      (`self.K2_EndAbility`)
      (bind _returnvalue_3 (`KismetSystemLibrary.K2_SetTimerDelegate` (`|CreateDelegate` :!event `ResetTheRecoil`) (`BWeapon.GetRecoilCooldown` (`self.SourceWeapon`))))
      (set `self.ResetRecoilHandle` _returnvalue_3)
      (else
        (`self.K2_EndAbility`)))
    (else
      (`self.K2_EndAbility`))))

(event `ResetTheRecoil`
  (set `self.RecoilTime` 0.0))

(event `CheckRecoilStopped`
  (bind _resetrecoilhandle (`self.ResetRecoilHandle`))
  (if (`KismetSystemLibrary.K2_TimerExistsHandle` _resetrecoilhandle)
    (set `self.RecoilTime` (/ (`KismetSystemLibrary.K2_GetTimerElapsedTimeHandle` _resetrecoilhandle) (`self.RecoilTime`)))
    (`KismetSystemLibrary.K2_ClearAndInvalidateTimerHandle` (`self.ResetRecoilHandle`))))

(fn `GSCheckCost`
  (params (Handle :type "GameplayAbilitySpecHandle Structure") (ActorInfo :type "GameplayAbilityActorInfo Structure (by ref)"))
  (returns (ReturnValue :type Boolean))
  (bind _asbweapon (cast `BWeapon` (`self.K2_GetSourceObject` Handle ActorInfo)))
  (if (and (or (>= (`BWeapon.GetPrimaryClipAmmo` _asbweapon) (`self.AmmoCost`)) (`BWeapon.HasInfiniteAmmo` _asbweapon)) (`parent.GSCheckCost` Handle ActorInfo))
    (return true)
    (else
      ;[1 1 1] Activate Reload Ability
      (`AbilitySystemComponent.TryActivateAbilitiesByTag` (`.AbilitySystemComponent` (break `GameplayAbilityActorInfo` ActorInfo)) (`BlueprintGameplayTagLibrary.MakeGameplayTagContainerFromArray` (`|MakeArray` (struct :`TagName` "Ability.Weapon.Reload") :!type "GameplayTag Structure")) true)
      (return false))))