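; Gameplay ability for the sniper's secondary action: a hold-to-scope zoom on the first-person camera.
; On activation it caches the owning character and source weapon, uses WaitChangeFOV to narrow the view, and shows a scope widget for the locally controlled player.
; Releasing input tweens the FOV back, then removes the widget and ends the ability.
; OnEndAbility also resets FOV and removes the scope, covering endings before release.
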(event `self.K2_ActivateAbility`
  (bind _scopewidget (`self.ScopeWidget`))
  ;[1 1 1] Cache Variables
  (`self.OwningPlayer`
    (:`then`
      _)
    (:`else`
      (bind _asbp_fpcharacter (cast `/Game/ShiitakeSorcerers/Character/BP_FPCharacter` (`self.GetAvatarActorFromActorInfo`)))
      (set `self.OwningPlayer` _asbp_fpcharacter)))
  (`self.SourceWeapon`
    (:`then`
      _)
    (:`else`
      (bind _asbweapon (cast `BWeapon` (`self.GetCurrentSourceObject`)))
      (set `self.SourceWeapon` _asbweapon)))
  ;[1 1 1] Set FOV
  (`AT_LerpChangeFOV.WaitChangeFOV` "None" (`FP_Character.FirstPersonCameraComponent` (`self.OwningPlayer`)) 30.0 0.1
    (:`then`
      ;[1 1 1] Add the Scope Widet if Locally Controlled
      (`self.IsLocallyControlled`
        (:`True`
          (bind _returnvalue (`|CreateWidget` "/Game/ShiitakeSorcerers/UI/SniperScope/WB_SniperScope.WB_SniperScope_C"))
          (bind _output_get (set `self.ScopeWidget` _returnvalue))
          (`UserWidget.AddToViewport` _output_get 0))
        (:`False`
          _))
      (`AbilityTask_WaitInputRelease.WaitInputRelease` true
        (:`OnRelease`
          (`AT_LerpChangeFOV.WaitChangeFOV` "None" (`FP_Character.FirstPersonCameraComponent` (`self.OwningPlayer`)) 90.0 0.1
            (:`OnTargetFOVReached`
              (`self.IsLocallyControlled`
                (:`True`
                  (`/Engine/EditorBlueprintResources/StandardMacros.IsValid` _scopewidget
                    (:`Is Valid`
                      (`Widget.RemoveFromParent` _scopewidget)
                      (`self.K2_EndAbility`))
                    (:`Is Not Valid`
                      (`self.K2_EndAbility` :!label _label))))
                (:`False`
                  (goto _label))))))))))

(event `self.K2_OnEndAbility`
  (params (bWasCancelled :type Boolean))
  (bind _scopewidget (`self.ScopeWidget`))
  ;[1 1 1] Ends Ability if done before releasing input
  (`CameraComponent.SetFieldOfView` (`FP_Character.FirstPersonCameraComponent` (`self.OwningPlayer`)) 90.0)
  (`/Engine/EditorBlueprintResources/StandardMacros.IsValid` _scopewidget
    (:`Is Valid`
      (`Widget.RemoveFromParent` _scopewidget))))