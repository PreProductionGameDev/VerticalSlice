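; Burst rifle secondary-fire gameplay ability that zooms the player into a sniper scope.
; On activation it applies an aiming effect, tweens the camera FOV in, hides the first-person weapon mesh and swaps the crosshair for a scope widget on the local player.
; The HoldToZoom setting decides whether input release or another press zooms out and ends the ability.
; Ending restores FOV, mesh and crosshair, and clears the scope and aiming effects.
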(event `self.K2_ActivateAbility`
  (bind _scopewidget (`self.ScopeWidget`))
  ;[1 1 1] Cache Variables
  (`self.OwningPlayer`
    (:`then`
      _)
    (:`else`
      (bind _asbp_fpcharacter (cast `/Game/ShiitakeSorcerers/Character/BP_FPCharacter` (`self.GetAvatarActorFromActorInfo`)))
      (set `self.OwningPlayer` _asbp_fpcharacter)))
  (`self.SourceWeapon`
    (:`then`
      _)
    (:`else`
      (bind _asbweapon (cast `BWeapon` (`self.GetCurrentSourceObject`)))
      (set `self.SourceWeapon` _asbweapon)))
  (bind _returnvalue (`self.BP_ApplyGameplayEffectToOwner` "/Game/ShiitakeSorcerers/Weapons/NewWeapons/Sniper/Abilities/GameplayEffects/GE_SniperAimingAdd.GE_SniperAimingAdd_C" (`self.GetAbilityLevel`)))
  (set `self.AimingEffectHandle` _returnvalue)
  ;[1 1 1] Set FOV
  (`AT_LerpChangeFOV.WaitChangeFOV` "None" (`FP_Character.FirstPersonCameraComponent` (`self.OwningPlayer`)) 45.0 0.1
    (:`then`
      (`SceneComponent.SetVisibility` (`BWeapon.GetWeaponMesh1P` (`self.SourceWeapon`)) false false)
      (`self.IsLocallyControlled`
        (:`True`
          ;[1 1 1] Add the Scope Widet if Locally Controlled
          (`PlayerHUD.ToggleCrosshair` (`FP_Character.GetPlayerHUD` (`self.OwningPlayer`)) false)
          (bind _returnvalue_2 (`|CreateWidget` "/Game/ShiitakeSorcerers/UI/Game/SniperScope/WB_SniperScope.WB_SniperScope_C"))
          (bind _output_get (set `self.ScopeWidget` _returnvalue_2))
          (`UserWidget.AddToViewport` _output_get 0))
        (:`False`
          _))
      (bind _asgi_multiplayer (cast `GI_Multiplayer` (`GameplayStatics.GetGameInstance`)))
      (if (`SettingsSaveGame.bHoldToZoom` (`GI_Multiplayer.Settings` _asgi_multiplayer))
        (`AbilityTask_WaitInputRelease.WaitInputRelease` true
          (:`OnRelease`
            _))
        (else
          (`AbilityTask_WaitInputPress.WaitInputPress` false
            (:`OnPress`
              _))))
      (`AT_LerpChangeFOV.WaitChangeFOV` "None" (`FP_Character.FirstPersonCameraComponent` (`self.OwningPlayer`)) 90.0 0.1
        (:`OnTargetFOVReached`
          (`SceneComponent.SetVisibility` (`BWeapon.GetWeaponMesh1P` (`self.SourceWeapon`)) true false)
          (`self.IsLocallyControlled`
            (:`True`
              (`/Engine/EditorBlueprintResources/StandardMacros.IsValid` _scopewidget
                (:`Is Valid`
                  (`Widget.RemoveFromParent` _scopewidget)
                  (`self.K2_EndAbility`))
                (:`Is Not Valid`
                  (`self.K2_EndAbility` :!label _label))))
            (:`False`
              (goto _label))))))))

(event `self.K2_OnEndAbility`
  (params (bWasCancelled :type Boolean))
  (bind _scopewidget (`self.ScopeWidget`))
  (bind _returnvalue (`FP_Character.GetPlayerHUD` (`self.OwningPlayer`)))
  (`/Engine/EditorBlueprintResources/StandardMacros.IsValid` _returnvalue
    (:`Is Valid`
      (`PlayerHUD.ToggleCrosshair` _returnvalue true))
    (:`Is Not Valid`
      _))
  (bind _returnvalue_2 (`AbilitySystemBlueprintLibrary.GetActiveGameplayEffectStackCount` (`self.AimingEffectHandle`)))
  (if (not (> _returnvalue_2 0))
    (bind _returnvalue_3 (`self.BP_ApplyGameplayEffectToOwner` "/Game/ShiitakeSorcerers/Weapons/NewWeapons/Sniper/Abilities/GameplayEffects/GE_SniperAimingRemoval.GE_SniperAimingRemoval_C" (`self.GetAbilityLevel`)))
    (set `self.Remove Aiming Effect Handle` _returnvalue_3))
  (`self.BP_RemoveGameplayEffectFromOwnerWithHandle` (`self.AimingEffectHandle`))
  (`self.BP_RemoveGameplayEffectFromOwnerWithHandle` (`self.Remove Aiming Effect Handle`))
  (`SceneComponent.SetVisibility` (`BWeapon.GetWeaponMesh1P` (`self.SourceWeapon`)) true false)
  ;[1 1 1] Ends Ability if done before releasing input
  (`CameraComponent.SetFieldOfView` (`FP_Character.FirstPersonCameraComponent` (`self.OwningPlayer`)) 90.0)
  (`/Engine/EditorBlueprintResources/StandardMacros.IsValid` _scopewidget
    (:`Is Valid`
      (`Widget.RemoveFromParent` _scopewidget))))