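; Team deathmatch game mode for Red and Blue teams, ending when either reaches 20 kills.
; Players join a chosen, random or smaller team, then get a character with team flags and gameplay tag, placed at a team-tagged spawn volume or fallback PlayerStart.
; Per-player kill maps keyed by name are summed into team scores on each kill, driving lead-change notifications, the win check and the leaderboard sent to clients.
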(event `self.ReceiveBeginPlay`
  (`parent.ReceiveBeginPlay`))

(event `/Game/ShiitakeSorcerers/Core/GamemodeInterface.PlayerScored`
  (params (KillerName :type String) (KilledName :type String) (WeaponIcon :type "Texture2D Object Reference"))
  (bind _blueteamscore (`self.BlueTeamScore`))
  (bind _redteamscore (`self.RedTeamScore`))
  (bind (_value _returnvalue) (`BlueprintMapLibrary.Map_Find` (`self.RedTeamMap`) KillerName))
  (`parent.PlayerScored` KillerName KilledName WeaponIcon)
  (if _returnvalue
    (`BlueprintMapLibrary.Map_Add` (`self.RedTeamMap`) KillerName (+ _value 1))
    (set `self.RedTeamScore` 0)
    (bind _values (`BlueprintMapLibrary.Map_Values` (`self.RedTeamMap`)))
    (for _array_element _values
      (set `self.RedTeamScore` (+ _array_element _redteamscore)))
    (`self.PointCheck`)
    (if (>= _redteamscore 20)
      (`/Game/ShiitakeSorcerers/Core/GamemodeInterface.GameOver`))
    (else
      (`BlueprintMapLibrary.Map_Add` (`self.BlueTeamMap`) KillerName (+ (`BlueprintMapLibrary.Map_Find` (`self.BlueTeamMap`) KillerName) 1))
      (set `self.BlueTeamScore` 0)
      (bind _values_2 (`BlueprintMapLibrary.Map_Values` (`self.BlueTeamMap`)))
      (for _array_element_2 _values_2
        (set `self.BlueTeamScore` (+ _array_element_2 _blueteamscore)))
      (`self.PointCheck`)
      (if (>= _blueteamscore 20)
        (`/Game/ShiitakeSorcerers/Core/GamemodeInterface.GameOver`)))))

(event `self.K2_PostLogin`
  (params (NewPlayer :type "PlayerController Object Reference"))
  (`parent.K2_PostLogin` NewPlayer))

(event `self.HandleStartingNewPlayer`
  (params (NewPlayer :type "PlayerController Object Reference"))
  (`parent.HandleStartingNewPlayer` NewPlayer))

(event `self.K2_OnLogout`
  (params (ExitingController :type "Controller Object Reference"))
  (bind _returnvalue (`PlayerState.GetPlayerName` (`Controller.PlayerState` ExitingController)))
  (`parent.K2_OnLogout` ExitingController)
  (`BlueprintMapLibrary.Map_Remove` (`self.RedTeamMap`) _returnvalue)
  (`BlueprintMapLibrary.Map_Remove` (`self.BlueTeamMap`) _returnvalue))

(event `/Game/ShiitakeSorcerers/Core/GamemodeInterface.RedTeam`
  (params (Controller :type "Controller Object Reference"))
  (`BlueprintMapLibrary.Map_Add` (`self.RedTeamMap`) (`PlayerState.GetPlayerName` (`Controller.PlayerState` Controller)))
  (`self.SpawnPlayer` Controller (struct :`TagName` "Team.Red")))

(event `SpawnPlayer`
  (params (Controller :type "Controller Object Reference") (TeamTag :type "GameplayTag Structure"))
  (bind _outactors (`GameplayStatics.GetAllActorsOfClass` "/Script/Engine.PlayerStart"))
  (bind _returnvalue (`|SpawnActorFromClass` "/Game/ShiitakeSorcerers/Character/BP_FPCharacter.BP_FPCharacter_C" (`self.GetTransform` (`KismetArrayLibrary.Array_Random` _outactors)) "Undefined" "OverrideRootScale" null null))
  (`Controller.Possess` Controller _returnvalue)
  (`/Game/ShiitakeSorcerers/Character/BP_FPCharacter.ClientLoadCosmetcs` _returnvalue)
  (set `/Game/ShiitakeSorcerers/Character/BP_FPCharacter.Red` (== TeamTag (struct :`TagName` "Team.Red")) _returnvalue)
  (set `/Game/ShiitakeSorcerers/Character/BP_FPCharacter.Blue` (== TeamTag (struct :`TagName` "Team.Blue")) _returnvalue)
  (`AbilitySystemBlueprintLibrary.AddLooseGameplayTags` _returnvalue (`BlueprintGameplayTagLibrary.MakeGameplayTagContainerFromArray` (`|MakeArray` TeamTag)))
  (`/Game/ShiitakeSorcerers/Core/GamemodeInterface.Respawn` _returnvalue))

(event `/Game/ShiitakeSorcerers/Core/GamemodeInterface.BlueTeam`
  (params (Controller :type "Controller Object Reference"))
  (`BlueprintMapLibrary.Map_Add` (`self.BlueTeamMap`) (`PlayerState.GetPlayerName` (`Controller.PlayerState` Controller)))
  (`self.SpawnPlayer` Controller (struct :`TagName` "Team.Blue")))

(event `/Game/ShiitakeSorcerers/Core/GamemodeInterface.Random`
  (params (Controller :type "Controller Object Reference"))
  (bind _returnvalue (`BlueprintMapLibrary.Map_Length` (`self.BlueTeamMap`)))
  (bind _returnvalue_2 (`BlueprintMapLibrary.Map_Length` (`self.RedTeamMap`)))
  (bind _returnvalue_3 (`PlayerState.GetPlayerName` (`Controller.PlayerState` Controller)))
  (if (> _returnvalue_2 _returnvalue)
    (`BlueprintMapLibrary.Map_Add` (`self.BlueTeamMap`) _returnvalue_3 :!label _label)
    (`self.SpawnPlayer` Controller (struct :`TagName` "Team.Blue"))
    (else
      (if (not (> _returnvalue _returnvalue_2))
        (`|MultiGate` true
          (:`Out 0`
            (goto _label))
          (:`Out 1`
            _)))
      (`BlueprintMapLibrary.Map_Add` (`self.RedTeamMap`) _returnvalue_3)
      (`self.SpawnPlayer` Controller (struct :`TagName` "Team.Red")))))

(fn `FindRespawnPoint`
  (params (PlayerName :type String))
  (returns (SpawnLocation :type "Vector Structure") (SpawnRotation :type "Rotator Structure"))
  (locals (Index :type Integer) (RandomVolume :type "/Game/ShiitakeSorcerers/Core/Map/BP_SpawnVolume Object Reference"))
  (bind _randomvolume (`local.RandomVolume`))
  (bind (_returnvalue_x _returnvalue_y _returnvalue_z) (`KismetMathLibrary.BreakVector` (`SceneComponent.K2_GetComponentLocation` (`/Game/ShiitakeSorcerers/Core/Map/BP_SpawnVolume.LookLocation` _randomvolume))))
  (bind _outactors (`GameplayStatics.GetAllActorsOfClass` "/Game/ShiitakeSorcerers/Core/Map/BP_SpawnVolume.BP_SpawnVolume_C"))
  (if (< (`KismetArrayLibrary.Array_Length` _outactors) 1)
    (bind _outactors_2 (`GameplayStatics.GetAllActorsOfClass` "/Script/Engine.PlayerStart"))
    (if (`.ReturnValue` (`BlueprintMapLibrary.Map_Find` (`self.RedTeamMap`) (`local.PlayerName`)))
      (for (_array_element _array_index) _outactors_2
        (if (== (`PlayerStart.PlayerStartTag` _array_element) "Red")
          (set `local.Index` _array_index)
          (break)))
      (else
        (for (_array_element_2 _array_index_2) _outactors_2
          (if (== (`PlayerStart.PlayerStartTag` _array_element_2) "Blue")
            (set `local.Index` _array_index_2)
            (break)))))
    (bind _output (`|GetArrayItem` _outactors_2 (`local.Index`)))
    (return (`self.K2_GetActorLocation` _output) (`self.K2_GetActorRotation` _output))
    (else
      (if (`.ReturnValue` (`BlueprintMapLibrary.Map_Find` (`self.RedTeamMap`) (`local.PlayerName`)))
        (bind _outitem (`KismetArrayLibrary.Array_Random` _outactors))
        (bind _output_get (set `local.RandomVolume` _outitem :!label _label))
        (if (== (`/Game/ShiitakeSorcerers/Core/Map/BP_SpawnVolume.SpawnTag` _output_get) "Red")
          _
          (else
            (goto _label)))
        (else
          (bind _output_get_2 (set `local.RandomVolume` _outitem :!label _label_2))
          (if (== (`/Game/ShiitakeSorcerers/Core/Map/BP_SpawnVolume.SpawnTag` _output_get_2) "Blue")
            _
            (else
              (goto _label_2)))))
      (bind (_transform _found) (`/Game/ShiitakeSorcerers/Core/Map/BP_SpawnVolume.FindSpawn` _randomvolume :!label _label_3))
      (if _found
        (return _transform (`KismetMathLibrary.MakeRotator` _returnvalue_x _returnvalue_y _returnvalue_z))
        (else
          (goto _label_3))))))

(fn `GetScores`
  (params (PlayerReq :type "/Game/ShiitakeSorcerers/Character/BP_FPCharacter Object Reference"))
  (returns (Return :type Boolean))
  (locals (BluePlayers :type "Array of Name") (BlueScore :type "Array of Integer64"))
  (bind _redteammap (`self.RedTeamMap`))
  (bind _blueteammap (`self.BlueTeamMap`))
  (bind _keys (`BlueprintMapLibrary.Map_Keys` _redteammap))
  (bind _keys_2 (`BlueprintMapLibrary.Map_Keys` _blueteammap))
  (for _array_element _keys_2
    (`KismetArrayLibrary.Array_Add` (`local.BluePlayers`) (`KismetStringLibrary.Conv_StringToName` _array_element)))
  (bind _values (`BlueprintMapLibrary.Map_Values` _redteammap))
  (bind _values_2 (`BlueprintMapLibrary.Map_Values` _blueteammap))
  (for _array_element_2 _values_2
    (`KismetArrayLibrary.Array_Add` (`local.BlueScore`) (`KismetMathLibrary.Conv_IntToInt64` _array_element_2)))
  (`/Game/ShiitakeSorcerers/Character/BP_FPCharacter.ClientTeamDeathMatchLeaderboard` PlayerReq _keys (`local.BluePlayers`) _values (`local.BlueScore`))
  (return false))

(fn `PointCheck`
  (bind _returnvalue (> (`self.RedTeamScore`) (`self.BlueTeamScore`)))
  (bind _outactors (`GameplayStatics.GetAllActorsOfClass` "/Game/ShiitakeSorcerers/Character/BP_FPCharacter.BP_FPCharacter_C"))
  (for _array_element _outactors
    (if (!= _returnvalue (`self.Red Winning`))
      (if (== (`/Game/ShiitakeSorcerers/Character/BP_FPCharacter.Red` _array_element) _returnvalue)
        (`/Game/ShiitakeSorcerers/Character/BP_FPCharacter.ClientTeamLead` _array_element)
        (else
          (`/Game/ShiitakeSorcerers/Character/BP_FPCharacter.ClientTeamLost` _array_element)))
      (set `self.Red Winning` _returnvalue))))

(fn `Respawn`
  (params (Player :type "/Game/ShiitakeSorcerers/Character/BP_FPCharacter Object Reference"))
  (returns (Return :type Boolean))
  (bind (_spawnlocation _spawnrotation) (`self.FindRespawnPoint` (`PlayerState.GetPlayerName` (`Pawn.PlayerState` Player))))
  (`self.K2_SetActorLocation` Player _spawnlocation false true)
  (`/Game/ShiitakeSorcerers/Character/BP_FPCharacter.ClientLookTowards` Player (`KismetMathLibrary.MakeVector` (.roll _spawnrotation) (.pitch _spawnrotation) (.yaw _spawnrotation)))
  (`self.EnableInput` Player null)
  (return false))

(fn `UserConstructionScript`
  (`parent.UserConstructionScript`))