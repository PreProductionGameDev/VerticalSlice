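; Deathmatch game mode for ShiitakeSorcerers that ends the match when a player reaches a score of ten.
; PlayerScored ignores empty killer names, increments the killer's entry in the name-keyed PlayerScores map, re-sorts it with SortScoreBoard, then checks for the win.
; GameOver and Respawn defer to the parent class, and GetScores exposes the sorted score map.
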(event `self.PlayerScored`
  (params (KillerName :type String) (KilledName :type String))
  (if (not (== (`KismetStringLibrary.Len` KillerName) 0))
    (`BlueprintMapLibrary.Map_Add` (`self.PlayerScores`) KillerName (+ (`BlueprintMapLibrary.Map_Find` (`self.PlayerScores`) KillerName) 1))
    (bind _returnvalue (`GI_Multiplayer.SortScoreBoard` (`self.PlayerScores`)))
    (set `self.PlayerScores` _returnvalue)
    (if (>= (`BlueprintMapLibrary.Map_Find` (`self.PlayerScores`) KillerName) 10)
      (`self.GameOver`))))

(event `self.GameOver`
  (`parent.GameOver`))

(fn `GetScores`
  (returns (Scores :type "Map of String to Integer"))
  (return (`self.PlayerScores`)))

(fn `Respawn`
  (params (Player :type "/Game/ShiitakeSorcerers/Character/BP_FPCharacter Object Reference"))
  (returns (Return :type Boolean))
  (bind _return (`parent.Respawn` Player))
  (return _return))

(fn `UserConstructionScript`
  (`parent.UserConstructionScript`))