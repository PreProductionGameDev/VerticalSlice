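; Capture-the-flag game mode, judging by its name, that balances players into Red and Blue teams and handles respawns.
; PostLogin adds player names to the smaller team, breaking ties with a random non-looping MultiGate that fires each output only once.
; Its debug prints label the teams in reverse.
; Respawn teleports players to the last PlayerStart tagged for their team, defaulting non-Red names to Blue, and re-enables input.
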(event `self.K2_PostLogin`
  (params (NewPlayer :type "PlayerController Object Reference"))
  (bind _returnvalue (`BlueprintMapLibrary.Map_Length` (`self.Red Team`)))
  (bind _returnvalue_2 (`BlueprintMapLibrary.Map_Length` (`self.Blue Team`)))
  (bind _returnvalue_3 (`PlayerState.GetPlayerName` (`Controller.PlayerState` NewPlayer)))
  (if (== _returnvalue _returnvalue_2)
    (`|MultiGate` true
      (:`Out 0`
        (`BlueprintMapLibrary.Map_Add` (`self.Blue Team`) _returnvalue_3 :!label _label)
        (`KismetSystemLibrary.PrintString` (`KismetStringLibrary.Concat_StrStr` _returnvalue_3 "red")))
      (:`Out 1`
        (`BlueprintMapLibrary.Map_Add` (`self.Red Team`) _returnvalue_3 :!label _label_2)
        (`KismetSystemLibrary.PrintString` (`KismetStringLibrary.Concat_StrStr` _returnvalue_3 "blue"))))
    (elif (> _returnvalue _returnvalue_2)
      (goto _label)
      (else
        (goto _label_2)))))

(fn `FindRespawnPoint`
  (params (PlayerName :type String))
  (returns (SpawnLocation :type "Vector Structure") (SpawnRotation :type "Rotator Structure"))
  (locals (Index :type Integer :default 0))
  (bind _outactors (`GameplayStatics.GetAllActorsOfClass` "/Script/Engine.PlayerStart"))
  (if (`.ReturnValue` (`BlueprintMapLibrary.Map_Find` (`self.Red Team`) PlayerName))
    (for (_array_element _array_index) _outactors
      (if (== (`PlayerStart.PlayerStartTag` _array_element) "Red")
        (set `local.Index` _array_index)))
    (else
      (for (_array_element_2 _array_index_2) _outactors
        (if (== (`PlayerStart.PlayerStartTag` _array_element_2) "Blue")
          (set `local.Index` _array_index_2)))))
  (bind _output (`|GetArrayItem` _outactors (`local.Index`)))
  (return (`self.K2_GetActorLocation` _output) (`self.K2_GetActorRotation` _output)))

(fn `Respawn`
  (params (Player :type "/Game/ShiitakeSorcerers/Character/BP_FPCharacter Object Reference"))
  (returns (Return :type Boolean))
  (bind (_spawnlocation _spawnrotation) (`self.FindRespawnPoint` (`PlayerState.GetPlayerName` (`Pawn.PlayerState` Player))))
  (`self.K2_SetActorLocationAndRotation` Player _spawnlocation _spawnrotation false true)
  (`self.EnableInput` Player null)
  (return false))

(fn `UserConstructionScript`
  (`parent.UserConstructionScript`))