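; Game mode for what appears to be a first-person test in Shiitake Sorcerers, handling player respawn and game over.
; Respawn teleports the given player to the location and rotation that FindRespawnPoint draws from random PlayerStart lookups, then re-enables input.
; GameOver calls MulticastGameOver on every BP_FPCharacter in the level.
; PlayerScored and GetScores are empty stubs, so no scoring logic exists here.
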(event `/Game/ShiitakeSorcerers/Core/GamemodeInterface.PlayerScored`
  (params (KillerName :type String) (KilledName :type String)))

(event `/Game/ShiitakeSorcerers/Core/GamemodeInterface.GameOver`
  (bind _outactors (`GameplayStatics.GetAllActorsOfClass` "/Game/ShiitakeSorcerers/Character/BP_FPCharacter.BP_FPCharacter_C"))
  (for _array_element _outactors
    (`/Game/ShiitakeSorcerers/Character/BP_FPCharacter.MulticastGameOver` _array_element)))

(fn `FindRespawnPoint`
  (returns (SpawnLocation :type "Vector Structure") (SpawnRotation :type "Rotator Structure"))
  ;[1 1 1] Gets a random spawn point
  (bind _outactors (`GameplayStatics.GetAllActorsOfClass` "/Script/Engine.PlayerStart"))
  (bind _output (`|GetArrayItem` _outactors (`KismetMathLibrary.RandomIntegerInRange` 0 (- (`KismetArrayLibrary.Array_Length` _outactors) 1))))
  (return (`self.K2_GetActorLocation` _output) (`self.K2_GetActorRotation` _output)))

(fn `GetScores`
  (returns (Scores :type "Map of String to Integer"))
  (return))

(fn `Respawn`
  (params (Player :type "/Game/ShiitakeSorcerers/Character/BP_FPCharacter Object Reference"))
  (returns (Return :type Boolean))
  (bind (_spawnlocation _spawnrotation) (`self.FindRespawnPoint`))
  (`self.K2_SetActorLocationAndRotation` Player _spawnlocation _spawnrotation false true)
  (`self.EnableInput` Player null)
  (return true))

(fn `UserConstructionScript`)