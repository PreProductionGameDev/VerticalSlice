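; Spawn volume actor that finds a random clear spawn point within the bounds of its scaled cube.
; FindSpawn line-traces down from a random point on the top, then sphere-traces upward from just above the hit to check for clearance.
; It returns a raised transform when clear, otherwise retries until a depth counter passes 25.
; That fallback returns a zero location but still reports Found as true.
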(event `self.ReceiveTick`
  (params (DeltaSeconds :type "Float (single-precision)")))

(fn `FindSpawn`
  (returns (Transform :type "Vector Structure") (Found :type Boolean))
  (locals (depth :type Integer))
  (bind (_returnvalue_x _returnvalue_y _returnvalue_z) (`KismetMathLibrary.BreakVector` (`self.GetActorScale3D`)))
  (bind (_min _max) (`StaticMeshComponent.GetLocalBounds` (`self.Cube`)))
  (bind _returnvalue (+ (`KismetMathLibrary.MakeVector` (`KismetMathLibrary.RandomFloatInRange` (* (.x _min) _returnvalue_x) (* (.x _max) _returnvalue_x)) (`KismetMathLibrary.RandomFloatInRange` (* (.y _min) _returnvalue_y) (* (.y _max) _returnvalue_y)) (* (.z _max) _returnvalue_z)) (`self.K2_GetActorLocation`)))
  (bind (_outhit _returnvalue_2) (`KismetSystemLibrary.LineTraceSingle` _returnvalue (- _returnvalue (`KismetMathLibrary.MakeVector` 0.0 0.0 (* (- (.z _max) (.z _min)) _returnvalue_z))) "TraceTypeQuery3" :!label _label))
  (if _returnvalue_2
    (bind _returnvalue_3 (+ (`.Location` (`GameplayStatics.BreakHitResult` _outhit)) (0.0 0.0 46.0)))
    (bind (_outhit_2 _returnvalue_4) (`KismetSystemLibrary.SphereTraceSingle` _returnvalue_3 (+ _returnvalue_3 (0.0 0.0 208.0)) 46.0 "TraceTypeQuery3"))
    (if _returnvalue_4
      _
      (else
        (return (+ _returnvalue_3 (0.0 0.0 104.0)) true))))
  (bind _result (`/Engine/EditorBlueprintResources/StandardMacros.IncrementInt` (`local.depth`))
    (:`  `
      (if (> _result 25)
        (return (0.0 0.0 0.0) true)
        (else
          (goto _label))))))

(fn `UserConstructionScript`)