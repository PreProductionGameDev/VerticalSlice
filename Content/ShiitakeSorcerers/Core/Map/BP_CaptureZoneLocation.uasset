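; BP_CaptureZoneLocation is a placed marker that spawns a capture zone for the King of the Hill game mode.
; On BeginPlay the server spawns BP_CaptureZone at its transform and adds it to GM_KOTH's Zones array.
; The add landing at hardcoded index 2, the third zone, shuffles ZoneOrder and activates the first.
; The marker destroys itself afterwards, and immediately on clients or in other game modes.
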(event `self.ReceiveBeginPlay`
  (if (`KismetSystemLibrary.IsServer`)
    (bind _asgm_koth (cast `/Game/ShiitakeSorcerers/Core/GM_KOTH` (`GameplayStatics.GetGameMode`))
      (:`then`
        (bind _returnvalue (`|SpawnActorFromClass` "/Game/ShiitakeSorcerers/Core/Map/BP_CaptureZone.BP_CaptureZone_C" (`self.GetTransform`) "Undefined" "OverrideRootScale" null null))
        (bind _returnvalue_2 (`KismetArrayLibrary.Array_Add` (`/Game/ShiitakeSorcerers/Core/GM_KOTH.Zones` _asgm_koth) _returnvalue))
        (if (== _returnvalue_2 2)
          (`KismetArrayLibrary.Array_Shuffle` (`/Game/ShiitakeSorcerers/Core/GM_KOTH.Zone order` _asgm_koth))
          (`/Game/ShiitakeSorcerers/Core/GM_KOTH.Activate` _asgm_koth 0))
        (`self.K2_DestroyActor`))
      (:`CastFailed`
        (`self.K2_DestroyActor`)))
    (else
      (`self.K2_DestroyActor`))))

(fn `UserConstructionScript`
  (bind _returnvalue (`PrimitiveComponent.CreateDynamicMaterialInstance` (`self.Cube`) 0 null "None"))
  (set `self.DynamicMaterial` _returnvalue))