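; King of the Hill capture zone that teams contest to earn score in GM_KOTH.
; A server timer nets red against blue players inside, shifting Progress and adding team score at either extreme.
; Tick turns state changes into multicast, throttled team-relative voice lines, blends barrier and beam colour, and keeps the marker widget camera-facing and distance-scaled.
; Replicated Active toggles visibility, and the first deactivation announces the zone has moved.
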(event `MulticastScoring`
  (params (RedTeam :type Boolean))
  (bind _captureddelay (`self.CapturedDelay`))
  (if RedTeam
    (`PrimitiveComponent.SetCustomDepthStencilValue` (`self.Widget`) 8)
    (else
      (`PrimitiveComponent.SetCustomDepthStencilValue` (`self.Widget`) 7)))
  (bind _asbp_fpcharacter (cast `/Game/ShiitakeSorcerers/Character/BP_FPCharacter` (`GameplayStatics.GetPlayerCharacter` 0)))
  (if (== (`/Game/ShiitakeSorcerers/Character/BP_FPCharacter.Red` _asbp_fpcharacter) RedTeam)
    (if (not _captureddelay)
      (`GameplayStatics.PlaySound2D` "/Game/ShiitakeSorcerers/Audio/SoundFX/GamemodeSounds/KOTH/A_We_have_captured_the_zone.A_We_have_captured_the_zone" 1.0 1.0 0.0 null null)
      (set `self.CapturedDelay` true :!label _label)
      (`KismetSystemLibrary.K2_SetTimerDelegate` (delegate `Captured Delay`) 2.5))
    (elif (not _captureddelay)
      (`GameplayStatics.PlaySound2D` "/Game/ShiitakeSorcerers/Audio/SoundFX/GamemodeSounds/KOTH/A_The_enemy_has_captured_the_zone.A_The_enemy_has_captured_the_zone" 1.0 1.0 0.0 null null)
      (goto _label))))

(event `Captured Delay`
  (set `self.CapturedDelay` false))

(event `MulticastCapturing`
  (params (RedTeam :type Boolean))
  (bind _capturingdelay (`self.CapturingDelay`))
  (bind _asbp_fpcharacter (cast `/Game/ShiitakeSorcerers/Character/BP_FPCharacter` (`GameplayStatics.GetPlayerCharacter` 0)))
  (if (== (`/Game/ShiitakeSorcerers/Character/BP_FPCharacter.Red` _asbp_fpcharacter) RedTeam)
    (if (not _capturingdelay)
      (`GameplayStatics.PlaySound2D` "/Game/ShiitakeSorcerers/Audio/SoundFX/GamemodeSounds/KOTH/A_We_are_capturing_the_zone.A_We_are_capturing_the_zone" 1.0 1.0 0.0 null null)
      (set `self.CapturingDelay` true :!label _label_2)
      (`KismetSystemLibrary.K2_SetTimerDelegate` (delegate `CaptureDelay`) 2.5))
    (elif (not _capturingdelay)
      (`GameplayStatics.PlaySound2D` "/Game/ShiitakeSorcerers/Audio/SoundFX/GamemodeSounds/KOTH/A_The_enemy_is_capturing_the_zone.A_The_enemy_is_capturing_the_zone" 1.0 1.0 0.0 null null)
      (goto _label_2))))

(event `CaptureDelay`
  (set `self.CapturingDelay` false))

(event `self.ReceiveBeginPlay`
  (if (`KismetSystemLibrary.IsServer`)
    (`KismetSystemLibrary.K2_SetTimerDelegate` (delegate `ServerProgress`) 0.1 true)))

(event `ServerProgress`
  (bind _direction (`self.Direction`))
  (bind _returnvalue (* (`self.Direction`) 0.1 0.1))
  (bind _returnvalue_2 (`KismetMathLibrary.Abs` _returnvalue))
  (bind _returnvalue_3 (+ (`self.Progress`) _returnvalue))
  (if (`self.Active`)
    (set `self.Direction` 0)
    (bind _asgm_koth (cast `/Game/ShiitakeSorcerers/Core/GM_KOTH` (`GameplayStatics.GetGameMode`)))
    (for _array_element (`PrimitiveComponent.GetOverlappingActors` (`self.Cylinder1`) "/Game/ShiitakeSorcerers/Character/BP_FPCharacter.BP_FPCharacter_C")
      (if (`.ReturnValue` (`BlueprintMapLibrary.Map_Find` (`/Game/ShiitakeSorcerers/Core/GM_KOTH.RedTeamKillsMap` _asgm_koth) (`PlayerState.GetPlayerName` (`Pawn.PlayerState` (cast `/Game/ShiitakeSorcerers/Character/BP_FPCharacter` _array_element :!pure true)))))
        (`/Engine/EditorBlueprintResources/StandardMacros.DecrementInt` _direction)
        (else
          (`/Engine/EditorBlueprintResources/StandardMacros.IncrementInt` _direction))))
    (if (<= _returnvalue_3 0.0)
      (set `self.Progress` 0.0)
      (set `/Game/ShiitakeSorcerers/Core/GM_KOTH.RedScore` (+ (`/Game/ShiitakeSorcerers/Core/GM_KOTH.RedScore` _asgm_koth) _returnvalue_2) _asgm_koth)
      (set `self.Scoring` true)
      (set `self.Capture State` 4)
      (elif (>= _returnvalue_3 1.0)
        (set `self.Progress` 1.0)
        (set `/Game/ShiitakeSorcerers/Core/GM_KOTH.BlueScore` (+ (`/Game/ShiitakeSorcerers/Core/GM_KOTH.BlueScore` _asgm_koth) _returnvalue_2) _asgm_koth)
        (set `self.Scoring` true)
        (set `self.Capture State` 1)
        (else
          (set `self.Progress` _returnvalue_3)
          (set `self.Scoring` false)
          (if (> (`self.Direction`) 0)
            (set `self.Capture State` 2)
            (elif (< (`self.Direction`) 0)
              (set `self.Capture State` 3)
              (else
                (set `self.Capture State` 0)))))))))

(event `self.ReceiveTick`
  (params (DeltaSeconds :type "Float (single-precision)"))
  (bind _capture_state (`self.Capture State`))
  (bind _dynamicmaterial (`self.DynamicMaterial`))
  (bind (_currentcolor_r _currentcolor_g _currentcolor_b) (break `LinearColor` (`self.CurrentColor`)))
  (`self.PointCamera`)
  (if (`self.Scoring`)
    (bind _output_get (set `self.CurrentColor` (`KismetMathLibrary.LinearColorLerp` (`KismetMathLibrary.LinearColorLerp` (make `LinearColor` 50.0 0.0 0.0 0.5) (make `LinearColor` 0.0 40.0 50.0 0.5) (`self.Progress`)) (`self.CurrentColor`) 0.9)))
    (`MaterialInstanceDynamic.SetVectorParameterValue` (`self.DynamicMaterial`) "BarrierColour" _output_get)
    (else
      (`PrimitiveComponent.SetCustomDepthStencilValue` (`self.Widget`) 6)
      (bind _output_get_2 (set `self.CurrentColor` (`KismetMathLibrary.LinearColorLerp` (`KismetMathLibrary.LinearColorLerp` (make `LinearColor` 5.0 0.0 0.0 0.5) (make `LinearColor` 0.0 4.0 5.0 0.5) (`self.Progress`)) (`self.CurrentColor`) 0.9)))
      (`MaterialInstanceDynamic.SetVectorParameterValue` _dynamicmaterial "BarrierColour" _output_get_2)))
  (`NiagaraComponent.SetVariableLinearColor` (`self.NS_ZoneLight`) "BeamColour" (make `LinearColor` _currentcolor_r _currentcolor_g _currentcolor_b 0.05))
  (`MaterialInstanceDynamic.SetScalarParameterValue` _dynamicmaterial "FadeDistance" (+ (* (`KismetMathLibrary.Sin` (* (`self.GetGameTimeSinceCreation`) 2.5)) 25.0) 80.0))
  (if (!= (`self.Previous State`) _capture_state)
    (switch `int` _capture_state
      (:`0`
        _)
      (:`1`
        (`self.MulticastScoring` false))
      (:`2`
        (`self.MulticastCapturing` false))
      (:`3`
        (`self.MulticastCapturing` true))
      (:`4`
        (`self.MulticastScoring` true)))
    (set `self.Previous State` (`self.Capture State`))))

(event `MulticastZoneMoved`
  (`GameplayStatics.PlaySound2D` "/Game/ShiitakeSorcerers/Audio/SoundFX/GamemodeSounds/KOTH/The_zone_has_moved.The_zone_has_moved" 1.0 1.0 0.0 null null))

(event `Activate`
  (set `self.Active` true))

(event `Deactivate`
  (set `self.Active` false)
  (if (not (`self.Moved`))
    (`self.MulticastZoneMoved`)
    (set `self.Moved` true)))

(fn `OnRep_Active`
  (`SceneComponent.SetVisibility` (`self.Cylinder`) (`self.Active`) false)
  (`SceneComponent.SetVisibility` (`self.Widget`) (`self.Active`) false)
  (`SceneComponent.SetVisibility` (`self.NS_ZoneLight`) (`self.Active`) false))

(fn `PointCamera`
  (bind _widget (`self.Widget`))
  (bind _returnvalue (`SceneComponent.K2_GetComponentLocation` _widget))
  (bind _asbp_fpcharacter (cast `/Game/ShiitakeSorcerers/Character/BP_FPCharacter` (`GameplayStatics.GetPlayerCharacter` 0)))
  (bind _returnvalue_2 (`SceneComponent.K2_GetComponentLocation` (`FP_Character.FirstPersonCameraComponent` _asbp_fpcharacter)))
  (`SceneComponent.K2_SetWorldRotation` _widget (`KismetMathLibrary.FindLookAtRotation` _returnvalue _returnvalue_2) false false)
  (bind _returnvalue_3 (`KismetMathLibrary.Vector_Distance` _returnvalue _returnvalue_2))
  (`WidgetComponent.SetDrawSize` (`self.Widget`) (`KismetMathLibrary.ClampAxes2D` (* (0.05 0.05) (`KismetMathLibrary.MakeVector2D` _returnvalue_3 _returnvalue_3)) 100.0 10000.0))
  (`SceneComponent.SetWorldScale3D` _widget (1.0 1.0 1.0)))

(fn `UserConstructionScript`
  (bind _returnvalue (`PrimitiveComponent.CreateDynamicMaterialInstance` (`self.Cylinder`) 0 null "None"))
  (set `self.DynamicMaterial` _returnvalue))