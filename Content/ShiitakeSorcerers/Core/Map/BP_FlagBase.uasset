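; BP_FlagBase is a team's Capture the Flag base, serving as both flag spawn and scoring zone.
; On BeginPlay the server spawns a BP_Flag linked to this base in GM_CTF, or sets Disabled in other game modes.
; A flag from another team's base overlapping it scores for this base's team, checked server-side.
; The Disabled RepNotify hides the mesh and turns off mesh and box collision.
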(event `self.ReceiveBeginPlay`
  (if (`KismetSystemLibrary.IsServer`)
    (cast `/Game/ShiitakeSorcerers/Core/GM_CTF` (`GameplayStatics.GetGameMode`)
      (:`then`
        (bind _returnvalue (`|SpawnActorFromClass` "/Game/ShiitakeSorcerers/Core/Map/BP_Flag.BP_Flag_C" (`self.GetTransform`) "Undefined" "OverrideRootScale" null null))
        (set `/Game/ShiitakeSorcerers/Core/Map/BP_Flag.Base` self _returnvalue))
      (:`CastFailed`
        (set `self.Disabled` true)))))

(event `self.ReceiveActorBeginOverlap`
  (params (OtherActor :type "Actor Object Reference"))
  (bind _team (`self.Team`))
  (if (`KismetSystemLibrary.IsServer`)
    (bind _asbp_flag (cast `/Game/ShiitakeSorcerers/Core/Map/BP_Flag` OtherActor))
    (if (`KismetStringLibrary.NotEqual_StrStr` (`/Game/ShiitakeSorcerers/Core/Map/BP_FlagBase.Team` (`/Game/ShiitakeSorcerers/Core/Map/BP_Flag.Base` _asbp_flag)) _team)
      (`/Game/ShiitakeSorcerers/Core/Map/BP_Flag.Score` _asbp_flag _team))))

(fn `OnRep_Disabled`
  (`SceneComponent.SetVisibility` (`self.StaticMesh`) false false)
  (`PrimitiveComponent.SetCollisionEnabled` (`self.StaticMesh`) "NoCollision")
  (`PrimitiveComponent.SetCollisionEnabled` (`self.Box`) "NoCollision"))

(fn `UserConstructionScript`)