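; Capture-the-flag flag actor that enemy players pick up by overlap and that returns to its Base on scoring or timeout.
; Team is resolved by looking up the player's name in GM_CTF's RedTeam, then compared with Base.Team.
; A fast looping timer lerps the flag toward its carrier; carrier death starts a delayed reset, cancelled by another pickup.
; Score increments the scoring team's GM_CTF flag count and resets the flag.
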(event `self.ReceiveActorBeginOverlap`
  (params (OtherActor :type "Actor Object Reference"))
  (if (not (`KismetSystemLibrary.K2_IsValidTimerHandle` (`self.ChaseTimer`)))
    (bind _asbp_fpcharacter (cast `/Game/ShiitakeSorcerers/Character/BP_FPCharacter` OtherActor))
    (bind _asgm_ctf (cast `/Game/ShiitakeSorcerers/Core/GM_CTF` (`GameplayStatics.GetGameMode`)))
    (if (`.ReturnValue` (`BlueprintMapLibrary.Map_Find` (`/Game/ShiitakeSorcerers/Core/GM_CTF.Red Team` _asgm_ctf) (`PlayerState.GetPlayerName` (`Pawn.PlayerState` _asbp_fpcharacter))))
      (if (not (`KismetStringLibrary.EqualEqual_StrStr` (`/Game/ShiitakeSorcerers/Core/Map/BP_FlagBase.Team` (`self.Base`)) "Red"))
        (set `self.FPCharacter` _asbp_fpcharacter :!label _label)
        (bind _returnvalue (`KismetSystemLibrary.K2_SetTimerDelegate` (delegate `FollowActor`) 0.001 true))
        (set `self.ChaseTimer` _returnvalue)
        (`KismetSystemLibrary.K2_ClearAndInvalidateTimerHandle` (`self.ResetTimer`)))
      (elif (not (`KismetStringLibrary.EqualEqual_StrStr` (`/Game/ShiitakeSorcerers/Core/Map/BP_FlagBase.Team` (`self.Base`)) "Blue"))
        (goto _label)))))

(event `FollowActor`
  (bind _returnvalue (`self.GetTransform`))
  (bind _returnvalue_2 (`self.GetTransform` (`self.FPCharacter`)))
  (if (not (< (`KismetMathLibrary.Vector_Distance` (.location _returnvalue_2) (.location _returnvalue)) 300.0))
    (`self.K2_SetActorTransform` (`KismetMathLibrary.TLerp` _returnvalue _returnvalue_2 0.01)))
  (bind _returnvalue_3 (`FP_Character.GetHealth` (`self.FPCharacter`)))
  (if (not (> _returnvalue_3 0.0))
    (`KismetSystemLibrary.K2_ClearAndInvalidateTimerHandle` (`self.ChaseTimer`))
    (bind _returnvalue_4 (`KismetSystemLibrary.K2_SetTimerDelegate` (delegate `ResetFlag`) 10.0))
    (set `self.ResetTimer` _returnvalue_4)))

(event `Score`
  (params (`Scoring Team` :type String))
  (bind _asgm_ctf (cast `/Game/ShiitakeSorcerers/Core/GM_CTF` (`GameplayStatics.GetGameMode`)))
  (switch `string` `Scoring Team`
    (:`Red`
      (set `/Game/ShiitakeSorcerers/Core/GM_CTF.RedFlags` (+ (`/Game/ShiitakeSorcerers/Core/GM_CTF.RedFlags` _asgm_ctf) 1) _asgm_ctf))
    (:`Blue`
      (set `/Game/ShiitakeSorcerers/Core/GM_CTF.BlueFlags` (+ (`/Game/ShiitakeSorcerers/Core/GM_CTF.BlueFlags` _asgm_ctf) 1) _asgm_ctf)))
  (`KismetSystemLibrary.K2_ClearAndInvalidateTimerHandle` (`self.ChaseTimer`))
  (`self.ResetFlag`))

(event `ResetFlag`
  (`KismetSystemLibrary.K2_ClearAndInvalidateTimerHandle` (`self.ResetTimer`))
  (`self.K2_SetActorTransform` (`self.GetTransform` (`self.Base`)) false true))

(fn `UserConstructionScript`)