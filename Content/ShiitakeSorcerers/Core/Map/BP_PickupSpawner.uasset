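; BP_PickupSpawner is a map actor that spawns a configurable pickup class at its root transform and respawns it once it is gone.
; It spawns on BeginPlay; server-side Tick starts a RespawnTime timer whenever the spawned actor is invalid and no timer is pending.
; ServerRespawnActor stores the new actor, clears the timer handle and marks BWeapon-derived spawns as pickupable.
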(event `self.ReceiveBeginPlay`
  (`self.ServerRespawn Actor`))

(event `self.ReceiveTick`
  (params (DeltaSeconds :type "Float (single-precision)"))
  (if (`KismetSystemLibrary.IsServer`)
    (`/Engine/EditorBlueprintResources/StandardMacros.IsValid` (`self.SpawnedActor`)
      (:`Is Not Valid`
        (if (not (`KismetSystemLibrary.K2_IsValidTimerHandle` (`self.RespawnHandle`)))
          (bind _returnvalue (`KismetSystemLibrary.K2_SetTimerDelegate` (delegate `ServerRespawn Actor`) (`self.RespawnTime`)))
          (set `self.RespawnHandle` _returnvalue))))))

(event `ServerRespawn Actor`
  (bind _returnvalue (`|SpawnActorFromClass` (`self.PickupType`) (`SceneComponent.K2_GetComponentToWorld` (`self.DefaultSceneRoot`)) "Undefined" "OverrideRootScale" null null))
  (set `self.SpawnedActor` _returnvalue)
  (`KismetSystemLibrary.K2_ClearAndInvalidateTimerHandle` (`self.RespawnHandle`))
  (if (`KismetMathLibrary.ClassIsChildOf` (`self.PickupType`) "/Script/VerticalSlice.BWeapon")
    (bind _asbweapon (cast `BWeapon` (`self.SpawnedActor`)))
    (set `BWeapon.Pickupable` true _asbweapon)))

(fn `UserConstructionScript`)