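; BP_TeamBarrier is a team barrier that lets characters carrying its TeamTag pass through it in team game modes.
; Construction picks the Serpents or Shrooms mesh for Blue or Red; BeginPlay destroys it unless running on the server with GM_FPTest's TeamGM set.
; On a Box hit, a matching ability system tag routes the character's capsule through server and multicast events to ignore the barrier when moving.
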(event `self.ReceiveBeginPlay`
  ;[1 1 1] Verify that it is a team game mode
  (if (`KismetSystemLibrary.IsServer`)
    (bind _asgm_fptest (cast `/Game/ShiitakeSorcerers/Core/GM_FPTest` (`GameplayStatics.GetGameMode`))
      (:`then`
        (if (not (`/Game/ShiitakeSorcerers/Core/GM_FPTest.TeamGM` _asgm_fptest))
          (`self.K2_DestroyActor`)))
      (:`CastFailed`
        (`self.K2_DestroyActor`)))
    (else
      (`self.K2_DestroyActor`))))

(event `self.Box.OnComponentHit`
  (params (HitComponent :type "PrimitiveComponent Object Reference") (OtherActor :type "Actor Object Reference") (OtherComp :type "PrimitiveComponent Object Reference") (NormalImpulse :type "Vector Structure") (Hit :type "HitResult Structure (by ref)"))
  (bind _asfp_character (cast `FP_Character` OtherActor))
  (if (`GameplayTagAssetInterface.HasAnyMatchingGameplayTags` (`AbilitySystemBlueprintLibrary.GetAbilitySystemComponent` _asfp_character) (`BlueprintGameplayTagLibrary.MakeGameplayTagContainerFromTag` (`self.Team Tag`)))
    (`self.Server_IgnoreActor` (`Character.CapsuleComponent` _asfp_character))))

(event `Server_IgnoreActor`
  (params (Target :type "PrimitiveComponent Object Reference"))
  (`self.Multicast_IgnoreActor` Target))

(event `Multicast_IgnoreActor`
  (params (Target :type "PrimitiveComponent Object Reference"))
  (`PrimitiveComponent.IgnoreActorWhenMoving` Target self true))

(fn `UserConstructionScript`
  (`|SwitchGameplayTag` (`self.Team Tag`)
    (:`Team.Blue`
      (`StaticMeshComponent.SetStaticMesh` (`self.Barrier`) "/Game/ShiitakeSorcerers/VFX/TeamFX/SM_TeamBarrierSerpents.SM_TeamBarrierSerpents"))
    (:`Team.Red`
      (`StaticMeshComponent.SetStaticMesh` (`self.Barrier`) "/Game/ShiitakeSorcerers/VFX/TeamFX/SM_TeamBarrierShrooms.SM_TeamBarrierShrooms"))))