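; BP_HealthPot is a health potion pickup that triggers the player character's heal when touched.
; Tick accumulates lifetime and drives a sine wave that bobs the static mesh and Niagara effect vertically.
; When the mesh overlaps a BP_FPCharacter, it simulates the Heal input press on that character's Ability System Component, then destroys itself.
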(event `self.ReceiveTick`
  (params (DeltaSeconds :type "Float (single-precision)"))
  (set `self.LifeTime` (+ DeltaSeconds (`self.LifeTime`)))
  (`SceneComponent.K2_SetRelativeLocation` (`self.StaticMesh`) (`KismetMathLibrary.MakeVector` 0.0 0.0 (* (`KismetMathLibrary.Sin` (`self.LifeTime`)) 20.0)) false false)
  (`SceneComponent.K2_SetRelativeLocation` (`self.Niagara`) (`KismetMathLibrary.MakeVector` 0.0 0.0 (* (`KismetMathLibrary.Sin` (`self.LifeTime`)) 20.0)) false false))

(event `self.StaticMesh.OnComponentBeginOverlap`
  (params (OverlappedComponent :type "PrimitiveComponent Object Reference") (OtherActor :type "Actor Object Reference") (OtherComp :type "PrimitiveComponent Object Reference") (OtherBodyIndex :type Integer) (bFromSweep :type Boolean) (SweepResult :type "HitResult Structure (by ref)"))
  (bind _asbp_fpcharacter (cast `/Game/ShiitakeSorcerers/Character/BP_FPCharacter` OtherActor))
  (`AbilitySystemComponent.PressInputID` (`AbilitySystemBlueprintLibrary.GetAbilitySystemComponent` _asbp_fpcharacter) (`KismetMathLibrary.Conv_ByteToInt` (enumliteral `EPlayerAbilityInputID` "Heal")))
  (`self.K2_DestroyActor`))

(fn `UserConstructionScript`)