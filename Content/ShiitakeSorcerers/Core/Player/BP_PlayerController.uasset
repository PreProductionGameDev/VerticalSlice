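; BP_PlayerController is the player controller for Shiitake Sorcerers that relays a player's team choice to the game mode.
; Four Server-prefixed events cover red team, blue team, random and spectate.
; Each calls the matching message function on the game mode and passes the controller itself, leaving the assignment logic outside this Blueprint.
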(event `ServerRedTeam`
  (message `/Game/ShiitakeSorcerers/Core/GamemodeInterface.RedTeam` (`GameplayStatics.GetGameMode`) self))

(event `ServerBlueTeam`
  (message `/Game/ShiitakeSorcerers/Core/GamemodeInterface.BlueTeam` (`GameplayStatics.GetGameMode`) self))

(event `ServerRandom`
  (message `/Game/ShiitakeSorcerers/Core/GamemodeInterface.Random` (`GameplayStatics.GetGameMode`) self))

(event `ServerSpectate`
  (message `/Game/ShiitakeSorcerers/Core/GamemodeInterface.Spectate` (`GameplayStatics.GetGameMode`) self))

(fn `UserConstructionScript`)