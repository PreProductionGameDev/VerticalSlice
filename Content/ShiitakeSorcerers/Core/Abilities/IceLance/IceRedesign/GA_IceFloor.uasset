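; Gameplay ability that lays a trail of BP_IceFloor actors beneath the player character while active.
; A fast looping timer drives SpawnIce, while a one-shot timer is set alongside it, with SpawnStopper clearing the loop and ending the ability.
; Each spawn calls ClientCameraRotation, waits for client-server net sync, then places ice below and slightly ahead of the ThrownItems transform, with clamped pitch.
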(event `self.K2_ActivateAbility`
  (bind _returnvalue (`KismetSystemLibrary.K2_SetTimerDelegate` (delegate `SpawnIce`) 0.1 true))
  (set `self.IceSpawningTimer` _returnvalue)
  (bind _returnvalue_2 (`KismetSystemLibrary.K2_SetTimerDelegate` (`|CreateDelegate` :!event `SpawnStopper`) 2.0))
  (set `self.EndTimer` _returnvalue_2))

(event `SpawnIce`
  (bind _asbp_fpcharacter (cast `/Game/ShiitakeSorcerers/Character/BP_FPCharacter` (`self.GetOwningActorFromActorInfo`)))
  (`FP_Character.ClientCameraRotation` _asbp_fpcharacter)
  (`AbilityTask_NetworkSyncPoint.WaitNetSync` "BothWait"
    (:`OnSync`
      (bind (_returnvalue_location _returnvalue_rotation _returnvalue_scale) (`KismetMathLibrary.BreakTransform` (`SceneComponent.K2_GetComponentToWorld` (`/Game/ShiitakeSorcerers/Character/BP_FPCharacter.ThrownItems` _asbp_fpcharacter))))
      (`|SpawnActorFromClass` "/Game/ShiitakeSorcerers/Core/Abilities/IceLance/IceRedesign/BP_IceFloor.BP_IceFloor_C" (`KismetMathLibrary.MakeTransform` (+ (0.0 0.0 -209.100006) _returnvalue_location (* (`SceneComponent.GetForwardVector` (`Character.CapsuleComponent` _asbp_fpcharacter)) 9.5)) (`KismetMathLibrary.MakeRotator` (.roll _returnvalue_rotation) (`KismetMathLibrary.FClamp` (.pitch _returnvalue_rotation) -45.0 45.0) (.yaw _returnvalue_rotation)) _returnvalue_scale) "Undefined" "OverrideRootScale" null null))))

(event `SpawnStopper`
  (`KismetSystemLibrary.K2_ClearAndInvalidateTimerHandle` (`self.IceSpawningTimer`))
  (`self.K2_EndAbility`))