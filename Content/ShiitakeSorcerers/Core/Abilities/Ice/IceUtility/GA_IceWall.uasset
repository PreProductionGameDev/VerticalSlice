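; Gameplay ability that lets the player aim and place an ice wall.
; While input is held, a looping timer moves a ghost wall to a camera trace hit, or traces down from its end on a miss, matching player yaw.
; On release, it spawns the real wall at the ghost's transform and destroys the ghost.
; A timer passed to the HUD serves as cooldown, delaying EndAbility until it expires.
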(event `self.K2_ActivateAbility`
  (bind _returnvalue (`|SpawnActorFromClass` "/Game/ShiitakeSorcerers/Core/Abilities/Ice/IceUtility/BP_IceWallGhost.BP_IceWallGhost_C" (`KismetMathLibrary.MakeTransform` (0.0 0.0 0.0)) "Undefined" "OverrideRootScale" null null))
  (set `self.IceWallGhost` _returnvalue)
  (bind _returnvalue_2 (`KismetSystemLibrary.K2_SetTimerDelegate` (delegate `MoveGhostWall`) 0.01 true))
  (set `self.WallMoveHandle` _returnvalue_2)
  (`AbilityTask_WaitInputRelease.WaitInputRelease` true
    (:`OnRelease`
      (`self.CastAbility`))))

(event `MoveGhostWall`
  (bind (_returnvalue_roll _returnvalue_pitch _returnvalue_yaw) (`KismetMathLibrary.BreakRotator` (`Actor.K2_GetActorRotation` (`self.GetOwningActorFromActorInfo`))))
  (bind (_returnvalue_roll_2 _returnvalue_pitch_2 _returnvalue_yaw_2) (`KismetMathLibrary.BreakRotator` (`Actor.K2_GetActorRotation` (`self.GetOwningActorFromActorInfo`))))
  (bind _firstpersoncameracomponent (`FP_Character.FirstPersonCameraComponent` (cast `/Game/ShiitakeSorcerers/Character/BP_FPCharacter` (`self.GetOwningActorFromActorInfo`) :!pure true)))
  (bind _returnvalue (`SceneComponent.K2_GetComponentLocation` _firstpersoncameracomponent))
  (bind (_outhit _returnvalue_2) (`KismetSystemLibrary.LineTraceSingle` _returnvalue (+ _returnvalue (* (`SceneComponent.GetForwardVector` _firstpersoncameracomponent) 2000.0)) "TraceTypeQuery1"))
  (if _returnvalue_2
    (`Actor.K2_SetActorTransform` (`self.IceWallGhost`) (`KismetMathLibrary.MakeTransform` (`.Location` (`GameplayStatics.BreakHitResult` _outhit)) (`KismetMathLibrary.MakeRotator` 0.0 0.0 _returnvalue_yaw)) false false)
    (else
      (bind _outhit_2 (`KismetSystemLibrary.LineTraceSingle` (`.TraceEnd` (`GameplayStatics.BreakHitResult` _outhit)) (- (`.TraceEnd` (`GameplayStatics.BreakHitResult` _outhit)) (0.0 0.0 5000.0)) "TraceTypeQuery1"))
      (`Actor.K2_SetActorTransform` (`self.IceWallGhost`) (`KismetMathLibrary.MakeTransform` (`.Location` (`GameplayStatics.BreakHitResult` _outhit_2)) (`KismetMathLibrary.MakeRotator` 0.0 0.0 _returnvalue_yaw_2)) false false))))

(event `self.K2_OnEndAbility`
  (params (bWasCancelled :type Boolean)))

(event `CastAbility`
  (bind _returnvalue (`FP_Character.GetPlayerHUD` (cast `/Game/ShiitakeSorcerers/Character/BP_FPCharacter` (`self.GetOwningActorFromActorInfo`) :!pure true)))
  (`KismetSystemLibrary.K2_ClearAndInvalidateTimerHandle` (`self.WallMoveHandle`))
  (`|SpawnActorFromClass` "/Game/ShiitakeSorcerers/Core/Abilities/Ice/IceUtility/BP_IceWall.BP_IceWall_C" (`Actor.GetTransform` (`self.IceWallGhost`)) "Undefined" "OverrideRootScale" null null)
  (`Actor.K2_DestroyActor` (`self.IceWallGhost`))
  (bind _returnvalue_2 (`KismetSystemLibrary.K2_SetTimerDelegate` (delegate `AbilityCooldown`) 15.0))
  (set `self.CooldownHandle` _returnvalue_2)
  (`/Engine/EditorBlueprintResources/StandardMacros.IsValid` _returnvalue
    (:`Is Valid`
      (`PlayerHUD.SetAbilityCooldown` _returnvalue (`self.CooldownHandle`)))))

(event `AbilityCooldown`
  (`KismetSystemLibrary.K2_ClearAndInvalidateTimerHandle` (`self.CooldownHandle`))
  (`self.K2_EndAbility`))