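; Ice Lance gameplay ability that fires BP_LanceProjectile from the player's camera and handles its hit and floor-ice speed boost.
; Gameplay events from the lance apply GE_LanceHit to struck characters or raise max walk speed on boosted ones, using WaitNetSync around networked steps.
; A looping timer restores each boosted player's speed once off BP_FloorIce.
; The ability stays active until its HUD-displayed cooldown timer ends it.
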(event `AbillityCooldown`
  ;[1 1 1] Abillity cooldown and reset
  (`self.K2_EndAbility`)
  (`KismetSystemLibrary.K2_ClearAndInvalidateTimerHandle` (`self.CooldownTimer`)))

(event `self.K2_ActivateAbility`
  (bind _boosed_players (`self.Boosed players`))
  (bind _asbp_fpcharacter (cast `/Game/ShiitakeSorcerers/Character/BP_FPCharacter` (`self.GetOwningActorFromActorInfo`)))
  (`FP_Character.ClientCameraRotation` _asbp_fpcharacter)
  (`AbilityTask_NetworkSyncPoint.WaitNetSync` "BothWait"
    (:`OnSync`
      (`|SpawnActorFromClass` "/Game/ShiitakeSorcerers/Core/Abilities/Ice/IceUtility/IceLance/BP_LanceProjectile.BP_LanceProjectile_C" (`SceneComponent.GetSocketTransform` (`FP_Character.FirstPersonCameraComponent` _asbp_fpcharacter) "None" "RTS_World") "Undefined" "OverrideRootScale" _asbp_fpcharacter _asbp_fpcharacter)
      ;[1 1 1] Boost player speed
      (bind (_asynctaskproxy _payload) (`AbilityTask_WaitGameplayEvent.WaitGameplayEvent` (struct :`TagName` "Ice.Lance.Speed.Boost") null)
        (:`then`
          ;[1 1 1] Abillity cooldown and reset
          (bind _returnvalue (`KismetSystemLibrary.K2_SetTimerDelegate` (delegate `AbillityCooldown`) 12.0))
          (set `self.CooldownTimer` _returnvalue)
          (bind _asbp_fpcharacter_2 (cast `/Game/ShiitakeSorcerers/Character/BP_FPCharacter` (`self.GetOwningActorFromActorInfo`)))
          (bind _returnvalue_2 (`FP_Character.GetPlayerHUD` _asbp_fpcharacter_2))
          (if (`KismetSystemLibrary.IsValid` _returnvalue_2)
            (`PlayerHUD.SetAbilityCooldown` _returnvalue_2 (`self.CooldownTimer`)))
          (bind (_asynctaskproxy_2 _payload_2) (`AbilityTask_WaitGameplayEvent.WaitGameplayEvent` (struct :`TagName` "Ice.Lance.Hit") null)
            (:`EventReceived`
              (bind _asbp_fpcharacter_3 (cast `/Game/ShiitakeSorcerers/Character/BP_FPCharacter` (`.Target` (break `GameplayEventData` _payload_2))))
              (`self.BP_ApplyGameplayEffectToTarget` (`AbilitySystemBlueprintLibrary.AbilityTargetDataFromActor` _asbp_fpcharacter_3) "/Game/ShiitakeSorcerers/Core/Abilities/Ice/IceUtility/IceLance/GE_LanceHit.GE_LanceHit_C"))))
        (:`EventReceived`
          (bind _asbp_fpcharacter_4 (cast `/Game/ShiitakeSorcerers/Character/BP_FPCharacter` (`.Target` (break `GameplayEventData` _payload))))
          (`AbilityTask_NetworkSyncPoint.WaitNetSync` "BothWait"
            (:`OnSync`
              (set `CharacterMovementComponent.MaxWalkSpeed` 2000.0 (`Character.CharacterMovement` _asbp_fpcharacter_4))
              (if (not (`KismetArrayLibrary.Array_Contains` _boosed_players _asbp_fpcharacter_4))
                (`KismetArrayLibrary.Array_Add` _boosed_players _asbp_fpcharacter_4)
                (if (not (`KismetSystemLibrary.K2_IsValidTimerHandle` (`self.Speed reset`)))
                  (bind _returnvalue_3 (`KismetSystemLibrary.K2_SetTimerDelegate` (delegate `Ice Check`) 0.1 true))
                  (set `self.Speed reset` _returnvalue_3))))))))))

(event `Ice Check`
  (bind _boosed_players (`self.Boosed players`))
  (if (> (`KismetArrayLibrary.Array_Length` _boosed_players) 0)
    (for _array_element _boosed_players
      (if (not (> (`KismetArrayLibrary.Array_Length` (`Actor.GetOverlappingActors` _array_element "/Game/ShiitakeSorcerers/Core/Abilities/Ice/IceUtility/IceLance/BP_FloorIce.BP_FloorIce_C")) 0))
        ;[1 1 1] Reduce player speed
        (`AbilityTask_NetworkSyncPoint.WaitNetSync` "BothWait"
          (:`OnSync`
            (set `CharacterMovementComponent.MaxWalkSpeed` 1200.0 (`Character.CharacterMovement` _array_element))
            (`AbilityTask_NetworkSyncPoint.WaitNetSync` "BothWait"
              (:`OnSync`
                (`KismetArrayLibrary.Array_RemoveItem` (`self.Boosed players`) _array_element)))))))
    (else
      (`KismetSystemLibrary.K2_ClearAndInvalidateTimerHandle` (`self.Speed reset`)))))