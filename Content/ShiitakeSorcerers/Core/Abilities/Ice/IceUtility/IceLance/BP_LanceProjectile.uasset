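; BP_LanceProjectile is the projectile for the Ice Lance ability, laying a trail of floor ice as it travels.
; A looping timer traces downward and spawns BP_FloorIce, yaw-aligned to the projectile, wherever the trace hits.
; Overlapping a valid non-owner actor sends an Ice.Lance.Hit gameplay event to the instigator with that actor as target, then despawns the projectile.
; Without a hit, a lifetime timer despawns it.
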(event `Despawn Projectile`
  (`KismetSystemLibrary.K2_ClearAndInvalidateTimerHandle` (`self.IceSpawning`))
  (`KismetSystemLibrary.K2_ClearAndInvalidateTimerHandle` (`self.DestroyProjectile`))
  (`self.K2_DestroyActor`))

(event `SpawnIce`
  (bind _returnvalue (`self.K2_GetActorLocation`))
  (bind (_returnvalue_roll _returnvalue_pitch _returnvalue_yaw) (`KismetMathLibrary.BreakRotator` (`self.K2_GetActorRotation`)))
  (bind (_outhit _returnvalue_2) (`KismetSystemLibrary.LineTraceSingle` _returnvalue (+ _returnvalue (0.0 0.0 -400.0)) "TraceTypeQuery1"))
  (if _returnvalue_2
    (`|SpawnActorFromClass` "/Game/ShiitakeSorcerers/Core/Abilities/Ice/IceUtility/IceLance/BP_FloorIce.BP_FloorIce_C" (`KismetMathLibrary.MakeTransform` (`.Location` (`GameplayStatics.BreakHitResult` _outhit)) (`KismetMathLibrary.MakeRotator` 0.0 0.0 _returnvalue_yaw)) "Undefined" "OverrideRootScale" null (`self.GetInstigator`))))

(event `self.ReceiveBeginPlay`
  (bind _returnvalue (`KismetSystemLibrary.K2_SetTimerDelegate` (delegate `SpawnIce`) 0.05 true))
  (set `self.IceSpawning` _returnvalue)
  (bind _returnvalue_2 (`KismetSystemLibrary.K2_SetTimerDelegate` (delegate `Despawn Projectile`) 1.0))
  (set `self.DestroyProjectile` _returnvalue_2)
  (`KismetSystemLibrary.Delay` 0.055)
  (`self.SpawnIce`))

(event `self.Sphere.OnComponentBeginOverlap`
  (params (OverlappedComponent :type "PrimitiveComponent Object Reference") (OtherActor :type "Actor Object Reference") (OtherComp :type "PrimitiveComponent Object Reference") (OtherBodyIndex :type Integer) (bFromSweep :type Boolean) (SweepResult :type "HitResult Structure (by ref)"))
  (if (`KismetSystemLibrary.IsValid` OtherActor)
    (if (!= OtherActor (`self.GetOwner`))
      (`AbilitySystemBlueprintLibrary.SendGameplayEventToActor` (`self.GetInstigator`) (struct :`TagName` "Ice.Lance.Hit") (make `GameplayEventData` (struct :`TagName` "Ice.Lance.Hit") null OtherActor))
      (`self.Despawn Projectile`))
    (else
      (`self.Despawn Projectile`))))

(fn `UserConstructionScript`)