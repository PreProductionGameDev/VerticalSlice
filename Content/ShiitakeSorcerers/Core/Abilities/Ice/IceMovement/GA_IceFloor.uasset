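; GA_IceFloor is a held gameplay ability that lays a trail of ice floor pieces beneath the player character.
; A looping timer spends stamina each tick, then after a net sync spawns BP_IceFloor below the capsule, aimed by ThrownItems with clamped pitch and randomly yawed ice.
; Releasing input or running out of stamina stops the timer, fades the attached looping sound and ends the ability.
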(event `self.K2_ActivateAbility`
  (bind _returnvalue (`KismetSystemLibrary.K2_SetTimerDelegate` (delegate `SpawnIce`) 0.1 true))
  (set `self.IceSpawningTimer` _returnvalue)
  (bind _returnvalue_2 (`GameplayStatics.SpawnSoundAttached` "/Game/ShiitakeSorcerers/Audio/Ice/IceFloor_Cue.IceFloor_Cue" (`FP_Character.FirstPersonCameraComponent` (cast `/Game/ShiitakeSorcerers/Character/BP_FPCharacter` (`self.GetOwningActorFromActorInfo`) :!pure true)) "None" (0.0 0.0 -100.0) (struct) "KeepRelativeOffset" false 1.0 1.0 0.0 null null))
  (set `self.SpawnedSound` _returnvalue_2)
  (`AbilityTask_WaitInputRelease.WaitInputRelease` true
    (:`OnRelease`
      (`self.SpawnStopper`))))

(event `SpawnIce`
  (bind _asbp_fpcharacter (cast `/Game/ShiitakeSorcerers/Character/BP_FPCharacter` (`self.GetOwningActorFromActorInfo`) :!pure true))
  (bind (_returnvalue_location _returnvalue_rotation _returnvalue_scale) (`KismetMathLibrary.BreakTransform` (`SceneComponent.K2_GetComponentToWorld` (`/Game/ShiitakeSorcerers/Character/BP_FPCharacter.ThrownItems` _asbp_fpcharacter))))
  (bind _canexecute (`/Game/ShiitakeSorcerers/Character/BP_FPCharacter.use Stamina` _asbp_fpcharacter 0.04))
  (if _canexecute
    (`FP_Character.ClientCameraRotation` _asbp_fpcharacter)
    (`AbilityTask_NetworkSyncPoint.WaitNetSync` "BothWait"
      (:`OnSync`
        (bind _returnvalue (`|SpawnActorFromClass` "/Game/ShiitakeSorcerers/Core/Abilities/Ice/IceMovement/BP_IceFloor.BP_IceFloor_C" (`KismetMathLibrary.MakeTransform` (+ (0.0 0.0 -104.0) (`SceneComponent.K2_GetComponentLocation` (`Character.CapsuleComponent` _asbp_fpcharacter))) (`KismetMathLibrary.MakeRotator` (.roll _returnvalue_rotation) (`KismetMathLibrary.FClamp` (.pitch _returnvalue_rotation) -40.0 40.0) (.yaw _returnvalue_rotation)) _returnvalue_scale) "Undefined" "OverrideRootScale" null null))
        (`SceneComponent.K2_SetRelativeRotation` (`/Game/ShiitakeSorcerers/Core/Abilities/Ice/IceMovement/BP_IceFloor.Ice` _returnvalue) (`KismetMathLibrary.MakeRotator` 0.0 0.0 (`KismetMathLibrary.RandomFloatInRange` 0.0 360.0)) false false)))
    (else
      (`self.SpawnStopper`))))

(event `SpawnStopper`
  (bind _spawnedsound (`self.SpawnedSound`))
  (`KismetSystemLibrary.K2_ClearAndInvalidateTimerHandle` (`self.IceSpawningTimer`))
  (`AudioComponent.FadeOut` _spawnedsound 0.5 0.0 "SCurve")
  (`ActorComponent.K2_DestroyComponent` _spawnedsound)
  (`self.K2_EndAbility`))