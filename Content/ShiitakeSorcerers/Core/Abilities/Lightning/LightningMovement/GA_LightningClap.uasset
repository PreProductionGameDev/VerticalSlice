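; Lightning Clap gameplay ability: a hold-to-charge teleport along the player's aim that spends stamina by distance.
; While held, a looping timer raises the cost up to available stamina and moves a spawned indicator along the camera forward vector, snapping to line trace hits.
; On release, it calls ClientCameraRotation and waits for net sync before the final placement.
; Ending teleports the character to the indicator and charges stamina; cancelling only destroys the indicator.
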(event `self.K2_ActivateAbility`
  (bind _asbp_fpcharacter (cast `/Game/ShiitakeSorcerers/Character/BP_FPCharacter` (`self.GetOwningActorFromActorInfo`)))
  (bind _returnvalue (`|SpawnActorFromClass` "/Game/ShiitakeSorcerers/Core/Abilities/Lightning/LightningMovement/BP_ClapIndicator.BP_ClapIndicator_C" (`Actor.GetTransform` _asbp_fpcharacter) "Undefined" "OverrideRootScale" null _asbp_fpcharacter))
  (set `self.ClapIndicator` _returnvalue)
  (bind _returnvalue_2 (`KismetSystemLibrary.K2_SetTimerDelegate` (delegate `UpdateIndicator`) 0.01 true))
  (set `self.IndicatorMovementHandle` _returnvalue_2)
  (`AbilityTask_WaitInputRelease.WaitInputRelease` true
    (:`OnRelease`
      (`KismetSystemLibrary.K2_ClearAndInvalidateTimerHandle` (`self.IndicatorMovementHandle`))
      (`FP_Character.ClientCameraRotation` (cast `/Game/ShiitakeSorcerers/Character/BP_FPCharacter` (`self.GetOwningActorFromActorInfo`) :!pure true))
      (`AbilityTask_NetworkSyncPoint.WaitNetSync` "BothWait"
        (:`OnSync`
          (`self.MoveIndicator`)
          (`self.K2_EndAbility`))))))

(event `UpdateIndicator`
  (bind _asbp_fpcharacter (cast `/Game/ShiitakeSorcerers/Character/BP_FPCharacter` (`self.GetOwningActorFromActorInfo`) :!pure true))
  (`/Game/ShiitakeSorcerers/Character/BP_FPCharacter.use Stamina` _asbp_fpcharacter 0.0)
  (if (>= (`/Game/ShiitakeSorcerers/Character/BP_FPCharacter.Stamina` _asbp_fpcharacter) (+ (`self.StaminaCost`) 0.005))
    (set `self.StaminaCost` (+ (`self.StaminaCost`) 0.005))
    (`self.MoveIndicator`)
    (else
      (set `self.StaminaCost` (`/Game/ShiitakeSorcerers/Character/BP_FPCharacter.Stamina` (cast `/Game/ShiitakeSorcerers/Character/BP_FPCharacter` (`self.GetOwningActorFromActorInfo`) :!pure true)))
      (`self.MoveIndicator`))))

(event `MoveIndicator`
  (bind _firstpersoncameracomponent (`FP_Character.FirstPersonCameraComponent` (cast `/Game/ShiitakeSorcerers/Character/BP_FPCharacter` (`self.GetOwningActorFromActorInfo`) :!pure true)))
  (bind _returnvalue (`SceneComponent.K2_GetComponentLocation` _firstpersoncameracomponent))
  (bind _returnvalue_2 (+ _returnvalue (* (`SceneComponent.GetForwardVector` _firstpersoncameracomponent) (* (`self.StaminaCost`) (`self.MaxDistance`)))))
  (`Actor.K2_SetActorLocation` (`self.ClapIndicator`) _returnvalue_2 true false)
  (bind (_outhit _returnvalue_3) (`KismetSystemLibrary.LineTraceSingle` _returnvalue _returnvalue_2 "TraceTypeQuery3"))
  (if _returnvalue_3
    (`Actor.K2_SetActorLocation` (`self.ClapIndicator`) (`.Location` (`GameplayStatics.BreakHitResult` _outhit)) true false)))

(event `self.K2_OnEndAbility`
  (params (bWasCancelled :type Boolean))
  (bind _asbp_fpcharacter (cast `/Game/ShiitakeSorcerers/Character/BP_FPCharacter` (`self.GetOwningActorFromActorInfo`) :!pure true))
  (if bWasCancelled
    (`Actor.K2_DestroyActor` (`self.ClapIndicator`))
    (else
      (`Actor.K2_SetActorLocation` _asbp_fpcharacter (`Actor.K2_GetActorLocation` (`self.ClapIndicator`)) false true)
      (`/Game/ShiitakeSorcerers/Character/BP_FPCharacter.use Stamina` _asbp_fpcharacter (`self.StaminaCost`))
      (`Actor.K2_DestroyActor` (`self.ClapIndicator`)))))