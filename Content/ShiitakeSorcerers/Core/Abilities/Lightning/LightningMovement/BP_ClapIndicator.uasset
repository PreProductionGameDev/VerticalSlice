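; Destination indicator for a lightning movement blink ability, with a sphere visible only when the instigator is the local player pawn.
; Tick shifts the capsule vertically according to the Forward vector to set the landing point.
; ServerBlink hides the caster, spawns a trail, and uses a timeline to animate FOV and teleport-lerp from Origin to the capsule.
; On finish it restores visibility, re-hides the widget through ClientHideHP, removes the movement tag and destroys itself after a delay.
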(event `self.ReceiveBeginPlay`
  (if (!= (`GameplayStatics.GetPlayerPawn` 0) (`self.GetInstigator`))
    (`SceneComponent.SetVisibility` (`self.Sphere`) false false)))

(event `self.ReceiveTick`
  (params (DeltaSeconds :type "Float (single-precision)"))
  (`SceneComponent.K2_SetRelativeLocation` (`self.Capsule`) (`KismetMathLibrary.MakeVector` 0.0 0.0 (- -120.0 (* (`KismetMathLibrary.Dot_VectorVector` (`KismetMathLibrary.Conv_RotatorToVector` (`KismetMathLibrary.FindLookAtRotation` (`self.forward`) (`KismetMathLibrary.MakeVector` 0.0 0.0 1.0))) (0.0 0.0 -1.0)) 240.0))) false false))

(event `ServerBlink`
  (bind _asbp_fpcharacter (cast `/Game/ShiitakeSorcerers/Character/BP_FPCharacter` (`self.GetInstigator`) :!pure true))
  (bind _asbp_fpcharacter_2 (cast `/Game/ShiitakeSorcerers/Character/BP_FPCharacter` (`self.GetInstigator`) :!pure true))
  (bind _mesh (`Character.Mesh` _asbp_fpcharacter_2))
  (`SceneComponent.SetVisibility` (`self.Sphere`) false false)
  (`SceneComponent.SetVisibility` _mesh false true)
  (`SceneComponent.SetVisibility` (`/Game/ShiitakeSorcerers/Character/BP_FPCharacter.Widget` _asbp_fpcharacter_2) false true)
  (`/Game/ShiitakeSorcerers/Character/BP_FPCharacter.MulticastSpawnTrail` _asbp_fpcharacter_2)
  (bind (_direction _completion _fov) (`Timeline|Timeline_0` :!via `PlayFromStart`)
    (:`Update`
      (`CameraComponent.SetFieldOfView` (`FP_Character.FirstPersonCameraComponent` _asbp_fpcharacter) _fov)
      (`self.K2_SetActorLocation` _asbp_fpcharacter (`KismetMathLibrary.VLerp` (`self.Origin`) (`SceneComponent.K2_GetComponentLocation` (`self.Capsule`)) _completion) false true))
    (:`Finished`
      (`SceneComponent.SetVisibility` _mesh true true)
      (`SceneComponent.SetVisibility` (`/Game/ShiitakeSorcerers/Character/BP_FPCharacter.Widget` _asbp_fpcharacter_2) true true)
      (`self.ClientHideHP`)
      (`AbilitySystemBlueprintLibrary.RemoveLooseGameplayTags` _asbp_fpcharacter (`BlueprintGameplayTagLibrary.MakeGameplayTagContainerFromArray` (`|MakeArray` (struct :`TagName` "Ability.Element.Movement") :!type "GameplayTag Structure")) true)
      (`KismetSystemLibrary.Delay` 0.6)
      (`self.K2_DestroyActor`))))

(event `ClientHideHP`
  (`SceneComponent.SetVisibility` (`/Game/ShiitakeSorcerers/Character/BP_FPCharacter.Widget` (cast `/Game/ShiitakeSorcerers/Character/BP_FPCharacter` (`self.GetInstigator`) :!pure true)) false true))

(fn `UserConstructionScript`)