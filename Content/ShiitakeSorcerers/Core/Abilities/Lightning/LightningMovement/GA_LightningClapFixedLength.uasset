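; Gameplay ability for a lightning blink: hold input to aim a destination indicator, release to blink there.
; If stamina suffices, it spawns the indicator and a looping timer keeps it at max camera-forward distance, pulled back to any traced hit.
; Camera rotation updates and WaitNetSync precede each placement.
; Normal end spawns vanish FX, calls the indicator's ServerBlink and spends stamina, while cancelling destroys the indicator.
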(event `self.K2_ActivateAbility`
  (bind _asbp_fpcharacter (cast `/Game/ShiitakeSorcerers/Character/BP_FPCharacter` (`self.GetOwningActorFromActorInfo`) :!pure true))
  (if (>= (`/Game/ShiitakeSorcerers/Character/BP_FPCharacter.Stamina` _asbp_fpcharacter) (`self.StaminaCost`))
    (bind _returnvalue (`|SpawnActorFromClass` "/Game/ShiitakeSorcerers/Core/Abilities/Lightning/LightningMovement/BP_ClapIndicator.BP_ClapIndicator_C" (`Actor.GetTransform` _asbp_fpcharacter) "Undefined" "OverrideRootScale" null _asbp_fpcharacter))
    (set `self.ClapIndicator` _returnvalue)
    (bind _returnvalue_2 (`KismetSystemLibrary.K2_SetTimerDelegate` (delegate `UpdateIndicator`) 0.01 true))
    (set `self.IndicatorMovementHandle` _returnvalue_2)
    (`AbilityTask_WaitInputRelease.WaitInputRelease` true
      (:`OnRelease`
        (`KismetSystemLibrary.K2_ClearAndInvalidateTimerHandle` (`self.IndicatorMovementHandle`))
        (`FP_Character.ClientCameraRotation` (cast `/Game/ShiitakeSorcerers/Character/BP_FPCharacter` (`self.GetOwningActorFromActorInfo`) :!pure true))
        (`AbilityTask_NetworkSyncPoint.WaitNetSync` "BothWait"
          (:`OnSync`
            (`self.MoveIndicator`)
            (`self.K2_EndAbility`)))))
    (else
      (`self.K2_CancelAbility`))))

(event `UpdateIndicator`
  (`/Game/ShiitakeSorcerers/Character/BP_FPCharacter.use Stamina` (cast `/Game/ShiitakeSorcerers/Character/BP_FPCharacter` (`self.GetOwningActorFromActorInfo`) :!pure true) 0.0)
  (`self.MoveIndicator`))

(event `MoveIndicator`
  (bind _clapindicator (`self.ClapIndicator`))
  (bind _firstpersoncameracomponent (`FP_Character.FirstPersonCameraComponent` (cast `/Game/ShiitakeSorcerers/Character/BP_FPCharacter` (`self.GetOwningActorFromActorInfo`) :!pure true)))
  (bind _returnvalue (`SceneComponent.GetForwardVector` _firstpersoncameracomponent))
  (bind _returnvalue_2 (`SceneComponent.K2_GetComponentLocation` _firstpersoncameracomponent))
  (bind _returnvalue_3 (+ _returnvalue_2 (* _returnvalue (`self.MaxDistance`))))
  (`FP_Character.ClientCameraRotation` (cast `/Game/ShiitakeSorcerers/Character/BP_FPCharacter` (`self.GetOwningActorFromActorInfo`) :!pure true))
  (`AbilityTask_NetworkSyncPoint.WaitNetSync` "BothWait"
    (:`OnSync`
      (set `/Game/ShiitakeSorcerers/Core/Abilities/Lightning/LightningMovement/BP_ClapIndicator.forward` _returnvalue _clapindicator)
      (`Actor.K2_SetActorLocation` _clapindicator _returnvalue_3 true false)
      (bind (_outhit _returnvalue_4) (`KismetSystemLibrary.LineTraceSingle` _returnvalue_2 _returnvalue_3 "TraceTypeQuery3"))
      (if _returnvalue_4
        (`Actor.K2_SetActorLocation` (`self.ClapIndicator`) (+ (`.Location` (`GameplayStatics.BreakHitResult` _outhit)) (* (`.Normal` (`GameplayStatics.BreakHitResult` _outhit)) 44.0)) true false)))))

(event `self.K2_OnEndAbility`
  (params (bWasCancelled :type Boolean))
  (bind _clapindicator (`self.ClapIndicator`))
  (bind _clapindicator_2 (`self.ClapIndicator`))
  (bind _asbp_fpcharacter (cast `/Game/ShiitakeSorcerers/Character/BP_FPCharacter` (`self.GetOwningActorFromActorInfo`) :!pure true))
  (if bWasCancelled
    (`/Engine/EditorBlueprintResources/StandardMacros.IsValid` _clapindicator
      (:`Is Valid`
        (`Actor.K2_DestroyActor` _clapindicator)))
    (else
      (bind _output_get (set `/Game/ShiitakeSorcerers/Core/Abilities/Lightning/LightningMovement/BP_ClapIndicator.Origin` (`SceneComponent.K2_GetComponentLocation` (`Character.CapsuleComponent` _asbp_fpcharacter)) _clapindicator_2))
      (`|SpawnActorFromClass` "/Game/ShiitakeSorcerers/VFX/BP_VanishFX.BP_VanishFX_C" (`KismetMathLibrary.MakeTransform` _output_get (`SceneComponent.K2_GetComponentRotation` (`FP_Character.FirstPersonCameraComponent` _asbp_fpcharacter))) "Undefined" "OverrideRootScale" null null)
      (`/Game/ShiitakeSorcerers/Core/Abilities/Lightning/LightningMovement/BP_ClapIndicator.ServerBlink` _clapindicator_2)
      (`/Game/ShiitakeSorcerers/Character/BP_FPCharacter.use Stamina` _asbp_fpcharacter (`self.StaminaCost`)))))