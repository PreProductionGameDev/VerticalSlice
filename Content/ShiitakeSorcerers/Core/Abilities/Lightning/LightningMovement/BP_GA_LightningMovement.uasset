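; Lightning movement gameplay ability that blinks the player, with its logic in a TeleportPlayer event.
; The event has the character spawn a lightning dash sound on its first-person camera through a server call.
; It then passes the owner's location and camera forward vector to the BP_ClapIndicator and calls ServerBlink, delegating the teleport to that indicator.
; ActivateAbility and OnEndAbility are unused here.
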(event `self.TeleportPlayer`
  (bind _returnvalue (`self.GetOwningActorFromActorInfo`))
  (bind _asfp_character (cast `FP_Character` _returnvalue :!pure true))
  (bind _firstpersoncameracomponent (`FP_Character.FirstPersonCameraComponent` _asfp_character))
  (`FP_Character.ServerSpawnSoundAttached` :`self` _asfp_character :`Sound` "/Game/ShiitakeSorcerers/Audio/SoundFX/Lightning/A_LightningDash_Cue.A_LightningDash_Cue" :`AttachToComponent` _firstpersoncameracomponent :`AttenuationSettings` null :`ConcurrencySettings` null)
  (bind _asbp_clap_indicator (cast `/Game/ShiitakeSorcerers/Core/Abilities/Lightning/LightningMovement/BP_ClapIndicator` (`self.Indicator`)))
  (set `/Game/ShiitakeSorcerers/Core/Abilities/Lightning/LightningMovement/BP_ClapIndicator.Origin` (`Actor.K2_GetActorLocation` _returnvalue) _asbp_clap_indicator)
  (set `/Game/ShiitakeSorcerers/Core/Abilities/Lightning/LightningMovement/BP_ClapIndicator.forward` (`SceneComponent.GetForwardVector` _firstpersoncameracomponent) _asbp_clap_indicator)
  (`/Game/ShiitakeSorcerers/Core/Abilities/Lightning/LightningMovement/BP_ClapIndicator.ServerBlink` _asbp_clap_indicator))