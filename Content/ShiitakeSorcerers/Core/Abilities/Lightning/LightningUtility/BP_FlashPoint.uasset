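; Flash point actor for a lightning utility ability that blinds characters after a short fuse, then fades its audio and destroys itself.
; A BeginPlay timer triggers Flash, with Niagara activating shortly beforehand.
; Flash line-traces to every BP_FPCharacter's camera and calls ClientFlash on those with clear line of sight.
; Blind strength comes from a view-direction dot product remapped to 0–1, strongest when looking straight at the flash.
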(event `self.ReceiveBeginPlay`
  (`KismetSystemLibrary.K2_SetTimerDelegate` (delegate `Flash`) 2.0)
  (`KismetSystemLibrary.Delay` 1.5)
  (`ActorComponent.Activate` (`self.Niagara`) false))

(event `Flash`
  (bind _outactors (`GameplayStatics.GetAllActorsOfClass` "/Game/ShiitakeSorcerers/Character/BP_FPCharacter.BP_FPCharacter_C"))
  (for _array_element _outactors
    (bind (_blind _blindstrength) (`self.BlindCheck` _array_element))
    (if _blind
      (`/Game/ShiitakeSorcerers/Character/BP_FPCharacter.ClientFlash` _array_element _blindstrength)))
  (`AudioComponent.FadeOut` (`self.Audio`) 0.5 0.0 "Linear")
  (`KismetSystemLibrary.Delay` 0.5)
  (`self.K2_DestroyActor`))

(fn `BlindCheck`
  (params (Character :type "/Game/ShiitakeSorcerers/Character/BP_FPCharacter Object Reference"))
  (returns (Blind :type Boolean) (BlindStrength :type "Float (double-precision)"))
  (bind _returnvalue (`self.K2_GetActorLocation`))
  (bind _firstpersoncameracomponent (`FP_Character.FirstPersonCameraComponent` Character))
  (bind _returnvalue_2 (`SceneComponent.K2_GetComponentLocation` _firstpersoncameracomponent))
  (bind _returnvalue_3 (`KismetMathLibrary.Conv_RotatorToVector` (`SceneComponent.K2_GetComponentRotation` _firstpersoncameracomponent)))
  (bind _returnvalue_4 (`KismetMathLibrary.Conv_RotatorToVector` (`KismetMathLibrary.FindLookAtRotation` _returnvalue_2 _returnvalue)))
  (bind (_outhit _returnvalue_5) (`KismetSystemLibrary.LineTraceSingle` _returnvalue _returnvalue_2 "TraceTypeQuery1"))
  (return (not _returnvalue_5) (+ (/ (`KismetMathLibrary.Dot_VectorVector` _returnvalue_4 _returnvalue_3) (+ (`KismetMathLibrary.VSize` _returnvalue_4) (`KismetMathLibrary.VSize` _returnvalue_3))) 0.5)))

(fn `UserConstructionScript`)