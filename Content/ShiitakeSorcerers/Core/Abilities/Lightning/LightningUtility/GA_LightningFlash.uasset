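; Lightning Flash gameplay ability that lets the player aim a flash point while holding input and places it on release.
; A looping timer moves a ghost marker, visible only to the local player, along a net-synced camera trace to the hit surface or maximum range.
; Release spawns BP_FlashPoint at the ghost's transform, destroys the ghost and starts a cooldown timer shown on the HUD.
; Cancellation removes the ghost and clears both timers.
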(event `self.K2_ActivateAbility`
  (bind _returnvalue (`|SpawnActorFromClass` "/Game/ShiitakeSorcerers/Core/Abilities/Lightning/LightningUtility/BP_FlashPointGhost.BP_FlashPointGhost_C" (`KismetMathLibrary.MakeTransform` (0.0 0.0 0.0)) "Undefined" "OverrideRootScale" null null))
  (bind _output_get (set `self.FlashPointGhost` _returnvalue))
  (`self.IsLocallyControlled`
    (:`True`
      _)
    (:`False`
      (`Actor.SetActorHiddenInGame` _output_get true)))
  (bind _returnvalue_2 (`KismetSystemLibrary.K2_SetTimerDelegate` (delegate `MoveGhost`) 0.01 true))
  (set `self.MoveGhostHandle` _returnvalue_2)
  (`AbilityTask_WaitInputRelease.WaitInputRelease` true
    (:`OnRelease`
      (`self.CastAbility`))))

(event `MoveGhost`
  (bind _asbp_fpcharacter (cast `/Game/ShiitakeSorcerers/Character/BP_FPCharacter` (`self.GetOwningActorFromActorInfo`) :!pure true))
  (bind _firstpersoncameracomponent (`FP_Character.FirstPersonCameraComponent` _asbp_fpcharacter))
  (bind _returnvalue (`SceneComponent.K2_GetComponentLocation` _firstpersoncameracomponent))
  (bind _returnvalue_2 (+ _returnvalue (* (`SceneComponent.GetForwardVector` _firstpersoncameracomponent) 4000.0)))
  (`FP_Character.ClientCameraRotation` _asbp_fpcharacter)
  (`AbilityTask_NetworkSyncPoint.WaitNetSync` "BothWait"
    (:`OnSync`
      (bind _outhit (`KismetSystemLibrary.LineTraceSingle` _returnvalue _returnvalue_2 "TraceTypeQuery1" false (`|MakeArray` _asbp_fpcharacter (`FP_Character.GetCurrentWeapon` _asbp_fpcharacter) :!type "Actor Object Reference")))
      (if (`GameplayStatics.BreakHitResult` _outhit)
        (`Actor.K2_SetActorLocation` (`self.FlashPointGhost`) (+ (`.Normal` (`GameplayStatics.BreakHitResult` _outhit)) (`.Location` (`GameplayStatics.BreakHitResult` _outhit))) false false)
        (else
          (`Actor.K2_SetActorLocation` (`self.FlashPointGhost`) _returnvalue_2 false false))))))

(event `CastAbility`
  (bind _returnvalue (`FP_Character.GetPlayerHUD` (cast `/Game/ShiitakeSorcerers/Character/BP_FPCharacter` (`self.GetOwningActorFromActorInfo`) :!pure true)))
  (`KismetSystemLibrary.K2_ClearAndInvalidateTimerHandle` (`self.MoveGhostHandle`))
  (`|SpawnActorFromClass` "/Game/ShiitakeSorcerers/Core/Abilities/Lightning/LightningUtility/BP_FlashPoint.BP_FlashPoint_C" (`Actor.GetTransform` (`self.FlashPointGhost`)) "Undefined" "OverrideRootScale" null null)
  (`Actor.K2_DestroyActor` (`self.FlashPointGhost`))
  (bind _returnvalue_2 (`KismetSystemLibrary.K2_SetTimerDelegate` (`|CreateDelegate` :!event `AbilityCooldown`) 15.0))
  (set `self.CooldownHandle` _returnvalue_2)
  (`/Engine/EditorBlueprintResources/StandardMacros.IsValid` _returnvalue
    (:`Is Valid`
      (`PlayerHUD.SetAbilityCooldown` _returnvalue (`self.CooldownHandle`)))))

(event `self.K2_OnEndAbility`
  (params (bWasCancelled :type Boolean))
  (if bWasCancelled
    (`Actor.K2_DestroyActor` (`self.FlashPointGhost`))
    (`KismetSystemLibrary.K2_ClearAndInvalidateTimerHandle` (`self.MoveGhostHandle`))
    (`KismetSystemLibrary.K2_ClearAndInvalidateTimerHandle` (`self.CooldownHandle`))))

(event `AbilityCooldown`
  (`KismetSystemLibrary.K2_ClearAndInvalidateTimerHandle` (`self.CooldownHandle`))
  (`self.K2_EndAbility`))