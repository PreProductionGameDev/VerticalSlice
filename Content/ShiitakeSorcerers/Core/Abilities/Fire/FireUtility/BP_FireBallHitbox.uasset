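; Short-lived burn area for the Fire ability's fireball, affecting characters inside its box.
; A looping timer polls the box for overlapping BP_FPCharacter actors several times per second.
; For each one, it sends a Fire.Ball.Burn gameplay event to its Instigator with that character as Target, applying no effect itself.
; A second timer clears the tick and destroys the actor after a few seconds.
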(event `BurnOut`
  (`KismetSystemLibrary.K2_ClearAndInvalidateTimerHandle` (`self.FireTick`))
  (`self.K2_DestroyActor`))

(event `Fire Tick`
  (for _array_element (`PrimitiveComponent.GetOverlappingActors` (`self.Box`) "/Game/ShiitakeSorcerers/Character/BP_FPCharacter.BP_FPCharacter_C")
    (`AbilitySystemBlueprintLibrary.SendGameplayEventToActor` (`self.Instigator`) (struct :`TagName` "Fire.Ball.Burn") (make `GameplayEventData` (struct :`TagName` "Fire.Ball.Burn") null _array_element))))

(event `self.ReceiveBeginPlay`
  (bind _returnvalue (`KismetSystemLibrary.K2_SetTimerDelegate` (delegate `Fire Tick`) 0.2 true))
  (set `self.FireTick` _returnvalue)
  (bind _returnvalue_2 (`KismetSystemLibrary.K2_SetTimerDelegate` (delegate `BurnOut`) 5.5 true))
  (set `self.Burn Out` _returnvalue_2))

(fn `UserConstructionScript`)