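; Fireball projectile for the fire utility ability that reports impacts to the Gameplay Ability System.
; On spawn it launches forward with a slight lift plus scaled inherited velocity, and a looping timer restarts its audio from a fixed offset.
; Each tick it line-traces two frames ahead along its velocity, ignoring the caster and weapon.
; A blocking hit sends a Fire.Ball.Hit event targeting itself, leaving impact handling outside this Blueprint.
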(event `ResetSound`
  (`AudioComponent.Play` (`self.Audio`) 1.4))

(event `self.ReceiveBeginPlay`
  (set `MovementComponent.Velocity` (+ (* (`self.initVel`) 2.5) (* (`SceneComponent.GetForwardVector` (`self.Sphere`)) 3500.0) (0.0 0.0 50.0)) (`self.ProjectileMovement`))
  (`KismetSystemLibrary.K2_SetTimerDelegate` (delegate `ResetSound`) 0.1 true 1.4))

(event `self.ReceiveTick`
  (params (DeltaSeconds :type "Float (single-precision)"))
  (bind _returnvalue (`SceneComponent.K2_GetComponentLocation` (`self.Sphere`)))
  (bind _asbp_fpcharacter (cast `/Game/ShiitakeSorcerers/Character/BP_FPCharacter` (`self.GetInstigator`)))
  (bind (_outhits _returnvalue_2) (`KismetSystemLibrary.LineTraceMulti` _returnvalue (+ _returnvalue (* (`MovementComponent.Velocity` (`self.ProjectileMovement`)) DeltaSeconds 2.0)) "TraceTypeQuery2" false (`|MakeArray` _asbp_fpcharacter (`FP_Character.GetCurrentWeapon` _asbp_fpcharacter) :!type "Actor Object Reference")))
  (if _returnvalue_2
    (`AbilitySystemBlueprintLibrary.SendGameplayEventToActor` (`self.Instagator`) (struct :`TagName` "Fire.Ball.Hit") (make `GameplayEventData` (struct :`TagName` "Fire.Ball.Hit") null self))))

(fn `UserConstructionScript`)