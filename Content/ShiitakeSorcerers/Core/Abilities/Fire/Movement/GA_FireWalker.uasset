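; GA_FireWalker is a fire movement gameplay ability that speeds up the character and leaves a flame trail while the input is held.
; On activation it raises walk speed and acceleration and starts a looping timer that spends stamina to spawn BP_FlameTrail actors at the character's transform.
; Input release or failed stamina use clears the timer, sets movement back to hardcoded lower values and ends the ability.
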(event `self.K2_ActivateAbility`
  (bind _returnvalue (`KismetSystemLibrary.K2_SetTimerDelegate` (delegate `SpawnFire`) 0.1 true))
  (set `self.Spawning Fire` _returnvalue)
  (bind _asfp_character (cast `FP_Character` (`self.GetOwningActorFromActorInfo`)))
  (bind _charactermovement (`Character.CharacterMovement` _asfp_character))
  (set `CharacterMovementComponent.MaxWalkSpeed` 1700.0 _charactermovement)
  (set `CharacterMovementComponent.MaxAcceleration` 3048.0 _charactermovement)
  (`AbilityTask_WaitInputRelease.WaitInputRelease` true
    (:`OnRelease`
      (`self.StopSpawning`))))

(event `SpawnFire`
  (bind _asbp_fpcharacter (cast `/Game/ShiitakeSorcerers/Character/BP_FPCharacter` (`self.GetOwningActorFromActorInfo`)))
  (bind _canexecute (`/Game/ShiitakeSorcerers/Character/BP_FPCharacter.use Stamina` _asbp_fpcharacter 0.05))
  (if _canexecute
    (`|SpawnActorFromClass` "/Game/ShiitakeSorcerers/Core/Abilities/Fire/Movement/BP_FlameTrail.BP_FlameTrail_C" (`Actor.GetTransform` _asbp_fpcharacter) "Undefined" "OverrideRootScale" null _asbp_fpcharacter)
    (else
      (`self.StopSpawning`))))

(event `StopSpawning`
  (`KismetSystemLibrary.K2_ClearAndInvalidateTimerHandle` (`self.Spawning Fire`))
  (bind _asfp_character (cast `FP_Character` (`self.GetOwningActorFromActorInfo`)))
  (bind _charactermovement (`Character.CharacterMovement` _asfp_character))
  (set `CharacterMovementComponent.MaxWalkSpeed` 1200.0 _charactermovement)
  (set `CharacterMovementComponent.MaxAcceleration` 2048.0 _charactermovement)
  (`self.K2_EndAbility`))