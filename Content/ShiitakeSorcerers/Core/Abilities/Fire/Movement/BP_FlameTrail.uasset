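; BP_FlameTrail is a flame trail hazard for the Fire movement abilities that reports player characters touching it, excluding its instigator.
; On overlap it prints a debug string, sends a Fire.Trail.Burn gameplay event to the instigator with the victim as target, and starts a short timer.
; BurnTick resends the event for each character still overlapping the capsule and re-arms the timer, leaving burn handling to the instigator.
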(event `self.ReceiveActorBeginOverlap`
  (params (OtherActor :type "Actor Object Reference"))
  (bind _asbp_fpcharacter (cast `/Game/ShiitakeSorcerers/Character/BP_FPCharacter` OtherActor))
  (if (!= OtherActor (`self.GetInstigator`))
    (`KismetSystemLibrary.PrintString` "Hello")
    (`AbilitySystemBlueprintLibrary.SendGameplayEventToActor` (`self.Instigator`) (struct :`TagName` "Fire.Trail.Burn") (make `GameplayEventData` (struct :`TagName` "Fire.Trail.Burn") null _asbp_fpcharacter))
    (`KismetSystemLibrary.K2_SetTimerDelegate` (delegate `Burn Tick`) 0.1)))

(event `Burn Tick`
  (for _array_element (`PrimitiveComponent.GetOverlappingActors` (`self.Capsule`) "/Game/ShiitakeSorcerers/Character/BP_FPCharacter.BP_FPCharacter_C")
    (if (!= _array_element (`self.GetInstigator`))
      (`AbilitySystemBlueprintLibrary.SendGameplayEventToActor` (`self.GetInstigator`) (struct :`TagName` "Fire.Trail.Burn") (make `GameplayEventData` (struct :`TagName` "Fire.Trail.Burn") null _array_element))
      (`KismetSystemLibrary.K2_SetTimerDelegate` (delegate `Burn Tick`) 0.1))))

(fn `UserConstructionScript`)