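; Black hole gravity ability actor that pulls first-person characters toward its center, then destroys itself.
; BeginPlay or the Simulate event starts the GravityTime timeline, whose Range and PullSpeed tracks shape the pull over its lifetime.
; Each update sphere-overlaps BP_FPCharacter actors and applies a velocity-change impulse toward the sphere, scaled by a square-root falloff that strengthens closer to the center.
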(event `Simulate`
  (bind (_direction _range _pullspeed) (`Timeline|GravityTime` :!via `PlayFromStart` :!label _label)
    (:`Update`
      (bind _outactors (`KismetSystemLibrary.SphereOverlapActors` (`SceneComponent.K2_GetComponentLocation` (`self.Sphere`)) _range (`|MakeArray` "ObjectTypeQuery1" "ObjectTypeQuery2" "ObjectTypeQuery3" :!type "EObjectTypeQuery Enum") "/Game/ShiitakeSorcerers/Character/BP_FPCharacter.BP_FPCharacter_C"))
      (for _array_element _outactors
        (bind _asbp_fpcharacter (cast `/Game/ShiitakeSorcerers/Character/BP_FPCharacter` _array_element))
        (bind _returnvalue (- (`SceneComponent.K2_GetComponentLocation` (`self.Sphere`)) (`SceneComponent.K2_GetComponentLocation` (`Character.CapsuleComponent` _asbp_fpcharacter))))
        (`CharacterMovementComponent.AddImpulse` (`Character.CharacterMovement` _asbp_fpcharacter) (* (`KismetMathLibrary.Sqrt` (- 1.0 (/ (`KismetMathLibrary.Vector_Distance` _returnvalue) _range))) _pullspeed (`KismetMathLibrary.Normal` _returnvalue)) true)))
    (:`Finished`
      (`self.K2_DestroyActor`))))

(event `self.ReceiveBeginPlay`
  (goto _label :!via `PlayFromStart`))

(fn `UserConstructionScript`)