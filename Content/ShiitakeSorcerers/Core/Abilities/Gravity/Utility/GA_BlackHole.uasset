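; Gameplay ability that lets the player aim and place a black hole with a ghost preview.
; While input is held, a fast looping timer syncs client camera rotation via WaitNetSync, then moves the ghost along a camera line trace.
; Releasing input swaps the ghost for the black hole, plays its attached sound and starts a HUD-displayed cooldown timer.
; Cancellation destroys the ghost and clears both timers.
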(event `self.K2_ActivateAbility`
  (bind _returnvalue (`|SpawnActorFromClass` "/Game/ShiitakeSorcerers/Core/Abilities/Gravity/Utility/BP_BlackHoleGhost.BP_BlackHoleGhost_C" (`Actor.GetTransform` (`self.GetOwningActorFromActorInfo`)) "Undefined" "OverrideRootScale" null null))
  (set `self.BlackHoleGhost` _returnvalue)
  (bind _returnvalue_2 (`KismetSystemLibrary.K2_SetTimerDelegate` (delegate `MoveGhost`) 0.01 true))
  (set `self.MoveGhostHandle` _returnvalue_2)
  (`AbilityTask_WaitInputRelease.WaitInputRelease` true
    (:`OnRelease`
      (`self.ActivateAbility`))))

(event `MoveGhost`
  (bind _asbp_fpcharacter (cast `/Game/ShiitakeSorcerers/Character/BP_FPCharacter` (`self.GetOwningActorFromActorInfo`) :!pure true))
  (bind _firstpersoncameracomponent (`FP_Character.FirstPersonCameraComponent` _asbp_fpcharacter))
  (bind _returnvalue_location (`KismetMathLibrary.BreakTransform` (`SceneComponent.K2_GetComponentToWorld` _firstpersoncameracomponent)))
  (`FP_Character.ClientCameraRotation` _asbp_fpcharacter)
  (`AbilityTask_NetworkSyncPoint.WaitNetSync` "BothWait"
    (:`OnSync`
      (bind (_outhit _returnvalue) (`KismetSystemLibrary.LineTraceSingle` _returnvalue_location (+ _returnvalue_location (* (`SceneComponent.GetForwardVector` _firstpersoncameracomponent) 2000.0)) "TraceTypeQuery1" false (`|MakeArray` _asbp_fpcharacter :!type "Actor Object Reference")))
      (if _returnvalue
        (`Actor.K2_SetActorLocation` (`self.BlackHoleGhost`) (`.Location` (`GameplayStatics.BreakHitResult` _outhit)) false false)
        (else
          (`Actor.K2_SetActorLocation` (`self.BlackHoleGhost`) (`.TraceEnd` (`GameplayStatics.BreakHitResult` _outhit)) false false))))))

(event `ActivateAbility`
  (bind _returnvalue (`FP_Character.GetPlayerHUD` (cast `/Game/ShiitakeSorcerers/Character/BP_FPCharacter` (`self.GetOwningActorFromActorInfo`) :!pure true)))
  (bind _returnvalue_2 (`|SpawnActorFromClass` "/Game/ShiitakeSorcerers/Core/Abilities/Gravity/Utility/BP_BlackHole.BP_BlackHole_C" (`Actor.GetTransform` (`self.BlackHoleGhost`)) "Undefined" "OverrideRootScale" null null))
  (`KismetSystemLibrary.K2_ClearAndInvalidateTimerHandle` (`self.MoveGhostHandle`))
  (`Actor.K2_DestroyActor` (`self.BlackHoleGhost`))
  (`FP_Character.ServerSpawnSoundAttached` :`self` (cast `/Game/ShiitakeSorcerers/Character/BP_FPCharacter` (`self.GetOwningActorFromActorInfo`) :!pure true) :`Sound` "/Game/ShiitakeSorcerers/Audio/SoundFX/Elements/Gravity/A_BlackHole_Cue.A_BlackHole_Cue" :`AttachToComponent` (`Actor.RootComponent` _returnvalue_2) :`bStopWhenAttachedToDestroyed` true :`AttenuationSettings` null :`ConcurrencySettings` null)
  (bind _returnvalue_3 (`KismetSystemLibrary.K2_SetTimerDelegate` (`|CreateDelegate` :!event `AbilityCooldown`) 15.0))
  (set `self.CooldownHandle` _returnvalue_3)
  (`/Engine/EditorBlueprintResources/StandardMacros.IsValid` _returnvalue
    (:`Is Valid`
      (`PlayerHUD.SetAbilityCooldown` _returnvalue (`self.CooldownHandle`)))))

(event `AbilityCooldown`
  (`KismetSystemLibrary.K2_ClearAndInvalidateTimerHandle` (`self.CooldownHandle`))
  (`self.K2_EndAbility`))

(event `self.K2_OnEndAbility`
  (params (bWasCancelled :type Boolean))
  (if bWasCancelled
    (`Actor.K2_DestroyActor` (`self.BlackHoleGhost`))
    (`KismetSystemLibrary.K2_ClearAndInvalidateTimerHandle` (`self.MoveGhostHandle`))
    (`KismetSystemLibrary.K2_ClearAndInvalidateTimerHandle` (`self.CooldownHandle`))))