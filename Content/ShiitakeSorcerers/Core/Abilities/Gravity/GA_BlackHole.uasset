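; Gameplay ability that lets the player aim a black hole while holding input and places it on release.
; On activation it spawns a ghost actor, which a fast looping timer moves along a camera line trace to the hit point or maximum range.
; Each tick calls the character's ClientCameraRotation and waits for net sync before tracing.
; Any ability end spawns BP_BlackHole at the ghost's transform, clears the timer and destroys the ghost.
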(event `self.K2_ActivateAbility`
  (bind _returnvalue (`|SpawnActorFromClass` "/Game/ShiitakeSorcerers/Core/Abilities/Gravity/BP_BlackHoleGhost.BP_BlackHoleGhost_C" (`Actor.GetTransform` (`self.GetOwningActorFromActorInfo`)) "Undefined" "OverrideRootScale" null null))
  (set `self.BlackHoleGhost` _returnvalue)
  (bind _returnvalue_2 (`KismetSystemLibrary.K2_SetTimerDelegate` (delegate `MoveGhost`) 0.01 true))
  (set `self.MoveGhostHandle` _returnvalue_2)
  (`AbilityTask_WaitInputRelease.WaitInputRelease` true
    (:`OnRelease`
      (`self.K2_EndAbility`))))

(event `MoveGhost`
  (bind _asbp_fpcharacter (cast `/Game/ShiitakeSorcerers/Character/BP_FPCharacter` (`self.GetOwningActorFromActorInfo`) :!pure true))
  (bind _firstpersoncameracomponent (`FP_Character.FirstPersonCameraComponent` _asbp_fpcharacter))
  (bind _returnvalue_location (`KismetMathLibrary.BreakTransform` (`SceneComponent.K2_GetComponentToWorld` _firstpersoncameracomponent)))
  (`FP_Character.ClientCameraRotation` _asbp_fpcharacter)
  (`AbilityTask_NetworkSyncPoint.WaitNetSync` "BothWait"
    (:`OnSync`
      (bind (_outhit _returnvalue) (`KismetSystemLibrary.LineTraceSingle` _returnvalue_location (+ _returnvalue_location (* (`SceneComponent.GetForwardVector` _firstpersoncameracomponent) 2000.0)) "TraceTypeQuery1" false (`|MakeArray` _asbp_fpcharacter :!type "Actor Object Reference")))
      (if _returnvalue
        (`Actor.K2_SetActorLocation` (`self.BlackHoleGhost`) (`.Location` (`GameplayStatics.BreakHitResult` _outhit)) false false)
        (else
          (`Actor.K2_SetActorLocation` (`self.BlackHoleGhost`) (`.TraceEnd` (`GameplayStatics.BreakHitResult` _outhit)) false false))))))

(event `self.K2_OnEndAbility`
  (params (bWasCancelled :type Boolean))
  (`|SpawnActorFromClass` "/Game/ShiitakeSorcerers/Core/Abilities/Gravity/BP_BlackHole.BP_BlackHole_C" (`Actor.GetTransform` (`self.BlackHoleGhost`)) "Undefined" "OverrideRootScale" null null)
  (`KismetSystemLibrary.K2_ClearAndInvalidateTimerHandle` (`self.MoveGhostHandle`))
  (`Actor.K2_DestroyActor` (`self.BlackHoleGhost`)))