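; Fireball gameplay ability that throws a projectile and leaves branching patches of fire where it hits.
; After a net sync it spawns the projectile, listens for hit and burn events, and starts a HUD-linked timer that ends the ability as its cooldown.
; On hit, the server grows fire outward radially, splitting angles and line-tracing each step to avoid walls and cliffs.
; Burn events apply GE_BurnDamage to their target.
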(event `ServerSpawnFireBall`
  (params (Transform :type "Transform Structure") (Inst :type "/Game/ShiitakeSorcerers/Character/BP_FPCharacter Object Reference"))
  ;[1 1 1] Server spawns the fireball so their is no duplicates
  (`|SpawnActorFromClass` "/Game/ShiitakeSorcerers/Core/Abilities/FireBall/BP_FireBallProjectile.BP_FireBallProjectile_C" Transform "Undefined" "OverrideRootScale" null Inst Inst))

(event `AbillityCooldown`
  ;[1 1 1] Abillity cooldown and reset
  (`self.K2_EndAbility`)
  (`KismetSystemLibrary.K2_ClearAndInvalidateTimerHandle` (`self.CooldownTimer`)))

(event `self.K2_ActivateAbility`
  ;[1 1 1] Spawns the fireball if the server before waiting for the gameplay event
  (bind _asbp_fpcharacter (cast `/Game/ShiitakeSorcerers/Character/BP_FPCharacter` (`self.GetOwningActorFromActorInfo`)))
  (`FP_Character.ClientCameraRotation` _asbp_fpcharacter)
  (`AbilityTask_NetworkSyncPoint.WaitNetSync` "BothWait"
    (:`OnSync`
      (`self.ServerSpawnFireBall` (`SceneComponent.K2_GetComponentToWorld` (`/Game/ShiitakeSorcerers/Character/BP_FPCharacter.ThrownItems` _asbp_fpcharacter)) _asbp_fpcharacter)
      (bind (_asynctaskproxy _payload) (`AbilityTask_WaitGameplayEvent.WaitGameplayEvent` (struct :`TagName` "Fire.Ball.Hit") null)
        (:`then`
          (set `self.AsyncCollisionTask` _asynctaskproxy)
          ;[1 1 1] Abillity cooldown and reset
          (bind _returnvalue (`KismetSystemLibrary.K2_SetTimerDelegate` (delegate `AbillityCooldown`) 15.0))
          (set `self.CooldownTimer` _returnvalue)
          (bind _asbp_fpcharacter_2 (cast `/Game/ShiitakeSorcerers/Character/BP_FPCharacter` (`self.GetOwningActorFromActorInfo`)))
          (bind _hud (`/Game/ShiitakeSorcerers/Character/BP_FPCharacter.Hud` _asbp_fpcharacter_2))
          (if (`KismetSystemLibrary.IsValid` _hud)
            (set `/Game/ShiitakeSorcerers/UI/HUD/WB_IconButton.AbilityCD` (`self.CooldownTimer`) (`/Game/ShiitakeSorcerers/UI/HUD/WB_HUD.WB_IconButton` _hud)))
          ;[1 1 1] Burn Damage
          (if (`KismetSystemLibrary.IsServer`)
            (bind (_asynctaskproxy_2 _payload_2) (`AbilityTask_WaitGameplayEvent.WaitGameplayEvent` (struct :`TagName` "Fire.Ball.Burn") null)
              (:`EventReceived`
                (`self.BP_ApplyGameplayEffectToTarget` (`AbilitySystemBlueprintLibrary.AbilityTargetDataFromActor` (`.Target` (break `GameplayEventData` _payload_2))) "/Game/ShiitakeSorcerers/Core/Abilities/FireBall/GE_BurnDamage.GE_BurnDamage_C")))))
        (:`EventReceived`
          ;[1 1 1] Leave the ground if in it
          (if (`KismetSystemLibrary.IsServer`)
            (bind (_eventtag _instigator _target) (break `GameplayEventData` _payload))
            (bind _returnvalue_2 (+ (`Actor.K2_GetActorLocation` _target) (0.0 0.0 50.0) (* (`Actor.GetActorForwardVector` _target) -1.0)))
            (bind _outhit (`KismetSystemLibrary.LineTraceSingle` _returnvalue_2 (- _returnvalue_2 (0.0 0.0 400.0)) "TraceTypeQuery1"))
            (`Actor.K2_DestroyActor` _target)
            ;[1 1 1] Creates the fire effect in 8 directions around the hit location
            (for _index (range 9)
              (bind _returnvalue_3 (`KismetMathLibrary.MultiplyByPi` (/ (`KismetMathLibrary.Conv_IntToDouble` _index) 4.0)))
              (bind _returnvalue_4 (`KismetMathLibrary.Sin` _returnvalue_3))
              (bind _returnvalue_5 (`KismetMathLibrary.Cos` _returnvalue_3))
              (bind (_spawned _location) (`self.FireSpread` (+ (`.Location` (`GameplayStatics.BreakHitResult` _outhit)) (0.0 0.0 1.0)) (`KismetMathLibrary.MakeVector` _returnvalue_4 _returnvalue_5) 100.0 100.0))
              (if _spawned
                (bind (_split1 _split2) (`self.Split Angle` (`KismetMathLibrary.MakeVector` _returnvalue_4 _returnvalue_5) 22.5))
                (bind (_spawned_2 _location_2) (`self.FireSpread` _location (`KismetMathLibrary.MakeVector` (.x _split1) (.y _split1)) 100.0 100.0))
                (bind (_spawned_3 _location_3) (`self.FireSpread` _location (`KismetMathLibrary.MakeVector` (.x _split2) (.y _split2)) 100.0 100.0))
                (if _spawned_2
                  (bind (_split1_2 _split2_2) (`self.Split Angle` (`KismetMathLibrary.MakeVector` (.x _split1) (.y _split1)) 22.5))
                  (`self.FireSpread` _location_2 (`KismetMathLibrary.MakeVector` (.x _split1_2) (.y _split1_2)) 100.0 100.0)
                  (`self.FireSpread` _location_2 (`KismetMathLibrary.MakeVector` (.x _split2_2) (.y _split2_2)) 100.0 100.0))
                (if _spawned_3
                  (bind _split1_3 (`self.Split Angle` (`KismetMathLibrary.MakeVector` (.x _split2) (.y _split2)) 22.5))
                  (`self.FireSpread` _location_3 (`KismetMathLibrary.MakeVector` (.x _split1_3) (.y _split1_3)) 100.0 100.0))))
            (`KismetSystemLibrary.DelayUntilNextTick`)
            (bind _asbp_fpcharacter_3 (cast `/Game/ShiitakeSorcerers/Character/BP_FPCharacter` (`self.GetOwningActorFromActorInfo`)))
            (`/Game/ShiitakeSorcerers/Character/BP_FPCharacter.ServerSpawnFire` _asbp_fpcharacter_3 (`.Location` (`GameplayStatics.BreakHitResult` _outhit)))))))))

(event `self.K2_OnEndAbility`
  (params (bWasCancelled :type Boolean))
  (bind _asynccollisiontask (`self.AsyncCollisionTask`))
  ;[1 1 1] ends tasks
  (if (`KismetSystemLibrary.IsValid` _asynccollisiontask)
    (`GameplayTask.EndTask` _asynccollisiontask)))

(fn `FireSpread`
  (params (Start :type "Vector Structure") (Direction :type "Vector Structure") (`Max Height` :type "Float (double-precision)") (Distance :type "Float (double-precision)"))
  (returns (Spawned :type Boolean) (Location :type "Vector Structure"))
  (bind _returnvalue (`KismetSystemLibrary.IsServer`))
  (bind _returnvalue_2 (+ Start (* Direction Distance) (`KismetMathLibrary.MakeVector` 0.0 0.0 `Max Height`) (0.0 0.0 0.0)))
  ;[1 1 1] Find The next spawn location if their is no wall or cliff
  (bind (_outhit _returnvalue_3) (`KismetSystemLibrary.LineTraceSingle` :`Start` Start :`End` _returnvalue_2 :`TraceChannel` "TraceTypeQuery1" :`DrawDebugType` "ForDuration"))
  (if _returnvalue_3
    (return false (0.0 0.0 0.0))
    (else
      (bind (_outhit_2 _returnvalue_4) (`KismetSystemLibrary.LineTraceSingle` :`Start` _returnvalue_2 :`End` (- _returnvalue_2 (`KismetMathLibrary.MakeVector` 0.0 0.0 (* `Max Height` 2.0))) :`TraceChannel` "TraceTypeQuery1" :`DrawDebugType` "ForDuration"))
      (if _returnvalue_4
        (bind _asbp_fpcharacter (cast `/Game/ShiitakeSorcerers/Character/BP_FPCharacter` (`self.GetOwningActorFromActorInfo`)))
        (if _returnvalue
          (`/Game/ShiitakeSorcerers/Character/BP_FPCharacter.ServerSpawnFire` _asbp_fpcharacter (`.Location` (`GameplayStatics.BreakHitResult` _outhit_2))))
        (return _returnvalue (+ (`.Location` (`GameplayStatics.BreakHitResult` _outhit_2)) (0.0 0.0 1.0)))
        (else
          (return false (0.0 0.0 0.0)))))))

(fn `Split Angle`
  (params (DirectionVector :type "Vector Structure") (`Rotation Amount` :type "Float (double-precision)"))
  (returns (Split1 :type "Vector Structure") (Split2 :type "Vector Structure"))
  (return (`KismetMathLibrary.RotateAngleAxis` DirectionVector `Rotation Amount` (0.0 0.0 1.0)) (`KismetMathLibrary.RotateAngleAxis` DirectionVector (* `Rotation Amount` -1.0) (0.0 0.0 1.0))))