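; King of the Hill game mode for two teams, Red and Blue, ending when either score reaches 10.
; Tick switches the active zone along ZoneOrder as scores cross thresholds, while a looping timer pushes scores to character HUDs.
; Players join a chosen or auto-balanced team, then get a possessed, team-tagged character.
; Respawns retry random team-matching spawn volumes, falling back to PlayerStarts when no volumes exist.
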(event `UpdatePlayerHuds`
  (for _array_element (`self.Actors`)
    (`/Game/ShiitakeSorcerers/Character/BP_FPCharacter.ClientKingOfTheHillHead` _array_element (`KismetMathLibrary.MakeVector` (`self.BlueScore`) (`self.RedScore`)))
    (`KismetSystemLibrary.PrintString` "Hello")))

(event `self.ReceiveBeginPlay`
  (`parent.ReceiveBeginPlay`)
  (`KismetSystemLibrary.K2_SetTimerDelegate` (delegate `UpdatePlayerHuds`) 1.0 true))

(event `self.ReceiveTick`
  (params (DeltaSeconds :type "Float (single-precision)"))
  (`parent.ReceiveTick` DeltaSeconds)
  (`self.ScoreInBounds` 3.3 6.6 1)
  (`self.ScoreInBounds` 6.6 10.0 2)
  (if (and (or (>= (`self.BlueScore`) 10.0) (>= (`self.RedScore`) 10.0)) (not (`self.Winning`)))
    (set `self.Winning` true)
    (`self.GameOver`)))

(event `self.PlayerScored`
  (params (KillerName :type String) (KilledName :type String) (WeaponIcon :type "Texture2D Object Reference"))
  (`parent.PlayerScored` KillerName KilledName WeaponIcon))

(event `self.K2_PostLogin`
  (params (NewPlayer :type "PlayerController Object Reference"))
  (`parent.K2_PostLogin` NewPlayer))

(event `self.HandleStartingNewPlayer`
  (params (NewPlayer :type "PlayerController Object Reference"))
  (`parent.HandleStartingNewPlayer` NewPlayer))

(event `self.K2_OnLogout`
  (params (ExitingController :type "Controller Object Reference"))
  (bind _returnvalue (`PlayerState.GetPlayerName` (`Controller.PlayerState` ExitingController)))
  (`parent.K2_OnLogout` ExitingController)
  (`BlueprintMapLibrary.Map_Remove` (`self.RedTeamMap`) _returnvalue)
  (`BlueprintMapLibrary.Map_Remove` (`self.BlueTeamMap`) _returnvalue)
  (bind _outactors (`GameplayStatics.GetAllActorsOfClass` "/Game/ShiitakeSorcerers/Character/BP_FPCharacter.BP_FPCharacter_C"))
  (set `self.Actors` _outactors)
  (`self.UpdatePlayerHuds`))

(event `self.RedTeam`
  (params (Controller :type "Controller Object Reference"))
  (`BlueprintMapLibrary.Map_Add` (`self.RedTeamMap`) (`PlayerState.GetPlayerName` (`Controller.PlayerState` Controller)))
  (`self.SpawnPlayer` Controller (struct :`TagName` "Team.Red")))

(event `self.BlueTeam`
  (params (Controller :type "Controller Object Reference"))
  (`BlueprintMapLibrary.Map_Add` (`self.BlueTeamMap`) (`PlayerState.GetPlayerName` (`Controller.PlayerState` Controller)))
  (`self.SpawnPlayer` Controller (struct :`TagName` "Team.Blue")))

(event `self.Random`
  (params (Controller :type "Controller Object Reference"))
  (bind _returnvalue (`BlueprintMapLibrary.Map_Length` (`self.BlueTeamMap`)))
  (bind _returnvalue_2 (`BlueprintMapLibrary.Map_Length` (`self.RedTeamMap`)))
  (bind _returnvalue_3 (`PlayerState.GetPlayerName` (`Controller.PlayerState` Controller)))
  (if (> _returnvalue_2 _returnvalue)
    (`BlueprintMapLibrary.Map_Add` (`self.BlueTeamMap`) _returnvalue_3 :!label _label)
    (`self.SpawnPlayer` Controller (struct :`TagName` "Team.Blue"))
    (else
      (if (not (> _returnvalue _returnvalue_2))
        (`|MultiGate` true
          (:`Out 0`
            (goto _label))
          (:`Out 1`
            _)))
      (`BlueprintMapLibrary.Map_Add` (`self.RedTeamMap`) _returnvalue_3)
      (`self.SpawnPlayer` Controller (struct :`TagName` "Team.Red")))))

(event `SpawnPlayer`
  (params (Controller :type "Controller Object Reference") (TeamTag :type "GameplayTag Structure"))
  (bind _outactors (`GameplayStatics.GetAllActorsOfClass` "/Script/Engine.PlayerStart"))
  (bind _returnvalue (`|SpawnActorFromClass` "/Game/ShiitakeSorcerers/Character/BP_FPCharacter.BP_FPCharacter_C" (`self.GetTransform` (`KismetArrayLibrary.Array_Random` _outactors)) "Undefined" "OverrideRootScale" null null))
  (`Controller.Possess` Controller _returnvalue)
  (`/Game/ShiitakeSorcerers/Character/BP_FPCharacter.ClientLoadCosmetcs` _returnvalue)
  (`AbilitySystemBlueprintLibrary.AddLooseGameplayTags` _returnvalue (`BlueprintGameplayTagLibrary.MakeGameplayTagContainerFromArray` (`|MakeArray` TeamTag)))
  (set `/Game/ShiitakeSorcerers/Character/BP_FPCharacter.Red` (== TeamTag (struct :`TagName` "Team.Red")) _returnvalue)
  (set `/Game/ShiitakeSorcerers/Character/BP_FPCharacter.Blue` (== TeamTag (struct :`TagName` "Team.Blue")) _returnvalue)
  (`self.Respawn` _returnvalue)
  (`KismetSystemLibrary.Delay` 0.1)
  (bind _outactors_2 (`GameplayStatics.GetAllActorsOfClass` "/Game/ShiitakeSorcerers/Character/BP_FPCharacter.BP_FPCharacter_C"))
  (set `self.Actors` _outactors_2))

(fn `Activate`
  (params (Index :type Integer))
  (`/Game/ShiitakeSorcerers/Core/Map/BP_CaptureZone.Activate` (`|GetArrayItem` (`self.Zones`) (`|GetArrayItem` (`self.Zone order`) Index))))

(fn `Deactivate`
  (params (`Index-1` :type Integer))
  (`/Game/ShiitakeSorcerers/Core/Map/BP_CaptureZone.Deactivate` (`|GetArrayItem` (`self.Zones`) (`|GetArrayItem` (`self.Zone order`) (- `Index-1` 1)))))

(fn `FindRespawnPoint`
  (params (PlayerName :type String))
  (returns (SpawnLocation :type "Vector Structure") (SpawnRotation :type "Rotator Structure"))
  (locals (RandomVolume :type "/Game/ShiitakeSorcerers/Core/Map/BP_SpawnVolume Object Reference"))
  (bind _randomvolume (`local.RandomVolume`))
  (bind (_returnvalue_x _returnvalue_y _returnvalue_z) (`KismetMathLibrary.BreakVector` (`SceneComponent.K2_GetComponentLocation` (`/Game/ShiitakeSorcerers/Core/Map/BP_SpawnVolume.LookLocation` _randomvolume))))
  (bind _outactors (`GameplayStatics.GetAllActorsOfClass` "/Game/ShiitakeSorcerers/Core/Map/BP_SpawnVolume.BP_SpawnVolume_C"))
  (if (< (`KismetArrayLibrary.Array_Length` _outactors) 1)
    (bind _outactors_2 (`GameplayStatics.GetAllActorsOfClass` "/Script/Engine.PlayerStart"))
    (bind _outitem (`KismetArrayLibrary.Array_Random` _outactors_2))
    (return (`self.K2_GetActorLocation` _outitem) (`self.K2_GetActorRotation` _outitem))
    (else
      (if (`.ReturnValue` (`BlueprintMapLibrary.Map_Find` (`self.RedTeamMap`) (`local.PlayerName`)))
        (bind _outitem_2 (`KismetArrayLibrary.Array_Random` _outactors))
        (bind _output_get (set `local.RandomVolume` _outitem_2 :!label _label))
        (if (== (`/Game/ShiitakeSorcerers/Core/Map/BP_SpawnVolume.SpawnTag` _output_get) "Red")
          _
          (else
            (goto _label)))
        (else
          (bind _output_get_2 (set `local.RandomVolume` _outitem_2 :!label _label_2))
          (if (== (`/Game/ShiitakeSorcerers/Core/Map/BP_SpawnVolume.SpawnTag` _output_get_2) "Blue")
            _
            (else
              (goto _label_2)))))
      (bind (_transform _found) (`/Game/ShiitakeSorcerers/Core/Map/BP_SpawnVolume.FindSpawn` _randomvolume :!label _label_3))
      (if _found
        (return _transform (`KismetMathLibrary.MakeRotator` _returnvalue_x _returnvalue_y _returnvalue_z))
        (else
          (goto _label_3))))))

(fn `GetScores`
  (params (PlayerReq :type "/Game/ShiitakeSorcerers/Character/BP_FPCharacter Object Reference"))
  (returns (Return :type Boolean))
  (locals (BluePlayers :type "Array of Name") (BlueScores :type "Array of Integer64"))
  (bind _redteammap (`self.RedTeamMap`))
  (bind _blueteammap (`self.BlueTeamMap`))
  (bind _keys (`BlueprintMapLibrary.Map_Keys` _redteammap))
  (bind _keys_2 (`BlueprintMapLibrary.Map_Keys` _blueteammap))
  (for _array_element _keys_2
    (`KismetArrayLibrary.Array_Add` (`local.BluePlayers`) (`KismetStringLibrary.Conv_StringToName` _array_element)))
  (bind _values (`BlueprintMapLibrary.Map_Values` _redteammap))
  (bind _values_2 (`BlueprintMapLibrary.Map_Values` _blueteammap))
  (for _array_element_2 _values_2
    (`KismetArrayLibrary.Array_Add` (`local.BlueScores`) (`KismetMathLibrary.Conv_IntToInt64` _array_element_2)))
  (`/Game/ShiitakeSorcerers/Character/BP_FPCharacter.ClientKingOfTheHillLeaderboard` PlayerReq _keys _values (`local.BluePlayers`) (`local.BlueScores`) (`KismetMathLibrary.MakeVector` (`self.RedScore`) (`self.BlueScore`)))
  (return false))

(fn `Respawn`
  (params (Player :type "/Game/ShiitakeSorcerers/Character/BP_FPCharacter Object Reference"))
  (returns (Return :type Boolean))
  (bind (_spawnlocation _spawnrotation) (`self.FindRespawnPoint` (`PlayerState.GetPlayerName` (`Pawn.PlayerState` Player))))
  (`self.K2_SetActorLocation` Player _spawnlocation false true)
  (`/Game/ShiitakeSorcerers/Character/BP_FPCharacter.ClientLookTowards` Player (`KismetMathLibrary.MakeVector` (.roll _spawnrotation) (.pitch _spawnrotation) (.yaw _spawnrotation)))
  (`self.EnableInput` Player null)
  (return false))

(fn `ScoreInBounds`
  (params (LowerBound :type "Float (double-precision)") (UpperBound :type "Float (double-precision)") (ActivateIndex :type Integer))
  (if (and (or (>= (`self.BlueScore`) LowerBound) (>= (`self.RedScore`) LowerBound)) (not (or (>= (`self.BlueScore`) UpperBound) (>= (`self.RedScore`) UpperBound))))
    (`self.Activate` ActivateIndex)
    (`self.Deactivate` ActivateIndex)))

(fn `UserConstructionScript`
  (`parent.UserConstructionScript`))